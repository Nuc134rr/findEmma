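; Lockable VR drawer that slides on a physics constraint and implements the VR grip interface.
; BeginPlay offsets the linear constraint's reference position and limits X travel to the drawer's linear limit.
; Replicated Locked and Closed changes update a separate constraint's angular offset and swing limit, tight when closed and locked, wider when unlocked.
; Dropping the drawer runs a server-only release from the holding hand, if still held.
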(event `self.ReceiveBeginPlay`
  ;[1 1 1] Begin Play - set physics constraint reference position and linear x limit
  (`PhysicsConstraintComponent.SetConstraintReferencePosition` (`self.Drawer1Constraint`) "Frame1" (+ (`SceneComponent.K2_GetComponentLocation` (`self.Drawer1`)) (`KismetMathLibrary.TransformDirection` (`SceneComponent.K2_GetComponentToWorld` (`self.Drawer1Constraint`)) (`KismetMathLibrary.MakeVector` (`self.DrawerLinearLimit`)))))
  (`PhysicsConstraintComponent.SetLinearXLimit` (`self.Drawer1Constraint`) "LCM_Limited" (`self.DrawerLinearLimit`)))

(event `self.Drawer1.OnDropped`
  (params (GrippingController :type "GripMotionControllerComponent Object Reference") (GripInformation :type "BPActorGripInformation Structure (by ref)") (bWasSocketed :type Boolean))
  (`self. Drop Drawer If Held` null))

(fn ` Drop Drawer If Held`
  (params (HoldingHand :type "GripMotionControllerComponent Object Reference"))
  (locals (NewLocalVar_0 :type "GrippableStaticMeshComponent Object Reference"))
  (bind _drawer1 (`self.Drawer1`))
  (`/Engine/EditorBlueprintResources/ActorMacros.Switch Has Authority`
    (:`Authority`
      (if (`GripMotionControllerComponent.GetIsObjectHeld` HoldingHand _drawer1)
        (`GripMotionControllerComponent.DropObjectByInterface` HoldingHand _drawer1 0 (0.0 0.0 0.0) (0.0 0.0 0.0)))
      (return))))

(fn `AdvancedGripSettings`
  (returns (ReturnValue :type "BPAdvGripSettings Structure"))
  (return))

(fn `AllowsMultipleGrips`
  (returns (ReturnValue :type Boolean))
  (return false))

(fn `ClosestGripSlotInRange`
  (params (WorldLocation :type "Vector Structure") (bSecondarySlot :type Boolean) (CallingController :type "GripMotionControllerComponent Object Reference") (OverridePrefix :type Name))
  (returns (bHadSlotInRange :type Boolean) (SlotWorldTransform :type "Transform Structure") (SlotName :type Name))
  (return false (struct) "None"))

(fn `DenyGripping`
  (params (GripInitiator :type "GripMotionControllerComponent Object Reference"))
  (returns (ReturnValue :type Boolean))
  (return false))

(fn `GetGripScripts`
  (returns (ArrayReference :type "Array of VRGripScriptBase Object Reference") (ReturnValue :type Boolean))
  (return _ false))

(fn `GetGripStiffnessAndDamping`
  (returns (GripStiffnessOut :type "Float (double-precision)") (GripDampingOut :type "Float (double-precision)"))
  (return 0.0 0.0))

(fn `GetPrimaryGripType`
  (params (bIsSlot :type Boolean))
  (returns (ReturnValue :type "EGripCollisionType Enum"))
  (return "InteractiveCollisionWithPhysics"))

(fn `GripBreakDistance`
  (returns (ReturnValue :type "Float (double-precision)"))
  (return 0.0))

(fn `GripLateUpdateSetting`
  (returns (ReturnValue :type "EGripLateUpdateSettings Enum"))
  (return "LateUpdatesAlwaysOn"))

(fn `GripMovementReplicationType`
  (returns (ReturnValue :type "EGripMovementReplicationSettings Enum"))
  (return "KeepOriginalMovement"))

(fn `IsHeld`
  (returns (HoldingControllers :type "Array of BPGripPair Structure") (bIsHeld :type Boolean))
  (return _ false))

(fn `On Rep Locked`
  (`self.Set angle`))

(fn `On Rep_Closed`
  (`self.Set angle`))

(fn `RequestsSocketing`
  (returns (ParentToSocketTo :type "SceneComponent Object Reference") (OptionalSocketName :type Name) (RelativeTransform :type "Transform_NetQuantize Structure") (ReturnValue :type Boolean))
  (return null "None" (struct) false))

(fn `SecondaryGripType`
  (returns (ReturnValue :type "ESecondaryGripType Enum"))
  (return "SG_None"))

(fn `Set angle`
  (bind _vrephysicsconstraint (`self.VREPhysicsConstraint`))
  (bind _locked (`self.Locked`))
  (bind _returnvalue (`VREPhysicsConstraintComponent.GetAngularOffset` _vrephysicsconstraint))
  (if true
    (if (and (`self.Closed`) _locked)
      (if (!= _returnvalue (struct :`Yaw` -1.0))
        (`VREPhysicsConstraintComponent.SetAngularOffset` _vrephysicsconstraint (struct :`Pitch` -1.0))
        (`PhysicsConstraintComponent.SetAngularSwing1Limit` _vrephysicsconstraint "ACM_Free" 1.0))
      (elif _locked
        _
        (elif (!= _returnvalue (struct :`Yaw` -45.0))
          (`VREPhysicsConstraintComponent.SetAngularOffset` _vrephysicsconstraint (struct :`Pitch` -45.0))
          (`PhysicsConstraintComponent.SetAngularSwing1Limit` _vrephysicsconstraint "ACM_Free" 45.0))))))

(fn `SimulateOnDrop`
  (returns (ReturnValue :type Boolean))
  (return false))

(fn `TeleportBehavior`
  (returns (ReturnValue :type "EGripInterfaceTeleportBehavior Enum"))
  (return "TeleportAllComponents"))

(fn `UserConstructionScript`)