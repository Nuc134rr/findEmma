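; Screw actor that can be unscrewed by rotation, then picked up and dropped as a physics object.
; AddRotationValue rolls the screw and moves it along its Arrow in proportion to ThreadPitch, accumulating travel distance.
; Past MaximumScrewDistance it clears IsScrewed, fires the Released dispatcher and enables physics.
; Pickup attaches only a released screw to the given component with physics off, and Drop detaches it with physics on.
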(event `self.ReceiveBeginPlay`
  ;[1 1 1] Turn of Physics Simulation if the screw is already released
  (`PrimitiveComponent.SetSimulatePhysics` (`self.StaticMeshComponent`) (not (`self.is Screwed`))))

(event `/Game/VirtualRealityBP/Blueprints/PickupActorInterface.Pickup`
  (params (AttachTo :type "SceneComponent Object Reference"))
  ;[1 1 1] Pickup and Drop
  ;;[0 1 0.00041] You can pickup screw only if it is released
  (if (not (`self.is Screwed`))
    (`PrimitiveComponent.SetSimulatePhysics` (`self.StaticMeshComponent`) false)
    (`SceneComponent.K2_AttachToComponent` (`self.K2_GetRootComponent`) AttachTo "None" "KeepWorld" "KeepWorld" "KeepWorld" false)))

(event `/Game/VirtualRealityBP/Blueprints/PickupActorInterface.Drop`
  ;[1 1 1] Pickup and Drop
  (`self.K2_DetachFromActor` "KeepWorld" "KeepWorld" "KeepWorld")
  (`PrimitiveComponent.SetSimulatePhysics` (`self.StaticMeshComponent`) true))

(fn `Add Rotation Value`
  (params (`Delta Rotation Amount` :type "Float (double-precision)"))
  (returns (`screw out` :type Boolean))
  (bind _returnvalue (* `Delta Rotation Amount` (/ (`self.Thread Pitch`) 360.0)))
  ;[1 1 1] Controls the movement of screw. Controls release of the screw.
  (`self.K2_AddActorLocalRotation` (`KismetMathLibrary.MakeRotator` `Delta Rotation Amount`))
  (`self.K2_AddActorWorldOffset` (* (`SceneComponent.GetForwardVector` (`self.Arrow`)) _returnvalue))
  (bind _output_get (set `self.current distance` (+ _returnvalue (`self.current distance`))))
  (bind _returnvalue_2 (> _output_get (`self.maximum screw distance`)))
  (if _returnvalue_2
    (set `self.is Screwed` false)
    (`self.Released`) ; Call Event Dispatcher
    (`PrimitiveComponent.SetSimulatePhysics` (`self.StaticMeshComponent`) true))
  (return _returnvalue_2))

(fn `UserConstructionScript`)