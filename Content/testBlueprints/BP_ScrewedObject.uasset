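; BP_ScrewedObject is an actor held in place by screws that motion controllers can pick up once it is fully unscrewed.
; Physics starts off, and a ScrewsControlComponent callback turns simulation on when all screws are released.
; Pickup, gated on FreeOfScrews, disables physics and attaches the root to the given component keeping world transforms; Drop re-enables physics and detaches it.
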(event `self.ReceiveBeginPlay`
  (`PrimitiveComponent.SetSimulatePhysics` (`self.StaticMeshComponent`) false)
  (add `/Game/ScrewMechanicsVR/Blueprints/BP_ScrewFixComponent.All Screws Released` (`self.ScrewsControlComponent`) (delegate `Turn On Physics Simulation`)))

(event `Turn On Physics Simulation`
  (`PrimitiveComponent.SetSimulatePhysics` (`self.StaticMeshComponent`) true) ; When all screws is released
)

(event `/Game/VirtualRealityBP/Blueprints/PickupActorInterface.Pickup`
  (params (AttachTo :type "SceneComponent Object Reference"))
  ;[1 1 1] Pickup and Drop
  ;;[0 1 0.00041] You can pick up this object only if all screws are released
  (if (`/Game/ScrewMechanicsVR/Blueprints/BP_ScrewFixComponent.Free of Screws` (`self.ScrewsControlComponent`))
    (`PrimitiveComponent.SetSimulatePhysics` (`self.StaticMeshComponent`) false)
    (`SceneComponent.K2_AttachToComponent` (`self.K2_GetRootComponent`) AttachTo "None" "KeepWorld" "KeepWorld" "KeepWorld" false)))

(event `/Game/VirtualRealityBP/Blueprints/PickupActorInterface.Drop`
  ;[1 1 1] Pickup and Drop
  (`PrimitiveComponent.SetSimulatePhysics` (`self.StaticMeshComponent`) true)
  (`self.K2_DetachFromActor` "KeepWorld" "KeepWorld" "KeepWorld"))

(fn `UserConstructionScript`)