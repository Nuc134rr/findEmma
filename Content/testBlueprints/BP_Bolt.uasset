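; BP_Bolt is a test VR deadbolt whose lever state changes are passed on through DeadboltLockState.
; On BeginPlay it sets a VR rotation, keeping the Bolt's roll and pitch and computing yaw from transform vectors and the right motion controller's position.
; The cast supplying the Vive pawn for that math is never executed, and Tick is disabled.
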(event EventTick
  (params (DeltaSeconds :type Float%20%28single-precision%29)))

(event EventLeverStateChanged
  (params (LeverStatus :type Boolean) (LeverStatusType :type EVRInteractibleLeverEventType%20Enum :default "LeverPositive") (LeverAngleAtTime :type Float%20%28single-precision%29) (FullLeverAngleAttime :type Float%20%28single-precision%29))
  (Default|CallDeadboltLockState LeverStatus))

(event EventBeginPlay
  (bind _returnvalue (Math|Transform|TransformLocation))
  (bind _bolt (Variables|Default|GetBolt))
  (bind _returnvalue_2 (Math|Conversions|RotationFromXVector _returnvalue))
  (bind _returnvalue_3 (Transformation|GetWorldRotation _bolt))
  (bind _returnvalue_4 (Math|Vector|GetRightVector _returnvalue_2))
  (Class|VRBaseCharacter|SetActorRotationVR (Math|Rotator|MakeRotator (.roll _returnvalue_3) (.pitch _returnvalue_3) (+ (.Yaw (Math|Rotator|BreakRotator (Math|Conversions|RotationFromXVector _returnvalue))) (+ (.x (- (* _returnvalue _returnvalue_4) (* _returnvalue_4 (Transformation|GetWorldLocation (Variables|/Script/VRExpansionPlugin.VRBaseCharacter|GetRightMotionController (stale _asvive_pawn_character)))))) (.y (- (* _returnvalue _returnvalue_4) (* _returnvalue_4 (Transformation|GetWorldLocation (Variables|/Script/VRExpansionPlugin.VRBaseCharacter|GetRightMotionController (stale _asvive_pawn_character))))))))) true true))