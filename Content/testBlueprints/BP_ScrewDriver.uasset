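; VR screwdriver that can be picked up and used to turn BP_Screw actors.
; While held, Tick attaches it to a nearby unreleased screw of matching TypeID, blending relative transforms to ease the snap.
; Positive motion controller roll deltas feed the screw's rotation and trigger periodic sound and rumble.
; It blends back into the hand when the screw releases or the controller-derived pointer moves too far away.
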(event `self.ReceiveTick`
  (params (DeltaSeconds :type "Float (single-precision)"))
  (if (`self.in hand`)
    (`|ExecutionSequence`
      (:`then_0`
        (if (`self.screw found`)
          (if (>= (`KismetMathLibrary.VSize` (- (`self.K2_GetActorLocation` (`self.active screw`)) (`self.ScrewDriverPointerLocation`))) (`self.Disconnect Distance`))
            ;[1 1 1] disconnect from screw in case of screwdriver
            (`SceneComponent.K2_AttachToComponent` (`self.K2_GetRootComponent`) (`self.active motion controller`) "None" "KeepWorld" "KeepWorld" "KeepWorld" false :!label _label)
            (set `self.screw found` false)
            (set `self.from Transform` (`SceneComponent.GetRelativeTransform` (`self.K2_GetRootComponent`)))
            (set `self.to Transform` (`self.initial in hand Transform`))
            (set `self.Transform Blending Coeff` 0.0) ; Start Transform Blending
            (else
              (`|ExecutionSequence`
                (:`then_0`
                  ;[1 1 1] Make Screw Rotate and Move
                  (set `self.newRotation` (`self.MotionControllerRoll`))
                  (set `self.deltaRotation` (- (`self.startRotation`) (`self.newRotation`)))
                  (if (> (`self.deltaRotation`) 0.0)
                    (`self.RotationSoundAndVibration` (`self.deltaRotation`))
                    (bind _screw_out (`/Game/ScrewMechanicsVR/Blueprints/BP_Screw.Add Rotation Value` (`self.active screw`) (`self.deltaRotation`)))
                    (if _screw_out
                      (goto _label))))
                (:`then_1`
                  (set `self.startRotation` (`self.newRotation`))))))
          (else
            ;[1 1 1] Find a Screw to connect with
            (bind _outactors (`GameplayStatics.GetAllActorsOfClass` "/Game/ScrewMechanicsVR/Blueprints/BP_Screw.BP_Screw_C"))
            (for _array_element _outactors
              (if (and (`/Game/ScrewMechanicsVR/Blueprints/BP_Screw.is Screwed` _array_element) (== (`/Game/ScrewMechanicsVR/Blueprints/BP_Screw.type_ID` _array_element) (`self.type_ID`)))
                (if (<= (`KismetMathLibrary.VSize` (- (`self.K2_GetActorLocation` _array_element) (`self.ScrewDriverPointerLocation`))) (`self.Connection Distance`))
                  (set `self.active screw` _array_element)
                  (`self.K2_AttachToActor` (`self.active screw`) "None" "KeepWorld" "KeepWorld" "KeepWorld" false) ; Attach to Screw
                  (set `self.from Transform` (`SceneComponent.GetRelativeTransform` (`self.StaticMeshComponent`)))
                  (set `self.to Transform` (`KismetMathLibrary.MakeTransform` (0.0 0.0 0.0) (struct :`Pitch` 180.0)))
                  (set `self.Transform Blending Coeff` 0.0)
                  (set `self.screw found` true)
                  (set `self.startRotation` (`self.MotionControllerRoll`))))))))
      (:`then_1`
        ;[1 1 1] Blending between Transforms - do until active (TransformBlendingCoeff<0)
        (if (< (`self.Transform Blending Coeff`) 1.0)
          (set `self.Transform Blending Coeff` (`KismetMathLibrary.FInterpTo` (`self.Transform Blending Coeff`) 1.0 DeltaSeconds 10.0))
          (`SceneComponent.K2_SetRelativeTransform` (`self.K2_GetRootComponent`) (`KismetMathLibrary.TLerp` (`self.from Transform`) (`self.to Transform`) (`self.Transform Blending Coeff`)) false false))))))

(event `RumbleController`
  (params (Intensity :type "Float (double-precision)"))
  (bind _returnvalue (select `EControllerHand` "Left" :`Left` true))
  (bind _returnvalue_2 (not _returnvalue))
  ;[1 1 1] Rumble Controller
  (`PlayerController.PlayDynamicForceFeedback` (`GameplayStatics.GetPlayerController` 0) Intensity 0.04 _returnvalue _returnvalue _returnvalue_2 _returnvalue_2))

(event `/Game/VirtualRealityBP/Blueprints/PickupActorInterface.Pickup`
  (params (AttachTo :type "SceneComponent Object Reference"))
  ;[1 1 1] "Standard" Pickup and Drow - using interface from basic VR template
  (`PrimitiveComponent.SetSimulatePhysics` (`self.StaticMeshComponent`) false)
  (`SceneComponent.K2_AttachToComponent` (`self.K2_GetRootComponent`) AttachTo "None" "KeepWorld" "KeepWorld" "KeepWorld" false)
  (set `self.in hand` true)
  (bind _asmotion_controller_component (cast `MotionControllerComponent` AttachTo))
  (set `self.active motion controller` _asmotion_controller_component) ; remember MotionController
  (set `self.initial in hand Transform` (`SceneComponent.GetRelativeTransform` (`self.K2_GetRootComponent`))) ; Remember initial transform
  (set `self.Transform Blending Coeff` 1.0) ; no transform blending
)

(event `/Game/VirtualRealityBP/Blueprints/PickupActorInterface.Drop`
  ;[1 1 1] "Standard" Pickup and Drow - using interface from basic VR template
  (`PrimitiveComponent.SetSimulatePhysics` (`self.StaticMeshComponent`) true)
  (`self.K2_DetachFromActor` "KeepWorld" "KeepWorld" "KeepWorld")
  (set `self.in hand` false)
  (set `self.screw found` false)
  (set `self.active motion controller` null)
  (set `self.active screw` null))

(fn `RotationSoundAndVibration`
  (params (`Rotation Amount` :type "Float (double-precision)"))
  ;[1 1 1] Function play the sound and activate vibration while player rotating screwdriver
  (bind _output_get (set `self.rotation to sound` (+ `Rotation Amount` (`self.rotation to sound`))))
  (if (> _output_get (`self.SoundAndVibrationEvery`))
    (set `self.rotation to sound` 0.0)
    ;;[0 1 0.000169] SOUND
    (`GameplayStatics.PlaySound2D` "/Game/ScrewMechanicsVR/Sounds/ScrewRotationSound.ScrewRotationSound" 1.0 1.0 0.0 null null)
    ;;[0 1 0.000169] VIBRATION
    (`self.RumbleController` 0.7)))

(fn `UserConstructionScript`)