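; VR radio tuning task with two grippable dials that drive a wave material on the radio.
; Each dial snap maps both angles through lookup arrays to wave speed and period, then plays a sound if they equal check values.
; BeginPlay plays a sound and randomizes both wave parameters, but nothing here sets the check values.
; Task completion, dial lockout, scoring and reset exist but are disconnected.
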(event `self.Dial_L.OnDialHitSnapAngle`
  (params (DialMilestoneAngle :type "Float (single-precision)"))
  ;[1 1 1] Scale
  (`self.RandomizeWaves`))

(event `self.Dial_R.OnDialHitSnapAngle`
  (params (DialMilestoneAngle :type "Float (single-precision)"))
  ;[1 1 1] Scale
  (`self.RandomizeWaves`))

(event `RandomizeWaves`
  (bind _radio_base (`self.Radio Base`))
  (bind _output (`|GetArrayItem` (`|MakeArray` 0.5 1.0 1.5 2.0 2.5 3.0 3.5 4.0 4.5 5.0 :!type "Float (single-precision)") (`KismetMathLibrary.FTrunc` (/ (`VRDialComponent.CurrentDialAngle` (`self.Dial_R`)) 20.0))))
  (bind _output_2 (`|GetArrayItem` (`|MakeArray` 0.15 0.2 0.35 0.3 0.4 0.25 0.1 0.45 0.05 0.5 :!type "Float (single-precision)") (`KismetMathLibrary.FTrunc` (/ (`VRDialComponent.CurrentDialAngle` (`self.Dial_L`)) 20.0))))
  ;[1 1 1] Scale
  (`MeshComponent.SetScalarParameterValueOnMaterials` _radio_base "SpeedWave" _output_2)
  (`MeshComponent.SetScalarParameterValueOnMaterials` _radio_base "TargetPeriodWave" _output)
  (set `self.Dial L ` _output_2)
  (set `self.Dial R` _output)
  (`self.Check`))

(event `Reset`
  ;[1 1 1] Scale
  (`VRDialComponent.SetDialAngle` (`self.Dial_L`) 0.0 false)
  (`VRDialComponent.SetDialAngle` (`self.Dial_R`) 0.0 false)
  (`VRDialComponent.ResetInitialDialLocation` (`self.Dial_L`))
  (`VRDialComponent.ResetInitialDialLocation` (`self.Dial_R`))
  (`self.RandomizeWaves`))

(event `Check`
  ;[1 1 1] Check
  (if (and (== (`self.Dial L `) (`self.Dial L Check`)) (== (`self.Dial R`) (`self.Dial R Check`)))
    (`GameplayStatics.PlaySoundAtLocation` null (`SceneComponent.K2_GetComponentLocation` (`self.Cube1`)) (struct) 3.0 1.0 0.0 null null null)))

(event `self.ReceiveBeginPlay`
  ;[1 1 1] Set Win Condition
  (`GameplayStatics.PlaySoundAtLocation` null (`SceneComponent.K2_GetComponentLocation` (`self.Radio Base`)) (struct) 2.0 1.0 0.0 null null null)
  (`self.Win`))

(event `Win`
  (bind _radio_base (`self.Radio Base`))
  ;[1 1 1] Set Win Condition
  (`MeshComponent.SetScalarParameterValueOnMaterials` _radio_base "TargetPeriodWave" (`KismetArrayLibrary.Array_Random` (`|MakeArray` 0.5 1.0 1.5 2.0 2.5 3.0 3.5 4.0 4.5 :!type "Float (single-precision)")))
  (`MeshComponent.SetScalarParameterValueOnMaterials` _radio_base "SpeedWave" (`KismetArrayLibrary.Array_Random` (`|MakeArray` 0.15 0.2 0.35 0.3 0.4 0.25 0.1 0.45 0.05 :!type "Float (single-precision)"))))

(event `DenyGripAll`
  (set `VRDialComponent.bDenyGripping` true (`self.Dial_R`))
  (set `VRDialComponent.bDenyGripping` true (`self.Dial_L`))
  (for _array_element (`|MakeArray` (`self.Dial_R`) (`self.Dial_L`))
    (`KismetSystemLibrary.Delay` 0.1)
    (`GripMotionControllerComponent.DropComponent` (`self.Gripping Controller`) _array_element false (0.0 0.0 0.0) (0.0 0.0 0.0))))

(event `self.Dial_L.OnGripped`
  (params (GrippingController :type "GripMotionControllerComponent Object Reference") (GripInformation :type "BPActorGripInformation Structure (by ref)"))
  (if (not (and (== (`VRDialComponent.CurrentDialAngle` (`self.Dial_R`)) (`self.Dial R Check`)) (== (`VRDialComponent.CurrentDialAngle` (`self.Dial_L`)) (`self.Dial L Check`))))
    (set `self.Gripping Controller` GrippingController)))

(event `self.Dial_R.OnGripped`
  (params (GrippingController :type "GripMotionControllerComponent Object Reference") (GripInformation :type "BPActorGripInformation Structure (by ref)"))
  (if (not (and (== (`VRDialComponent.CurrentDialAngle` (`self.Dial_R`)) (`self.Dial R Check`)) (== (`VRDialComponent.CurrentDialAngle` (`self.Dial_L`)) (`self.Dial L Check`))))
    (set `self.Gripping Controller` GrippingController)))

(fn `UserConstructionScript`)