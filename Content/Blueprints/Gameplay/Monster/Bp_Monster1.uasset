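; Monster actor that chases and faces TestBP actors it can see.
; Every tick, and once on BeginPlay, it loops over actors currently perceived by AI sight and casts each to TestBP.
; For each match it issues AIMoveTo toward that actor and sets its own yaw from a look-at rotation.
; A debug print and loop break are left unconnected.
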(event `self.ReceiveTick`
  (params (DeltaSeconds :type "Float (single-precision)"))
  (for _array_element (`AIPerceptionComponent.GetCurrentlyPerceivedActors` (`self.AIPerception`) "/Script/AIModule.AISense_Sight") :!label _label
    (bind _astest_bp (cast `/Game/Developers/ceroni/Collections/TestBP` _array_element))
    (bind _returnvalue (`self.K2_GetActorLocation` _astest_bp))
    (`|AIMoveTo` self _returnvalue _astest_bp
      (:`then`
        (bind (_returnvalue_roll _returnvalue_pitch _returnvalue_yaw) (`KismetMathLibrary.BreakRotator` (`KismetMathLibrary.FindLookAtRotation` (`self.K2_GetActorLocation`) _returnvalue)))
        (`self.K2_SetActorRotation` (`KismetMathLibrary.MakeRotator` 0.0 0.0 _returnvalue_yaw))))))

(event `self.ReceiveBeginPlay`
  (goto _label))

(fn `UserConstructionScript`)