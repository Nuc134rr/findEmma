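; BP_Emma runs one-time VR flashbacks for Emma, triggered by Paper, Mug and Floppy events.
; Mug and Floppy store the player's transform, teleport them to a room, briefly spawn a prop, play a fade-out sequence and return them turned 180 degrees.
; Paper only stores the transform, as its remaining sequence is disconnected.
; A helper returns its controller and a goal offset from the player's VR head.
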(event `self.ReceiveBeginPlay`
  ;[1 1 1] Day Check
  (`KismetSystemLibrary.Delay` 1.0)
  (bind _asbp_player_character (cast `/Game/Blueprints/Core/BP_PlayerCharacter` (`GameplayStatics.GetPlayerPawn` 0))
    (:`then`
      (set `self.Player` _asbp_player_character))
    (:`CastFailed`
      (`KismetSystemLibrary.PrintString` "player not set"))))

(event `PaperFlashback`
  (bind _rootcomponent (`Actor.RootComponent` (`self.Player`)))
  (bind (_returnvalue_roll _returnvalue_pitch _returnvalue_yaw) (`KismetMathLibrary.BreakRotator` (`SceneComponent.K2_GetComponentRotation` _rootcomponent)))
  ;[1 1 1] Paper Flashback
  (if (not (`self.paper`))
    (if true
      _
      (else
        _))
    (set `self.Baseloc` (`SceneComponent.K2_GetComponentLocation` _rootcomponent))
    (set `self.Baserot` (`KismetMathLibrary.MakeRotator` _returnvalue_roll _returnvalue_pitch (+ _returnvalue_yaw 180.0)))))

(event `MugFlashback`
  (bind (_returnvalue_location _returnvalue_rotation _returnvalue_scale) (`KismetMathLibrary.BreakTransform` (`SceneComponent.K2_GetComponentToWorld` (`self.StaticMesh`))))
  (bind _rootcomponent (`Actor.RootComponent` (`self.Player`)))
  (bind (_returnvalue_roll _returnvalue_pitch _returnvalue_yaw) (`KismetMathLibrary.BreakRotator` (`SceneComponent.K2_GetComponentRotation` _rootcomponent)))
  ;[1 1 1] Mug Flashback
  (if (not (`self.mug`))
    (if true
      _
      (else
        _))
    (set `self.Baseloc` (`SceneComponent.K2_GetComponentLocation` _rootcomponent))
    (set `self.Baserot` (`KismetMathLibrary.MakeRotator` _returnvalue_roll _returnvalue_pitch (+ _returnvalue_yaw 180.0)))
    (`VRBaseCharacter.SetActorLocationAndRotationVR` (`self.Player`) (`self.Roomloc`) (struct :`Yaw` 270.0) false true false)
    (`KismetSystemLibrary.Delay` 5.0)
    (bind _returnvalue (`|SpawnActorFromClass` "/Game/Blueprints/Gameplay/Flashbacks/FlashbackItems/BP_flashbackMug.BP_flashbackMug_C" (`KismetMathLibrary.MakeTransform` (+ _returnvalue_location (0.0 100.0 0.0)) _returnvalue_rotation _returnvalue_scale) "Undefined" "OverrideRootScale" null null))
    (`KismetSystemLibrary.Delay` 3.0)
    (bind _outactor (`LevelSequencePlayer.CreateLevelSequencePlayer` "/Game/Blueprints/Gameplay/Flashbacks/FlashbackItems/Sequences/LS_FadeOut_Flashback.LS_FadeOut_Flashback"))
    (`MovieSceneSequencePlayer.Play` (`LevelSequenceActor.SequencePlayer` _outactor))
    (`self.K2_DestroyActor` _returnvalue)
    (`VRBaseCharacter.SetActorLocationAndRotationVR` (`self.Player`) (`self.Baseloc`) (`self.Baserot`) true false true)
    (set `self.mug` true)))

(event `FloppyFlashback`
  (bind (_returnvalue_location _returnvalue_rotation _returnvalue_scale) (`KismetMathLibrary.BreakTransform` (`SceneComponent.K2_GetComponentToWorld` (`self.StaticMesh`))))
  (bind _rootcomponent (`Actor.RootComponent` (`self.Player`)))
  (bind (_returnvalue_roll _returnvalue_pitch _returnvalue_yaw) (`KismetMathLibrary.BreakRotator` (`SceneComponent.K2_GetComponentRotation` _rootcomponent)))
  ;[1 1 1] Floppy Flashback
  (if (not (`self.floppy`))
    (if true
      _
      (else
        _))
    (set `self.Baseloc` (`SceneComponent.K2_GetComponentLocation` _rootcomponent))
    (set `self.Baserot` (`KismetMathLibrary.MakeRotator` _returnvalue_roll _returnvalue_pitch (+ _returnvalue_yaw 180.0)))
    (`VRBaseCharacter.SetActorLocationAndRotationVR` (`self.Player`) (`self.Roomloc`) (struct :`Yaw` 270.0) false true false)
    (`KismetSystemLibrary.Delay` 5.0)
    (bind _returnvalue (`|SpawnActorFromClass` "/Game/Blueprints/Gameplay/Flashbacks/FlashbackItems/BP_floppy.BP_floppy_C" (`KismetMathLibrary.MakeTransform` (+ _returnvalue_location (0.0 100.0 0.0)) _returnvalue_rotation _returnvalue_scale) "Undefined" "OverrideRootScale" null null))
    (`KismetSystemLibrary.Delay` 3.0)
    (bind _outactor (`LevelSequencePlayer.CreateLevelSequencePlayer` "/Game/Blueprints/Gameplay/Flashbacks/FlashbackItems/Sequences/LS_FadeOut_Flashback.LS_FadeOut_Flashback"))
    (`MovieSceneSequencePlayer.Play` (`LevelSequenceActor.SequencePlayer` _outactor))
    (`self.K2_DestroyActor` _returnvalue)
    (`VRBaseCharacter.SetActorLocationAndRotationVR` (`self.Player`) (`self.Baseloc`) (`self.Baserot`) true false true)
    (set `self.floppy` true)))

(fn `GetGoalLocation`
  (returns (Controller :type "Controller Object Reference") (Goal :type "Vector Structure"))
  (bind _output_get (set `self.Goal` (+ (`VRBaseCharacter.K2_GetVRHeadLocation` (cast `/Game/Blueprints/Core/BP_PlayerCharacter` (`GameplayStatics.GetPlayerPawn` 0) :!pure true)) (`self.Offset`))))
  (return (`self.GetController`) _output_get))

(fn `UserConstructionScript`)