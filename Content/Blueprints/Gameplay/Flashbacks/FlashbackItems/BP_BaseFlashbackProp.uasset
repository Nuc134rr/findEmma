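; Base flashback prop that triggers a flashback when the player grips it in VR.
; On grip, if flashbacks are allowed and gripping is not denied, it sends a flashback type message, fixed to the dirt mug, to the player pawn and Emma.
; It then flags the Vive pawn as gripping a flashback and denies further gripping.
; The Emma reference is found by class search at BeginPlay.
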(event `VRGripInterface.OnGrip`
  (params (GrippingController :type "GripMotionControllerComponent Object Reference") (GripInformation :type "BPActorGripInformation Structure (by ref)"))
  (bind _returnvalue (`GameplayStatics.GetPlayerPawn` 0))
  (if (`self.bCanTriggerFlashback`)
    (bind _returnvalue_2 (`VRGripInterface.DenyGripping` null))
    (if (not _returnvalue_2)
      (message `/Game/Blueprints/Gameplay/Flashbacks/FlashbackItems/I_Flashbacks.FlashbackType` _returnvalue "/Game/Blueprints/Gameplay/Flashbacks/FlashbackItems/BP_dirtMug.BP_dirtMug")
      (message `/Game/Blueprints/Gameplay/Flashbacks/FlashbackItems/I_Flashbacks.FlashbackType` (stale `self.ReceiveBeginPlay` _output_get) "/Game/Blueprints/Gameplay/Flashbacks/FlashbackItems/BP_dirtMug.BP_dirtMug")
      (set `/Game/PluginContent/VRExpansion/Vive/Vive_PawnCharacter.bIsFlashbackGripped` true (cast `/Game/PluginContent/VRExpansion/Vive/Vive_PawnCharacter` _returnvalue :!pure true))
      (`self.SetDenyGripping` true))))

(event `self.ReceiveBeginPlay`
  (bind _outactors (`GameplayStatics.GetAllActorsOfClass` "/Game/Blueprints/Gameplay/Flashbacks/Emma/BP_Emma.BP_Emma_C"))
  (for _array_element _outactors
    (bind _output_get (set `self.EmmaRef` _array_element))))

(fn `UserConstructionScript`)