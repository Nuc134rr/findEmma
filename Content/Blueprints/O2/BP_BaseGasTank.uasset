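; Base grippable gas canister for the O2 task, in one of three colors (red, yellow, blue) set per instance.
; The construction script and BeginPlay both match the color against an array to pick the mesh material, with BeginPlay also storing the index.
; Gripping has the O2 task show holographic canisters for that index; releasing hides them and, if flagged as socketed, disables physics and further gripping.
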(event `self.ReceiveBeginPlay`
  (`self.Set Color Of Canister`))

(event `VRGripInterface.OnGrip`
  (params (GrippingController :type "GripMotionControllerComponent Object Reference") (GripInformation :type "BPActorGripInformation Structure (by ref)"))
  (`/Game/Blueprints/O2/O2_Task.Create Holographic Canisters` (`self.O2TaskRef`) (`self.Color Number`)))

(event `VRGripInterface.OnGripRelease`
  (params (ReleasingController :type "GripMotionControllerComponent Object Reference") (GripInformation :type "BPActorGripInformation Structure (by ref)") (bWasSocketed :type Boolean))
  (`/Game/Blueprints/O2/O2_Task.Hide Holographic Canisters` (`self.O2TaskRef`))
  ;[1 1 1] Of socketed, ignore physics and gripping (Set bIsSocketed in O2 Task)
  (if (`self.bIsSocketed`)
    (`PrimitiveComponent.SetSimulatePhysics` (`self.StaticMeshComponent`) false)
    (`self.SetDenyGripping` true)))

(fn `Set Color Of Canister`
  (locals (WhichColor :type Integer))
  ;[1 1 1] Sets color of canister (Set through Instance Editable)
  (for (_array_element _array_index) (`self.ColorArray`)
    (if (`KismetStringLibrary.EqualEqual_StrStr` _array_element (`self.Color`))
      (set `self.Color Number` _array_index)))
  (`PrimitiveComponent.SetMaterial` (`self.StaticMeshComponent`) 0 (select `int` (`self.Color Number`) :`0` "/Game/Assets/Tasks/OxygenPipes/Materials/cannister_red.cannister_red" :`1` "/Game/Assets/Tasks/OxygenPipes/Materials/cannister_yellow.cannister_yellow" :`2` "/Game/Assets/Tasks/OxygenPipes/Materials/cannister_blue.cannister_blue" :!type "MaterialInterface Object Reference")))

(fn `UserConstructionScript`
  (locals (WhichColor :type Integer))
  ;[1 1 1] Sets color of canister (Set through Instance Editable)
  (for (_array_element _array_index) (`self.ColorArray`)
    (if (`KismetStringLibrary.EqualEqual_StrStr` _array_element (`self.Color`))
      (set `local.WhichColor` _array_index)))
  (`PrimitiveComponent.SetMaterial` (`self.StaticMeshComponent`) 0 (select `int` (`local.WhichColor`) :`0` "/Game/Assets/Tasks/OxygenPipes/Materials/cannister_red.cannister_red" :`1` "/Game/Assets/Tasks/OxygenPipes/Materials/cannister_yellow.cannister_yellow" :`2` "/Game/Assets/Tasks/OxygenPipes/Materials/cannister_blue.cannister_blue" :!type "MaterialInterface Object Reference")))