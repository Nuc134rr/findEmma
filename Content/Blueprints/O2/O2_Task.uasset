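; O2 puzzle task, enabled by a GameInstance flag, where height fog thickens over time once activated until solved.
; Matching red, yellow and blue gas tanks lerp into sockets via timelines on overlap and attach, with holographic placement hints.
; Gripping valves starts a looping Checker timer that drives dials and tests valve pairs for purple and green.
; Achieving both plays a ding, locks valves, completes the notebook task and clears fog.
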(event `self.ReceiveBeginPlay`
  ;[1 0 0] Check if should activate in level
  ;;[1 0 0.4] Reset Fog
  (`ExponentialHeightFogComponent.SetFogDensity` (`self.ExponentialHeightFog`) 0.0)
  ;;[1 0 0.5] Create Arrays for Simplicity
  (`|ExecutionSequence`
    (:`then_0`
      (set `self.CanSocketedArray` (`|MakeArray` (`self.bRedCanSocketed`) (`self.bYellowCanSocketed`) (`self.bBlueCanSocketed`))))
    (:`then_1`
      (set `self.Holo Canister Array` (`|MakeArray` (`self.RedHoloCanister`) (`self.YellowHoloCanister`) (`self.BlueHoloCanister`))))
    (:`then_2`
      ;;[1 0 0.5] Should task be able to activate
      (if (`/Game/Blueprints/GameInstances_and_GameModes/BP_EmmaInstance_GI.Gas Canister` (cast `/Game/Blueprints/GameInstances_and_GameModes/BP_EmmaInstance_GI` (`GameplayStatics.GetGameInstance`) :!pure true))
        (set `self.CanActivate` true)
        ;;;[0 0 0] TEMPORARY
        (`KismetSystemLibrary.PrintString` "Activate O2")
        (else
          (`self.DenyGrippingAll`))))))

(event `self.ReceiveTick`
  (params (DeltaSeconds :type "Float (single-precision)"))
  (bind _returnvalue (+ (`self.Delta Seconds`) (`self.O2 Timer`)))
  ;[0 0 1] Event Tick
  (set `self.Delta Seconds` DeltaSeconds)
  ;[0 0 1] Add Delta Seconds to O2 Timer if Activated
  (`/Engine/EditorBlueprintResources/StandardMacros.Gate` true :!label _label
    (:`Exit`
      ;;[0 0.5 1] Set and Check Timer
      (if (>= _returnvalue 1000.0)
        ;;[0 0.5 1] Max Time
        (set `self.O2 Timer` 1000.0)
        (else
          (set `self.O2 Timer` _returnvalue)))
      ;[0 0 1] Set Fog Density
      (`ExponentialHeightFogComponent.SetFogDensity` (`self.ExponentialHeightFog`) (* (/ (`self.O2 Timer`) 1000.0) 1.5) :!label _label_2))))

(event `Activate O2 Task`
  ;[0 0 1] Add Delta Seconds to O2 Timer if Activated
  ;;[0 0.5 1 0.997] Activates Task Timer
  (if (`self.CanActivate`)
    (goto _label :!via `Open`)))

(event `Remove Fog`
  ;[0 0 1] Add Delta Seconds to O2 Timer if Activated
  (set `self.O2 Timer` 0.0)
  (`|ExecutionSequence`
    (:`then_0`
      (goto _label :!via `Close`))
    (:`then_1`
      (goto _label_2))))

(event `self.RedCanisterCollision.OnComponentBeginOverlap`
  (params (OverlappedComponent :type "PrimitiveComponent Object Reference") (OtherActor :type "Actor Object Reference") (OtherComp :type "PrimitiveComponent Object Reference") (OtherBodyIndex :type Integer) (bFromSweep :type Boolean) (SweepResult :type "HitResult Structure (by ref)"))
  (bind _as_bp_base_gas_tank_red (`self.As BP Base Gas Tank Red`))
  (bind _staticmeshcomponent (`self.StaticMeshComponent`))
  (bind _output (`|GetArrayItem` (`self.Holo Canister Array`) (`self.Canister Socket Number`)))
  ;[1 0 1] Attatch Corresponding Valve with Corresponding Canister on Overlap
  ;;[1 0.25 0.75] Checks Gas Tank and if corresponding color, then tells cannister that its socketed (Locking Position)
  (bind _asbp_base_gas_tank (cast `/Game/Blueprints/O2/BP_BaseGasTank` OtherActor))
  (if (== OtherComp (`/Game/Blueprints/O2/BP_BaseGasTank.Box` _asbp_base_gas_tank))
    (if (`KismetStringLibrary.EqualEqual_StrStr` (`/Game/Blueprints/O2/BP_BaseGasTank.Color` _asbp_base_gas_tank) "Red")
      (set `self.As BP Base Gas Tank Red` _asbp_base_gas_tank)
      (set `self.StartLocationRed` (`self.K2_GetActorLocation` (`self.As BP Base Gas Tank Red`)))
      (set `self.StartRotationRed` (`self.K2_GetActorRotation` (`self.As BP Base Gas Tank Red`)))
      (set `self.Canister Socket Number` 0)
      (set `/Game/Blueprints/O2/BP_BaseGasTank.bIsSocketed` true (`self.As BP Base Gas Tank Red`))
      ;;[1 1 1] Transition from location to socket location
      (`/Engine/EditorBlueprintResources/StandardMacros.DoOnce` false
        (:`Completed`
          (bind (_direction _newtrack_0) (`Timeline|TransitionRed` :!via `PlayFromStart`)
            (:`Update`
              (`self.K2_SetActorLocationAndRotation` _as_bp_base_gas_tank_red (`KismetMathLibrary.VLerp` (`self.StartLocationRed`) (`SceneComponent.GetSocketLocation` _staticmeshcomponent "RedCanister") _newtrack_0) (`KismetMathLibrary.RLerp` (`self.StartRotationRed`) (`SceneComponent.GetSocketRotation` _staticmeshcomponent "RedCanister") _newtrack_0 true) false false)
              (`KismetSystemLibrary.PrintString` (`KismetSystemLibrary.GetDisplayName` _as_bp_base_gas_tank_red)))
            (:`Finished`
              ;;[1 0.25 0.75] Attatch to actor
              (`self.K2_AttachToActor` (`self.As BP Base Gas Tank Red`) self "RedCanister" "SnapToTarget" "SnapToTarget" "KeepRelative" true)
              (`|ExecutionSequence` :!label _label_3
                (:`then_0`
                  ;;[1 0.25 0.75] Set visibility of indicator to invisible
                  (`SceneComponent.SetVisibility` _output false false))
                (:`then_1`
                  ;;[1 0.25 0.75] Play Sound
                  (`GameplayStatics.PlaySoundAtLocation` "/Game/Audio/16Canister_his.16Canister_his" (`SceneComponent.K2_GetComponentLocation` _output) (struct) 3.0 (`KismetMathLibrary.RandomFloatInRange` 0.5 2.0) 0.0 null null null))
                (:`then_2`
                  ;;[1 0.25 0.75] Sets Variables
                  (`|VariableSetRef` (`|GetArrayItem` (`self.CanSocketedArray`) (`self.Canister Socket Number`)) true))))))))))

(event `self.YellowCanisterCollision.OnComponentBeginOverlap`
  (params (OverlappedComponent :type "PrimitiveComponent Object Reference") (OtherActor :type "Actor Object Reference") (OtherComp :type "PrimitiveComponent Object Reference") (OtherBodyIndex :type Integer) (bFromSweep :type Boolean) (SweepResult :type "HitResult Structure (by ref)"))
  (bind _staticmeshcomponent (`self.StaticMeshComponent`))
  (bind _as_bp_base_gas_tank_yellow (`self.As BP Base Gas Tank Yellow`))
  ;[1 0 1] Attatch Corresponding Valve with Corresponding Canister on Overlap
  ;;[1 0.25 0.75] Checks Gas Tank and if corresponding color, then tells cannister that its socketed (Locking Position)
  (bind _asbp_base_gas_tank (cast `/Game/Blueprints/O2/BP_BaseGasTank` OtherActor))
  (if (== OtherComp (`/Game/Blueprints/O2/BP_BaseGasTank.Box` _asbp_base_gas_tank))
    (if (`KismetStringLibrary.EqualEqual_StrStr` (`/Game/Blueprints/O2/BP_BaseGasTank.Color` _asbp_base_gas_tank) "Yellow")
      (set `self.As BP Base Gas Tank Yellow` _asbp_base_gas_tank)
      (set `self.StartLocationYellow` (`self.K2_GetActorLocation` (`self.As BP Base Gas Tank Yellow`)))
      (set `self.StartRotationYellow` (`self.K2_GetActorRotation` (`self.As BP Base Gas Tank Yellow`)))
      (set `self.Canister Socket Number` 1)
      (set `/Game/Blueprints/O2/BP_BaseGasTank.bIsSocketed` true (`self.As BP Base Gas Tank Yellow`))
      ;;[1 1 1] Transition from location to socket location
      (`/Engine/EditorBlueprintResources/StandardMacros.DoOnce` false
        (:`Completed`
          (bind (_direction _newtrack_0) (`Timeline|Timeline_0` :!via `PlayFromStart`)
            (:`Update`
              (`self.K2_SetActorLocationAndRotation` _as_bp_base_gas_tank_yellow (`KismetMathLibrary.VLerp` (`self.StartLocationYellow`) (`SceneComponent.GetSocketLocation` _staticmeshcomponent "YellowCanister") _newtrack_0) (`KismetMathLibrary.RLerp` (`self.StartRotationYellow`) (`SceneComponent.GetSocketRotation` _staticmeshcomponent "YellowCanister") _newtrack_0 true) false false)
              (`KismetSystemLibrary.PrintString` (`KismetSystemLibrary.GetDisplayName` _as_bp_base_gas_tank_yellow)))
            (:`Finished`
              ;;[1 0.25 0.75] Attatch to actor
              (`self.K2_AttachToActor` (`self.As BP Base Gas Tank Yellow`) self "YellowCanister" "SnapToTarget" "SnapToTarget" "KeepRelative" true)
              (goto _label_3))))))))

(event `self.BlueCanisterCollision.OnComponentBeginOverlap`
  (params (OverlappedComponent :type "PrimitiveComponent Object Reference") (OtherActor :type "Actor Object Reference") (OtherComp :type "PrimitiveComponent Object Reference") (OtherBodyIndex :type Integer) (bFromSweep :type Boolean) (SweepResult :type "HitResult Structure (by ref)"))
  (bind _staticmeshcomponent (`self.StaticMeshComponent`))
  (bind _as_bp_base_gas_tank_blue (`self.As BP Base Gas Tank Blue`))
  ;[1 0 1] Attatch Corresponding Valve with Corresponding Canister on Overlap
  ;;[1 0.25 0.75] Checks Gas Tank and if corresponding color, then tells cannister that its socketed (Locking Position)
  (bind _asbp_base_gas_tank (cast `/Game/Blueprints/O2/BP_BaseGasTank` OtherActor))
  (if (== OtherComp (`/Game/Blueprints/O2/BP_BaseGasTank.Box` _asbp_base_gas_tank))
    (if (`KismetStringLibrary.EqualEqual_StrStr` (`/Game/Blueprints/O2/BP_BaseGasTank.Color` _asbp_base_gas_tank) "Blue")
      (set `self.As BP Base Gas Tank Blue` _asbp_base_gas_tank)
      (set `self.StartLocationBlue` (`self.K2_GetActorLocation` (`self.As BP Base Gas Tank Blue`)))
      (set `self.StartRotationBlue` (`self.K2_GetActorRotation` (`self.As BP Base Gas Tank Blue`)))
      (set `self.Canister Socket Number` 2)
      (set `/Game/Blueprints/O2/BP_BaseGasTank.bIsSocketed` true (`self.As BP Base Gas Tank Blue`))
      ;;[1 1 1] Transition from location to socket location
      (`/Engine/EditorBlueprintResources/StandardMacros.DoOnce` false
        (:`Completed`
          (bind (_direction _newtrack_0) (`Timeline|Timeline_1` :!via `PlayFromStart`)
            (:`Update`
              (`self.K2_SetActorLocationAndRotation` _as_bp_base_gas_tank_blue (`KismetMathLibrary.VLerp` (`self.StartLocationBlue`) (`SceneComponent.GetSocketLocation` _staticmeshcomponent "BlueCanister") _newtrack_0) (`KismetMathLibrary.RLerp` (`self.StartRotationBlue`) (`SceneComponent.GetSocketRotation` _staticmeshcomponent "BlueCanister") _newtrack_0 true) false false)
              (`KismetSystemLibrary.PrintString` (`KismetSystemLibrary.GetDisplayName` _as_bp_base_gas_tank_blue)))
            (:`Finished`
              ;;[1 0.25 0.75] Attatch to actor
              (`self.K2_AttachToActor` (`self.As BP Base Gas Tank Blue`) self "BlueCanister" "SnapToTarget" "SnapToTarget" "KeepRelative" true)
              (goto _label_3))))))))

(event `self.Valve_Blue2.OnGripped`
  (params (GrippingController :type "GripMotionControllerComponent Object Reference") (GripInformation :type "BPActorGripInformation Structure (by ref)"))
  (bind _notebookref (`self.notebookRef`))
  ;[0 1 0] Valve Check
  ;;[0.5 1 0] Makes Green
  ;;[0.5 1 0] Check Nozzle rotation every tiny interval of time, then stops when completed
  (`/Engine/EditorBlueprintResources/StandardMacros.DoOnce` false :!label _label_4
    (:`Completed`
      (bind _returnvalue (`KismetSystemLibrary.K2_SetTimer` null "Checker" 0.001 true))
      (if (and (stale `Check Purple` _output_get) (stale `Check Green` _output_get)) :!label _label_5
        (`KismetSystemLibrary.K2_ClearAndInvalidateTimerHandle` _returnvalue)
        ;;[0.5 1 0] Win Effects
        (`GameplayStatics.PlaySoundAtLocation` "/Game/Sound/ding.ding" (`SceneComponent.K2_GetComponentLocation` (`self.StaticMeshComponent`)) (struct) 3.0 1.0 0.0 null null null)
        (`self.DenyGrippingAll`)
        (`/Game/Blueprints/Props/BP_notebook.changeTextColorToComplete` _notebookref (`/Game/Blueprints/Props/BP_notebook.Task1` _notebookref) 0)
        (`self.Remove Fog`)))))

(event `self.Valve_Yellow.OnGripped`
  (params (GrippingController :type "GripMotionControllerComponent Object Reference") (GripInformation :type "BPActorGripInformation Structure (by ref)"))
  ;[0 1 0] Valve Check
  ;;[0.5 1 0] Makes Green
  (goto _label_4))

(event `Check Purple`
  ;[0 1 0] Valve Check
  ;;[0.5 1 0] Check Nozzle rotation every tiny interval of time, then stops when completed
  (if (and (>= (/ (`VRDialComponent.CurrentDialAngle` (`self.Valve_Red`)) 4.0) 80.0) (>= (/ (`VRDialComponent.CurrentDialAngle` (`self.Valve_Blue1`)) 4.0) 80.0))
    (bind _output_get (set `self.Purple` true))
    (goto _label_5)))

(event `Check Green`
  ;[0 1 0] Valve Check
  ;;[0.5 1 0] Check Nozzle rotation every tiny interval of time, then stops when completed
  (if (and (>= (/ (`VRDialComponent.CurrentDialAngle` (`self.Valve_Yellow`)) 4.0) 80.0) (>= (/ (`VRDialComponent.CurrentDialAngle` (`self.Valve_Blue2`)) 4.0) 80.0))
    (bind _output_get (set `self.Green` true))
    (goto _label_5)))

(event `self.Valve_Blue1.OnGripped`
  (params (GrippingController :type "GripMotionControllerComponent Object Reference") (GripInformation :type "BPActorGripInformation Structure (by ref)"))
  ;[0 1 0] Valve Check
  ;;[0.5 1 0] Makes Purple
  (goto _label_4))

(event `self.Valve_Red.OnGripped`
  (params (GrippingController :type "GripMotionControllerComponent Object Reference") (GripInformation :type "BPActorGripInformation Structure (by ref)"))
  ;[0 1 0] Valve Check
  ;;[0.5 1 0] Makes Purple
  (goto _label_4))

(event `Create Holographic Canisters`
  (params (`Color Number` :type Integer))
  ;[0 1 1] Holocanister Visibility
  ;;[0.5 1 1] (Called by BP_BaseGasTank when gripped) Sets corresponding Holocanister visible
  (`SceneComponent.SetVisibility` (select `int` `Color Number` :`0` (`self.RedHoloCanister`) :`1` (`self.YellowHoloCanister`) :`2` (`self.BlueHoloCanister`) :!type "SceneComponent Object Reference") true false))

(event `Hide Holographic Canisters`
  ;[0 1 1] Holocanister Visibility
  ;;[0.5 1 1] Called by BP_BaseGasTank when released) Sets Holocanisters invisible
  (`SceneComponent.SetVisibility` (`self.RedHoloCanister`) false false)
  (`SceneComponent.SetVisibility` (`self.YellowHoloCanister`) false false)
  (`SceneComponent.SetVisibility` (`self.BlueHoloCanister`) false false))

(event `DenyGrippingAll`
  ;[1 1 0] Enables gripping and disables gripping of valves
  (set `VRDialComponent.bDenyGripping` true (`self.Valve_Red`))
  (set `VRDialComponent.bDenyGripping` true (`self.Valve_Yellow`))
  (set `VRDialComponent.bDenyGripping` true (`self.Valve_Blue2`))
  (set `VRDialComponent.bDenyGripping` true (`self.Valve_Blue1`)))

(event `AllowGrippingAll`
  ;[1 1 0] Enables gripping and disables gripping of valves
  (set `VRDialComponent.bDenyGripping` false (`self.Valve_Red`))
  (set `VRDialComponent.bDenyGripping` false (`self.Valve_Yellow`))
  (set `VRDialComponent.bDenyGripping` false (`self.Valve_Blue2`))
  (set `VRDialComponent.bDenyGripping` false (`self.Valve_Blue1`)))

(fn `Checker`
  (bind _currentdialangle (`VRDialComponent.CurrentDialAngle` (`self.Valve_Blue2`)))
  (bind _currentdialangle_2 (`VRDialComponent.CurrentDialAngle` (`self.Valve_Blue1`)))
  (bind _returnvalue (`KismetMathLibrary.MakeRotator` (+ (/ (+ (/ _currentdialangle 4.0) (/ _currentdialangle_2 4.0)) -2.0) 45.0)))
  (`|ExecutionSequence`
    (:`then_0`
      (`self.Check Purple`)
      (`SceneComponent.K2_SetRelativeRotation` (`self.PurpleDial`) (`KismetMathLibrary.ComposeRotators` (struct) (`KismetMathLibrary.MakeRotator` (+ (/ (+ (/ (`VRDialComponent.CurrentDialAngle` (`self.Valve_Red`)) 4.0) (/ (`VRDialComponent.CurrentDialAngle` (`self.Valve_Blue1`)) 4.0)) -2.0) 45.0))) false false))
    (:`then_1`
      (`self.Check Green`)
      (`SceneComponent.K2_SetRelativeRotation` (`self.GreenDial`) (`KismetMathLibrary.ComposeRotators` (struct) (`KismetMathLibrary.MakeRotator` (+ (/ (+ (/ (`VRDialComponent.CurrentDialAngle` (`self.Valve_Yellow`)) 4.0) (/ (`VRDialComponent.CurrentDialAngle` (`self.Valve_Blue2`)) 4.0)) -2.0) 45.0))) false false))
    (:`then_2`
      (`SceneComponent.K2_SetRelativeRotation` (`self.Red_Dial`) (`KismetMathLibrary.ComposeRotators` (struct) (`KismetMathLibrary.MakeRotator` (+ (* (/ (`VRDialComponent.CurrentDialAngle` (`self.Valve_Red`)) 4.0) -1.0) 45.0))) false false))
    (:`then_3`
      (`SceneComponent.K2_SetRelativeRotation` (`self.Blue_Dial`) (`KismetMathLibrary.ComposeRotators` (struct) _returnvalue) false false)
      (`KismetSystemLibrary.PrintString` (`KismetStringLibrary.Conv_DoubleToString` _currentdialangle_2))
      (`KismetSystemLibrary.PrintString` (`KismetStringLibrary.Conv_DoubleToString` _currentdialangle))
      (`KismetSystemLibrary.PrintString` (`KismetStringLibrary.Conv_RotatorToString` _returnvalue)))
    (:`then_4`
      (`SceneComponent.K2_SetRelativeRotation` (`self.Yellow_Dial`) (`KismetMathLibrary.ComposeRotators` (struct) (`KismetMathLibrary.MakeRotator` (+ (* (/ (`VRDialComponent.CurrentDialAngle` (`self.Valve_Yellow`)) 4.0) -1.0) 45.0))) false false))))

(fn `CheckForBoxOverlap`)

(fn `UserConstructionScript`)

(fn `Which Color`
  (params (A :type String))
  (returns (Color :type String) (Integer :type Integer))
  (locals (Index :type Integer))
  (bind _index (`local.Index`))
  (bind _canistercolorarray (`self.CanisterColorArray`))
  (for (_array_element _array_index) _canistercolorarray
    (if (`KismetStringLibrary.EqualEqual_StrStr` A _array_element)
      (set `local.Index` _array_index)))
  (return (`|GetArrayItem` _canistercolorarray _index) _index))

(fn `WhichCanBeSocketed`
  (params (Index :type Integer))
  (locals (NewLocalVar_0 :type Boolean))
  (if (== Index 0)
    (set `self.bRedCanSocketed` true)
    (elif (== Index 1)
      (set `self.bBlueCanSocketed` true)
      (elif (== Index 2)
        (set `self.bYellowCanSocketed` true)))))