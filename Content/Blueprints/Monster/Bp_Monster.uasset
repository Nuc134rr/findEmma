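; VR monster actor that turns with the Vive player's stored rotation and dies when struck by BP_axe.
; A looping 0.01-second CheckHeight timer prints player distance, updates mesh yaw with an offset, and line-traces toward the player, incrementing AmountSeen whenever the hit actor is not the player.
; OnGrip stops the timer.
; An axe overlap, matched by display name, also stops it, ragdolls the mesh, sets IsDead and quits the game after a delay.
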(event `VRGripInterface.OnGrip`
  (params (GrippingController :type "GripMotionControllerComponent Object Reference") (GripInformation :type "BPActorGripInformation Structure (by ref)"))
  (`KismetSystemLibrary.K2_ClearAndInvalidateTimerHandle` (stale `Check Height Event` _returnvalue)))

(event `self.ReceiveBeginPlay`
  (`self.Check Height Event`))

(event `Check Height Event`
  (bind _returnvalue (`KismetSystemLibrary.K2_SetTimer` null "CheckHeight" 0.01 true)))

(event `self.Box.OnComponentBeginOverlap`
  (params (OverlappedComponent :type "PrimitiveComponent Object Reference") (OtherActor :type "Actor Object Reference") (OtherComp :type "PrimitiveComponent Object Reference") (OtherBodyIndex :type Integer) (bFromSweep :type Boolean) (SweepResult :type "HitResult Structure (by ref)"))
  (if (`KismetStringLibrary.EqualEqual_StrStr` (`KismetSystemLibrary.GetDisplayName` OtherActor) "BP_axe")
    (`KismetSystemLibrary.PrintString` "yes")
    (`KismetSystemLibrary.K2_ClearAndInvalidateTimerHandle` (stale `Check Height Event` _returnvalue))
    (`PrimitiveComponent.SetSimulatePhysics` (`self.SkeletalMeshComponent`) true)
    (set `self.bIsDead` true)
    (`KismetSystemLibrary.Delay` 5.0)
    (`KismetSystemLibrary.QuitGame` null "Quit" true)
    (else
      (`KismetSystemLibrary.PrintString` "no"))))

(fn `CheckHeight`
  (bind (_returnvalue_x _returnvalue_y) (`KismetMathLibrary.BreakVector` (`self.K2_GetActorLocation`)))
  (bind (_returnvalue_x_2 _returnvalue_y_2) (`KismetMathLibrary.BreakVector` (`self.K2_GetActorLocation` (`GameplayStatics.GetPlayerCharacter` 0))))
  (`KismetSystemLibrary.PrintString` (`KismetStringLibrary.Conv_DoubleToString` (+ (`KismetMathLibrary.Abs` (- _returnvalue_x_2 _returnvalue_x)) (`KismetMathLibrary.Abs` (- _returnvalue_y_2 _returnvalue_y)))))
  (`|ExecutionSequence`
    (:`then_0`
      (`SceneComponent.K2_SetRelativeRotation` (`self.SkeletalMeshComponent`) (`KismetMathLibrary.MakeRotator` (.roll (`/Game/PluginContent/VRExpansion/Vive/Vive_PawnCharacter.Rot` (cast `/Game/PluginContent/VRExpansion/Vive/Vive_PawnCharacter` (`GameplayStatics.GetPlayerPawn` 0) :!pure true))) (.pitch (`/Game/PluginContent/VRExpansion/Vive/Vive_PawnCharacter.Rot` (cast `/Game/PluginContent/VRExpansion/Vive/Vive_PawnCharacter` (`GameplayStatics.GetPlayerPawn` 0) :!pure true))) (- (.yaw (`/Game/PluginContent/VRExpansion/Vive/Vive_PawnCharacter.Rot` (cast `/Game/PluginContent/VRExpansion/Vive/Vive_PawnCharacter` (`GameplayStatics.GetPlayerPawn` 0) :!pure true))) 270.0)) false false))
    (:`then_1`
      (bind _outhit (`KismetSystemLibrary.LineTraceSingle` (`KismetMathLibrary.MakeVector` (.x (`self.K2_GetActorLocation`)) (.y (`self.K2_GetActorLocation`)) (+ (.z (`self.K2_GetActorLocation`)) 170.0)) (`KismetMathLibrary.MakeVector` (.x (`self.K2_GetActorLocation` (`GameplayStatics.GetPlayerCharacter` 0))) (.y (`self.K2_GetActorLocation` (`GameplayStatics.GetPlayerCharacter` 0))) (+ (.z (`self.K2_GetActorLocation` (`GameplayStatics.GetPlayerCharacter` 0))) 150.0)) "TraceTypeQuery1" true))
      (if (not (`KismetStringLibrary.EqualEqual_StrStr` (`KismetSystemLibrary.GetDisplayName` (`.HitActor` (`GameplayStatics.BreakHitResult` _outhit))) "Vive_PawnCharacter"))
        (set `self.Amount Seen` (+ (`self.Amount Seen`) 1))))))

(fn `UserConstructionScript`)