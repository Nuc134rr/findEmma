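; BP_Vent is a vent prop that plays a fan sound and unlocks a switchboard interaction flag.
; On BeginPlay it spawns the fan cue at the location of its fan plane.
; When the player pawn overlaps SwitchboardTrigger in the level at index 2 of the Vive pawn's LevelNames, it sets CanTurnOnSwitchboard to true, with no reset in this graph.
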(event `self.ReceiveBeginPlay`
  (`GameplayStatics.SpawnSoundAtLocation` "/Game/Assets/Tasks/Vent/SoundEffects/16Fan_Cue.16Fan_Cue" (`SceneComponent.K2_GetComponentLocation` (`self.VentFan_Plane`)) (struct) 1.0 1.0 0.0 null null))

(event `self.SwitchboardTrigger.OnComponentBeginOverlap`
  (params (OverlappedComponent :type "PrimitiveComponent Object Reference") (OtherActor :type "Actor Object Reference") (OtherComp :type "PrimitiveComponent Object Reference") (OtherBodyIndex :type Integer) (bFromSweep :type Boolean) (SweepResult :type "HitResult Structure (by ref)"))
  (bind _returnvalue (`GameplayStatics.GetPlayerPawn` 0))
  (bind _returnvalue_2 (`GameplayStatics.GetCurrentLevelName` true))
  (if (and (== OtherActor _returnvalue) (== (`KismetArrayLibrary.Array_Find` (`/Game/PluginContent/VRExpansion/Vive/Vive_PawnCharacter.Level_Names` (cast `/Game/PluginContent/VRExpansion/Vive/Vive_PawnCharacter` _returnvalue :!pure true)) _returnvalue_2) 2))
    (if (not (`self.CanTurnOnSwitchboard`))
      (set `self.CanTurnOnSwitchboard` true))))

(fn `UserConstructionScript`)