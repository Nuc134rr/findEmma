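; BP_Toilet is a toilet prop that flushes when its VR lever is pulled.
; Gripping the lever shows a Niagara effect and starts a looping timer that polls the lever angle through Flush.
; Past the angle threshold, Flushing swaps the Cube's material, then restores it to Blue after a delay.
; Dropping the lever clears the timer and hides the effect a few seconds later.
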(event `self.ReceiveBeginPlay`
  (`SceneComponent.SetVisibility` (`self.Niagara`) false false))

(event `self.VRLever.OnDropped`
  (params (GrippingController :type "GripMotionControllerComponent Object Reference") (GripInformation :type "BPActorGripInformation Structure (by ref)") (bWasSocketed :type Boolean))
  (`KismetSystemLibrary.K2_ClearAndInvalidateTimerHandle` (stale `self.VRLever.OnGripped` _returnvalue))
  (`KismetSystemLibrary.Delay` 4.0)
  (`SceneComponent.SetVisibility` (`self.Niagara`) false false))

(event `self.VRLever.OnGripped`
  (params (GrippingController :type "GripMotionControllerComponent Object Reference") (GripInformation :type "BPActorGripInformation Structure (by ref)"))
  (bind _returnvalue (`KismetSystemLibrary.K2_SetTimer` null "Flush" 0.2 true))
  (`SceneComponent.SetVisibility` (`self.Niagara`) true false))

(event `Flushing`
  (`PrimitiveComponent.SetMaterial` (`self.Cube`) 0 "/Game/Assets/Tasks/OxygenPipes/Materials/cannister_blue.cannister_blue")
  (`KismetSystemLibrary.Delay` 3.0)
  (`PrimitiveComponent.SetMaterial` (`self.Cube`) 0 "/Game/Miscellaneous/Materials/Blue.Blue"))

(fn `Flush`
  (bind _returnvalue (`VRLeverComponent.ReCalculateCurrentAngle` (`self.VRLever`) true))
  (if (> _returnvalue 30.0)
    (`self.Flushing`)))

(fn `UserConstructionScript`)