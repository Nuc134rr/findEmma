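; BP_FakeCan is a grippable VR can prop that completes a notebook task when tilted to a target angle.
; One second after BeginPlay, it denies gripping unless the current level is at index 1 of the pawn's LevelNames (day two).
; Gripping plays an opening sound and starts a looping timer that polls mesh roll against WinConditionAngle.
; A match swaps to the open mesh, stops the timer, marks Task1 complete and plays a sound.
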(event `self.ReceiveBeginPlay`
  (`KismetSystemLibrary.Delay` 1.0)
  (bind _returnvalue (`GameplayStatics.GetCurrentLevelName` true))
  (if (!= (`KismetArrayLibrary.Array_Find` (`/Game/PluginContent/VRExpansion/Vive/Vive_PawnCharacter.Level_Names` (cast `/Game/PluginContent/VRExpansion/Vive/Vive_PawnCharacter` (`GameplayStatics.GetPlayerPawn` 0) :!pure true)) _returnvalue) 1)
    (`KismetSystemLibrary.PrintString` "not day two LMAO")
    (`self.SetDenyGripping` true)))

(event `VRGripInterface.OnGrip`
  (params (GrippingController :type "GripMotionControllerComponent Object Reference") (GripInformation :type "BPActorGripInformation Structure (by ref)"))
  (bind _returnvalue (`KismetSystemLibrary.K2_SetTimer` null "CheckForAngle" 0.1 true))
  (`GameplayStatics.PlaySoundAtLocation` "/Game/Assets/Tasks/BeanCan/SoundEffects/16Can_opening.16Can_opening" (`SceneComponent.K2_GetComponentLocation` (`self.StaticMeshComponent`)) (struct) 1.0 1.0 0.0 null null null))

(event `WinCondition`
  (bind _notebookref (`self.notebookRef`))
  (`StaticMeshComponent.SetStaticMesh` (`self.StaticMeshComponent`) "/Game/Assets/Tasks/BeanCan/Meshes/can_open.can_open")
  (`KismetSystemLibrary.K2_ClearAndInvalidateTimerHandle` (stale `VRGripInterface.OnGrip` _returnvalue))
  (`/Game/Blueprints/Props/BP_notebook.changeTextColorToComplete` _notebookref (`/Game/Blueprints/Props/BP_notebook.Task1` _notebookref) 0)
  (`GameplayStatics.PlaySoundAtLocation` "/Game/Assets/Tasks/BeanCan/SoundEffects/16BEANS.16BEANS" (`SceneComponent.K2_GetComponentLocation` (`self.StaticMeshComponent`)) (struct) 1.0 1.0 0.0 null null null))

(fn `CheckForAngle`
  (if (`KismetMathLibrary.NearlyEqual_FloatFloat` (.roll (`SceneComponent.K2_GetComponentRotation` (`self.StaticMeshComponent`))) (`self.WinConditionAngle`) 10.0)
    (`self.WinCondition`)))

(fn `UserConstructionScript`)