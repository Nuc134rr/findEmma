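; Grass prop that falls apart when cut by the axe.
; On overlap with an actor whose display name is exactly "BP_axe", its grass components start simulating physics and switch to physics-only collision.
; After a short delay the whole actor destroys itself.
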(event `self.ReceiveActorBeginOverlap`
  (params (OtherActor :type "Actor Object Reference"))
  (if (`KismetStringLibrary.EqualEqual_StrStr` (`KismetSystemLibrary.GetDisplayName` OtherActor) "BP_axe")
    (`PrimitiveComponent.SetSimulatePhysics` (`self.Grass7`) true)
    (`PrimitiveComponent.SetSimulatePhysics` (`self.Grass12`) true)
    (`PrimitiveComponent.SetSimulatePhysics` (`self.Grass11`) true)
    (`PrimitiveComponent.SetSimulatePhysics` (`self.Grass10`) true)
    (`PrimitiveComponent.SetSimulatePhysics` (`self.Grass9`) true)
    (`PrimitiveComponent.SetSimulatePhysics` (`self.Grass8`) true)
    (`PrimitiveComponent.SetSimulatePhysics` (`self.Grass13`) true)
    (`PrimitiveComponent.SetSimulatePhysics` (`self.Grass5`) true)
    (`PrimitiveComponent.SetSimulatePhysics` (`self.Grass4`) true)
    (`PrimitiveComponent.SetSimulatePhysics` (`self.Grass3`) true)
    (`PrimitiveComponent.SetSimulatePhysics` (`self.Grass2`) true)
    (`PrimitiveComponent.SetSimulatePhysics` (`self.Grass1`) true)
    (`PrimitiveComponent.SetSimulatePhysics` (`self.Grass`) true)
    (`PrimitiveComponent.SetSimulatePhysics` (`self.Grass6`) true)
    (`PrimitiveComponent.SetCollisionEnabled` (`self.Grass6`) "PhysicsOnly")
    (`PrimitiveComponent.SetCollisionEnabled` (`self.Grass`) "PhysicsOnly")
    (`PrimitiveComponent.SetCollisionEnabled` (`self.Grass1`) "PhysicsOnly")
    (`PrimitiveComponent.SetCollisionEnabled` (`self.Grass2`) "PhysicsOnly")
    (`PrimitiveComponent.SetCollisionEnabled` (`self.Grass3`) "PhysicsOnly")
    (`PrimitiveComponent.SetCollisionEnabled` (`self.Grass4`) "PhysicsOnly")
    (`PrimitiveComponent.SetCollisionEnabled` (`self.Grass5`) "PhysicsOnly")
    (`PrimitiveComponent.SetCollisionEnabled` (`self.Grass13`) "PhysicsOnly")
    (`PrimitiveComponent.SetCollisionEnabled` (`self.Grass8`) "PhysicsOnly")
    (`PrimitiveComponent.SetCollisionEnabled` (`self.Grass9`) "PhysicsOnly")
    (`PrimitiveComponent.SetCollisionEnabled` (`self.Grass10`) "PhysicsOnly")
    (`PrimitiveComponent.SetCollisionEnabled` (`self.Grass11`) "PhysicsOnly")
    (`PrimitiveComponent.SetCollisionEnabled` (`self.Grass12`) "PhysicsOnly")
    (`PrimitiveComponent.SetCollisionEnabled` (`self.Grass7`) "PhysicsOnly")
    (`KismetSystemLibrary.Delay` 5.0)
    (`self.K2_DestroyActor`)))

(fn `UserConstructionScript`)