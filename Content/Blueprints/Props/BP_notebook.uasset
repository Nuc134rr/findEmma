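; Notebook prop that displays the current day's three tasks and tracks their completion.
; On BeginPlay or SwitchTextNote, it reads DayNum from BP_PlayerCharacter and fills the task texts for one of three days.
; ChangeTextColorToComplete flags a task and reveals its done marker rather than recoloring text, setting DayComplete once all three are done.
; Reset clears the flags and hides the Day1-named markers, which are the only ones used.
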(event `self.ReceiveBeginPlay`
  (switch `int` (`/Game/Blueprints/Core/BP_PlayerCharacter.DayNum` (cast `/Game/Blueprints/Core/BP_PlayerCharacter` (`GameplayStatics.GetPlayerPawn` 0) :!pure true)) :!label _label
    (:`0`
      ;[1 0.8594 0] Day1
      (`TextRenderComponent.K2_SetText` (`self.Task1`) (`self.dayOneTaskOne`))
      (`TextRenderComponent.K2_SetText` (`self.Task2`) (`self.dayOneTaskTwo`))
      (`TextRenderComponent.K2_SetText` (`self.Task3`) (`self.dayOneTaskThree`)))
    (:`1`
      ;[0 0 0] Day2
      (`TextRenderComponent.K2_SetText` (`self.Task1`) (`self.dayTwoTaskOne`))
      (`TextRenderComponent.K2_SetText` (`self.Task2`) (`self.dayTwoTaskTwo`))
      (`TextRenderComponent.K2_SetText` (`self.Task3`) (`self.dayTwoTaskThree`)))
    (:`2`
      ;[1 0 0.3371] Day3
      (`TextRenderComponent.K2_SetText` (`self.Task1`) (`self.dayThreeTaskOne`))
      (`TextRenderComponent.K2_SetText` (`self.Task2`) (`self.dayThreeTaskTwo`))
      (`TextRenderComponent.K2_SetText` (`self.Task3`) (`self.dayThreeTaskThree`)))))

(event `SwitchTextNote`
  (goto _label))

(event `Reset`
  ;[0 0 0] Reset
  (`|ExecutionSequence`
    (:`then_0`
      (set `self.TaskOneCompleted` false)
      (`SceneComponent.SetVisibility` (`self.task 1 done Day 1`) false false))
    (:`then_1`
      (set `self.TaskTwoCompleted` false)
      (`SceneComponent.SetVisibility` (`self.task 2 done Day 1`) false false))
    (:`then_2`
      (set `self.TaskThreeCompleted` false)
      (`SceneComponent.SetVisibility` (`self.task 3 done Day 1`) false false))
    (:`then_3`
      (set `self.DayComplete` false))))

(fn `changeTextColorToComplete`
  (params (Text :type "TextRenderComponent Object Reference") (CompletedTask :type Integer))
  (`KismetSystemLibrary.PrintString` "Gaming")
  (switch `int` CompletedTask
    (:`0`
      (bind _output_get (set `self.TaskOneCompleted` true))
      (`SceneComponent.SetVisibility` (`self.task 1 done Day 1`) true false))
    (:`1`
      (bind _output_get_2 (set `self.TaskTwoCompleted` true))
      (`SceneComponent.SetVisibility` (`self.task 2 done Day 1`) true false))
    (:`2`
      (bind _output_get_3 (set `self.TaskThreeCompleted` true))
      (`SceneComponent.SetVisibility` (`self.task 3 done Day 1`) true false)))
  (if (and _output_get _output_get_2 _output_get_3)
    (set `self.DayComplete` true)
    (else
      (`KismetSystemLibrary.PrintString` "you still have tasks to do"))))

(fn `UserConstructionScript`)