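; VR door prop that swings open or closed on alternate grips of its deadbolt.
; Each accepted grip force-releases the deadbolt, plays a creak and runs a rotation timeline forward or backward, locked until it finishes.
; The first grip also activates the gas task's O2 task if the game instance's GasCanister flag is set.
; Box overlap calls the pawn's TeleportToMap when the axe is gripped on Level_Day3 with Day3Insanity set.
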(event `self.Deadbolt.OnGripped`
  (params (GrippingController :type "GripMotionControllerComponent Object Reference") (GripInformation :type "BPActorGripInformation Structure (by ref)"))
  (`|ExecutionSequence`
    (:`then_0`
      ;[1 1 1] Task Punishments Start At Opening Door
      (`/Engine/EditorBlueprintResources/StandardMacros.DoOnce` false
        (:`Completed`
          (`self.Activate Tasks`))))
    (:`then_1`
      ;[1 1 1] Force release lock and play creak
      (`/Engine/EditorBlueprintResources/StandardMacros.DoOnce` false :!label _label
        (:`Completed`
          (`GripMotionControllerComponent.DropObject` GrippingController (`self.Deadbolt`) 0 false (0.0 0.0 0.0) (0.0 0.0 0.0))
          (`GameplayStatics.PlaySoundAtLocation` "/Game/Assets/Props/Door/SoundEffects/16Door_creaking.16Door_creaking" (`SceneComponent.K2_GetComponentLocation` (`self.Frame`)) (struct) 3.0 1.0 0.0 null null null)
          ;[1 1 1] Switch between opening and closing door, resets do once when finished
          (`/Engine/EditorBlueprintResources/StandardMacros.FlipFlop`
            (:`A`
              (bind (_direction _doorrotationz) (`Timeline|DoorTimelineComponent` :!label _label_2)
                (:`Update`
                  (`SceneComponent.K2_SetRelativeRotation` (`self.Door`) (`KismetMathLibrary.MakeRotator` 0.0 0.0 _doorrotationz) false false))
                (:`Finished`
                  (goto _label :!via `Reset`))))
            (:`B`
              (goto _label_2 :!via `Reverse`))))))))

(event `self.Box.OnComponentBeginOverlap`
  (params (OverlappedComponent :type "PrimitiveComponent Object Reference") (OtherActor :type "Actor Object Reference") (OtherComp :type "PrimitiveComponent Object Reference") (OtherBodyIndex :type Integer) (bFromSweep :type Boolean) (SweepResult :type "HitResult Structure (by ref)"))
  (bind _axeref (`self.AxeRef`))
  (bind _asvive_pawn_character (cast `/Game/PluginContent/VRExpansion/Vive/Vive_PawnCharacter` (`GameplayStatics.GetPlayerPawn` 0) :!pure true))
  (`/Engine/EditorBlueprintResources/StandardMacros.DoOnce` false :!label _label_3
    (:`Completed`
      (bind _returnvalue (`GameplayStatics.GetCurrentLevelName` true))
      (`/Engine/EditorBlueprintResources/StandardMacros.IsValid` _axeref
        (:`Is Valid`
          (if (and (`/Game/Blueprints/Props/BP_axe.bIsGripped` _axeref) (`KismetStringLibrary.EqualEqual_StrStr` _returnvalue "Level_Day3") (`/Game/PluginContent/VRExpansion/Vive/Vive_PawnCharacter.bDay3Insanity` _asvive_pawn_character))
            (`KismetSystemLibrary.PrintString` "good")
            (`/Game/PluginContent/VRExpansion/Vive/Vive_PawnCharacter.Teleport to Map` _asvive_pawn_character)
            (else
              (goto _label_3 :!via `Reset`))))
        (:`Is Not Valid`
          (goto _label_3 :!via `Reset`))))))

(fn `Activate Tasks`
  (bind _gastask (`self.GasTask`))
  (`|ExecutionSequence`
    (:`then_0`
      (if (`/Game/Blueprints/GameInstances_and_GameModes/BP_EmmaInstance_GI.Gas Canister` (cast `/Game/Blueprints/GameInstances_and_GameModes/BP_EmmaInstance_GI` (`GameplayStatics.GetGameInstance`) :!pure true))
        (`/Engine/EditorBlueprintResources/StandardMacros.IsValid` _gastask
          (:`Is Valid`
            (`/Game/Blueprints/O2/O2_Task.Activate O2 Task` _gastask)))))))

(fn `UserConstructionScript`
  (`parent.UserConstructionScript`))