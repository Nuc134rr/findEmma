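; Generator prop with a grippable pull cord and a wrench repair step that completes a notebook task.
; Tick sizes the cable to the handle's distance, forcing a drop at full stretch and starting a faulty engine sound the first time.
; A released handle eases back toward its starting location.
; Once pulled, wrench overlaps lower Health until the bad sound stops, idle audio plays and Task2 completes.
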(event `self.ReceiveTick`
  (params (DeltaSeconds :type "Float (single-precision)"))
  (bind _returnvalue (- (`KismetMathLibrary.Vector_Distance` (`SceneComponent.K2_GetComponentLocation` (`self.StaticMeshComponent`)) (`SceneComponent.K2_GetComponentLocation` (`self.Cube`))) 80.0))
  (if (< _returnvalue 100.0)
    (set `CableComponent.CableLength` _returnvalue (`self.Cable`))
    (else
      (`GripMotionControllerComponent.DropObject` (stale `self.Cube.OnGripped` _output_get) (`self.Cube`) 0 false (0.0 0.0 0.0) (0.0 0.0 0.0))
      (if (`self.Condition`)
        (set `self.Condition` false)
        (bind _returnvalue_2 (`GameplayStatics.SpawnSoundAtLocation` "/Game/Audio/GeneratorStart_Cue.GeneratorStart_Cue" (`SceneComponent.K2_GetComponentLocation` (`self.StaticMeshComponent`)) (struct) 2.0 0.9 0.0 null null))
        (set `self.BadGenSound` _returnvalue_2)
        (set `self.Pulled` true)))))

(event `self.Box.OnComponentBeginOverlap`
  (params (OverlappedComponent :type "PrimitiveComponent Object Reference") (OtherActor :type "Actor Object Reference") (OtherComp :type "PrimitiveComponent Object Reference") (OtherBodyIndex :type Integer) (bFromSweep :type Boolean) (SweepResult :type "HitResult Structure (by ref)"))
  (bind _notebookref (`self.notebookRef`))
  (bind _returnvalue (`SceneComponent.K2_GetComponentLocation` (`self.StaticMeshComponent`)))
  ;[1 1 1] Wrench Overlap
  (if (`self.Check`)
    (if (`self.Pulled`)
      (if (== OtherActor (`self.Wrench`))
        (set `self.Health` (- (`self.Health`) 1))
        (`GameplayStatics.PlaySoundAtLocation` "/Game/Sound/ding.ding" _returnvalue (struct) 1.0 1.0 0.0 null null null)
        (if (<= (`self.Health`) 0)
          (`/Game/Blueprints/Props/BP_notebook.changeTextColorToComplete` _notebookref (`/Game/Blueprints/Props/BP_notebook.Task2` _notebookref) 1)
          (set `self.Check` false)
          (`ActorComponent.SetActive` (`self.BadGenSound`) false false)
          (`GameplayStatics.PlaySoundAtLocation` "/Game/Audio/GeneratorIdle_Cue.GeneratorIdle_Cue" _returnvalue (struct) 5.0 1.0 0.0 null null null))))))

(event `self.Cube.OnGripped`
  (params (GrippingController :type "GripMotionControllerComponent Object Reference") (GripInformation :type "BPActorGripInformation Structure (by ref)"))
  ;[1 1 1] pulling
  (bind _output_get (set `self.Gripping Controller` GrippingController))
  (goto _label :!via `Stop`))

(event `self.Cube.OnDropped`
  (params (GrippingController :type "GripMotionControllerComponent Object Reference") (GripInformation :type "BPActorGripInformation Structure (by ref)") (bWasSocketed :type Boolean))
  ;[1 1 1] pulling
  (`KismetSystemLibrary.MoveComponentTo` (`self.Cube`) (stale `self.ReceiveBeginPlay` _output_get) (struct :`Roll` -35.0) false true 0.4 :!label _label))

(event `self.ReceiveBeginPlay`
  ;[1 1 1] pulling
  (bind _output_get (set `self.cube location` (`SceneComponent.K2_GetComponentLocation` (`self.Cube`)))))

(fn `UserConstructionScript`)