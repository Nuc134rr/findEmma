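; BP_Workbench is a workbench prop with a drawer that is unlocked by a key.
; When the held key overlaps the keyhole sphere, CheckForKey confirms it and the key snaps to the KeyHole socket, flagged as inserted.
; With the key inserted, overlapping the handle collision unlocks Drawer3Slider, and any end of overlap there locks it again.
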(event `self.Sphere.OnComponentBeginOverlap`
  (params (OverlappedComponent :type "PrimitiveComponent Object Reference") (OtherActor :type "Actor Object Reference") (OtherComp :type "PrimitiveComponent Object Reference") (OtherBodyIndex :type Integer) (bFromSweep :type Boolean) (SweepResult :type "HitResult Structure (by ref)"))
  ;[1 1 1] unlock the drawer with key1
  (set `self.Other Comp` OtherComp)
  (bind _bkeyinserted (`self.Check For Key`))
  (if _bkeyinserted
    (`SceneComponent.K2_AttachToComponent` (`Actor.RootComponent` (`self.keyRef`)) (`self.KeyHole`) "KeyHole" "SnapToTarget" "SnapToTarget" "KeepWorld" true) ; attaches key to keyhole at socket KeyHole
    (set `/Game/Blueprints/Props/BP_key1.bIsInKeyhole` true (`self.keyRef`))))

(event `self.handleCollision.OnComponentBeginOverlap`
  (params (OverlappedComponent :type "PrimitiveComponent Object Reference") (OtherActor :type "Actor Object Reference") (OtherComp :type "PrimitiveComponent Object Reference") (OtherBodyIndex :type Integer) (bFromSweep :type Boolean) (SweepResult :type "HitResult Structure (by ref)"))
  ;[1 1 1] handles collision for the drawer handle
  (if (`/Game/Blueprints/Props/BP_key1.bIsInKeyhole` (`self.keyRef`))
    (`VRSliderComponent.SetIsLocked` (`self.Drawer3Slider`) false)))

(event `self.handleCollision.OnComponentEndOverlap`
  (params (OverlappedComponent :type "PrimitiveComponent Object Reference") (OtherActor :type "Actor Object Reference") (OtherComp :type "PrimitiveComponent Object Reference") (OtherBodyIndex :type Integer))
  ;[1 1 1] handles collision for the drawer handle
  (`VRSliderComponent.SetIsLocked` (`self.Drawer3Slider`) true))

(fn `Check For Key`
  (returns (bKeyInserted :type Boolean))
  (bind _other_comp (`self.Other Comp`))
  (bind _keyref (`self.keyRef`))
  (`/Engine/EditorBlueprintResources/StandardMacros.IsValid` _other_comp
    (:`Is Valid`
      (if (and (`/Game/Blueprints/Props/BP_key1.bDoesHaveKey` _keyref) (== _other_comp (`Actor.RootComponent` _keyref)))
        (return true)))))

(fn `UserConstructionScript`)