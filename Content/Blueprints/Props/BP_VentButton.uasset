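; BP_VentButton is a lit button prop that completes the vent task on day two.
; On BeginPlay it checks the current level against the pawn's LevelNames array, starting a timeline on day two and disabling actor collision otherwise.
; A button state change toggles the point light, plays a sound, disables the button's collision, marks the notebook's second task complete and notifies VentTask.
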(event `self.ReceiveBeginPlay`
  (`KismetSystemLibrary.Delay` 1.0)
  (bind _returnvalue (`GameplayStatics.GetCurrentLevelName` true))
  (if (!= (`KismetArrayLibrary.Array_Find` (`/Game/PluginContent/VRExpansion/Vive/Vive_PawnCharacter.Level_Names` (cast `/Game/PluginContent/VRExpansion/Vive/Vive_PawnCharacter` (`GameplayStatics.GetPlayerPawn` 0) :!pure true)) _returnvalue) 1)
    (`KismetSystemLibrary.PrintString` "not day two")
    (`self.SetActorEnableCollision` false)
    (set `self.Timeline_0` null)
    (else
      (`TimelineComponent.PlayFromStart` (`self.Timeline_0`)))))

(event `self.ButtonComp.OnButtonStateChanged`
  (params (ButtonState :type Boolean) (InteractingActor :type "Actor Object Reference") (InteractingComponent :type "PrimitiveComponent Object Reference"))
  (bind _notebookref (`self.notebookRef`))
  (`self.TurnOffLight`)
  (`GameplayStatics.PlaySoundAtLocation` "/Game/Audio/ButtonCue.ButtonCue" (`SceneComponent.K2_GetComponentLocation` (`self.ButtonComp`)) (struct) 1.0 1.0 0.0 null null null)
  (`PrimitiveComponent.SetCollisionEnabled` (`self.ButtonComp`) "NoCollision")
  (`/Game/Blueprints/Props/BP_notebook.changeTextColorToComplete` _notebookref (`/Game/Blueprints/Props/BP_notebook.Task2` _notebookref) 1)
  (`/Game/Blueprints/Props/BP_VentTask.ButtonVentTask` (`self.VentTask`)))

(event `TurnOffLight`
  (`SceneComponent.ToggleVisibility` (`self.PointLight`) true))

(fn `UserConstructionScript`)