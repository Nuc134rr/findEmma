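; VR screw-fix component that tracks the screws holding its owner and signals when it is free of them.
; On BeginPlay it counts valid BP_Screw entries in its Screws array and binds to each one's Released event.
; The release logic decrements the count and, at zero, sets FreeOfScrews and calls AllScrewsReleased.
; An unconnected chain for disabling physics on the owner's static meshes never runs.
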(event `self.ReceiveBeginPlay`
  ;[1 1 1] Get number of connected screws
  (for _array_element (`self.screws`)
    (bind _asbp_screw (cast `/Game/findEmma/ScrewMechanicsVR/Blueprints/BP_Screw` _array_element))
    (if (!= _array_element null)
      (`/Engine/EditorBlueprintResources/StandardMacros.IncrementInt` (`self.Screws Count`) ; Increment screw count
        (:`  `
          (add `/Game/findEmma/ScrewMechanicsVR/Blueprints/BP_Screw.Released` _asbp_screw (delegate `Screw Released`))
          (`self.Screw Released`)
          ;[1 1 1] When each of the screws is released
          (bind _result (`/Engine/EditorBlueprintResources/StandardMacros.DecrementInt` (`self.Screws Count`) :!label _label) ; Decrement screw count
            (:`  `
              (if (<= _result 0)
                ;;[1 1 1] All screws released
                (set `self.Free of Screws` true)
                (`self.All Screws Released`)))))))))

(event `Screw Released`
  (goto _label))