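; VR switchboard puzzle actor that runs a sequential task: power on, tune the dial, plug two jacks into target ports, set a flipswitch combination.
; Success shorts the board, fading emissive materials, firing arcs and teleporting the player to the map.
; BeginPlay builds overlap spheres from mesh "Port" sockets to snap and attach jacks.
; Grip, drop and player-trigger events toggle cable simulation and jack physics, releasing held jacks when the player leaves.
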(event `Switchboard_debugTick`
  ;[1 1 1 1 96] Conlen's Debugging/Testing - Connect/Disconnect debug events from tick/begin play to toggle
)

(event `SwitchboardTaskEnd`
  ;[1 1 1 1 96] Conlen's Debugging/Testing - Connect/Disconnect debug events from tick/begin play to toggle
)

(event `Switchboard_debugInit`
  ;[1 1 1 1 96] Conlen's Debugging/Testing - Connect/Disconnect debug events from tick/begin play to toggle
  (`self.EnableInput` (`GameplayStatics.GetPlayerController` 0)))

(event `Key|F`
  (params (Key :type "Key Structure"))
  ;[1 1 1 1 96] Conlen's Debugging/Testing - Connect/Disconnect debug events from tick/begin play to toggle
  (:`Pressed`
    (`self.SwitchboardTaskStart`)))

(event `Key|H`
  (params (Key :type "Key Structure"))
  ;[1 1 1 1 96] Conlen's Debugging/Testing - Connect/Disconnect debug events from tick/begin play to toggle
  (:`Pressed`
    (`self.SwitchboardShort`)))

(event `self.ReceiveBeginPlay`
  (bind _s_switchboard (`self.S_Switchboard`))
  ;[1 1 1] Init
  (`self.Switchboard_debugInit`) ; Normally enables input so F can be used to start task
  ;[1 1 1] Create Port Triggers and create Overlap Events and set variable for ports B2 and D4 (win condition ports)
  (for _array_element (`SceneComponent.GetAllSocketNames` _s_switchboard)
    (bind _returnvalue (`KismetStringLibrary.Conv_NameToString` _array_element))
    (if (`KismetStringLibrary.Contains` _returnvalue "Port")
      (bind _returnvalue_2 (`AddComponent|NODE_AddSphereComponent-1` :`RelativeTransform` (`SceneComponent.GetSocketTransform` _s_switchboard _array_element "RTS_Actor")))
      (add `PrimitiveComponent.OnComponentBeginOverlap` _returnvalue_2 (delegate `BeginOverlap_Port`))
      (add `PrimitiveComponent.OnComponentEndOverlap` _returnvalue_2 (delegate `EndOverlap_Port`))
      (`KismetArrayLibrary.Array_Add` (`self.AllPortTriggers`) _returnvalue_2)
      (if (`KismetStringLibrary.Contains` _returnvalue "4e")
        (set `self.PortE4` _returnvalue_2)
        (elif (`KismetStringLibrary.Contains` _returnvalue "2b")
          (set `self.PortB2` _returnvalue_2))))))

(event `self.ReceiveTick`
  (params (DeltaSeconds :type "Float (single-precision)"))
  ;[1 1 1] Tick
)

(event `SwitchboardTaskStart`
  ;[1 1 1] Task Event Timeline - ERICK/SHAWN/GEORGE add sounds, delays, audio cues, etc. You guys also set up when task start is sent.
  (set `VRButtonComponent.bIsEnabled` true (`self.S_Switchboard_OnOff`))
  (`KismetSystemLibrary.PrintString` "Task Started - Turn On Switchboard"))

(event `self.S_Switchboard_Aux2_Grippable.OnDropped`
  (params (GrippingController :type "GripMotionControllerComponent Object Reference") (GripInformation :type "BPActorGripInformation Structure (by ref)") (bWasSocketed :type Boolean))
  (bind _s_switchboard_aux2_grippable (`self.S_Switchboard_Aux2_Grippable`))
  (bind _overlappedporttrigger (`self.OverlappedPortTrigger`))
  (bind _returnvalue (== (`self.PortB2`) (`self.AuxPort2`)))
  ;[1 1 1] Stop simulating cable when dropped, if dropped into port then snap to it
  (if (`KismetSystemLibrary.IsValid` _overlappedporttrigger)
    (`PrimitiveComponent.SetSimulatePhysics` _s_switchboard_aux2_grippable false)
    (`SceneComponent.K2_AttachToComponent` _s_switchboard_aux2_grippable _overlappedporttrigger "None" "SnapToTarget" "SnapToTarget" "KeepWorld" false) ; Attach to aux port trigger (same pos as socket)
    (`|ExecutionSequence`
      (:`then_0`
        (bind _output_get (set `self.AuxPort2` _overlappedporttrigger)) ; The port that aux jack 2 is currently in
        ;[1 1 1] Disable Gripping if correct slot, trigger next if both correct
        (if _returnvalue
          (`GrippableStaticMeshComponent.SetDenyGripping` (`self.S_Switchboard_Aux2_Grippable`) true)
          (if (and (`KismetSystemLibrary.IsValid` _output_get) (`KismetSystemLibrary.IsValid` (stale `self.S_Switchboard_Aux1_Grippable.OnDropped` _output_get)))
            (if (and _returnvalue (== (`self.PortE4`) (`self.AuxPort1`))) :!label _label
              (`self.SwitchboardCorrectAuxes`)
              (set `self.Switchboard_LiveAuxJacks` false)))))
      (:`then_1`
        (`KismetSystemLibrary.RetriggerableDelay` 0.5 :!label _label_2) ; Time for cable sim to stop
        (`ActorComponent.SetComponentTickEnabled` (`self.Aux2_Cable`) false) ; Stop cable sim
      ))
    (else
      (goto _label_2))))

(event `self.S_Switchboard_Flipswitch_3.OnButtonStateChanged`
  (params (ButtonState :type Boolean) (InteractingActor :type "Actor Object Reference") (InteractingComponent :type "PrimitiveComponent Object Reference"))
  (bind _s_switchboard_flipswitch_3 (`self.S_Switchboard_Flipswitch_3`))
  ;[1 1 1] Set rotation for Flipswitches + On/Off when pressed (They are VRButton Components but don't translate up or down when pressed, this makes them rotate correctly)
  (if (`VRButtonComponent.bButtonState` _s_switchboard_flipswitch_3)
    (`SceneComponent.K2_SetRelativeTransform` _s_switchboard_flipswitch_3 (`KismetMathLibrary.MakeTransform` (0.0 0.0 0.0) (struct :`Roll` 50.0)) false false)
    (else
      (`SceneComponent.K2_SetRelativeTransform` _s_switchboard_flipswitch_3 (`KismetMathLibrary.MakeTransform` (0.0 0.0 0.0)) false false))))

(event `self.S_Switchboard_Flipswitch_4.OnButtonStateChanged`
  (params (ButtonState :type Boolean) (InteractingActor :type "Actor Object Reference") (InteractingComponent :type "PrimitiveComponent Object Reference"))
  (bind _s_switchboard_flipswitch_4 (`self.S_Switchboard_Flipswitch_4`))
  ;[1 1 1] Set rotation for Flipswitches + On/Off when pressed (They are VRButton Components but don't translate up or down when pressed, this makes them rotate correctly)
  (if (`VRButtonComponent.bButtonState` _s_switchboard_flipswitch_4)
    (`SceneComponent.K2_SetRelativeTransform` _s_switchboard_flipswitch_4 (`KismetMathLibrary.MakeTransform` (0.0 0.0 0.0) (struct :`Roll` 50.0)) false false)
    (else
      (`SceneComponent.K2_SetRelativeTransform` _s_switchboard_flipswitch_4 (`KismetMathLibrary.MakeTransform` (0.0 0.0 0.0)) false false))))

(event `self.S_Switchboard_OnOff.OnButtonStateChanged`
  (params (ButtonState :type Boolean) (InteractingActor :type "Actor Object Reference") (InteractingComponent :type "PrimitiveComponent Object Reference"))
  (bind _s_switchboard_onoff (`self.S_Switchboard_OnOff`))
  ;[1 1 1] Task Event Timeline - ERICK/SHAWN/GEORGE add sounds, delays, audio cues, etc. You guys also set up when task start is sent.
  (if (`VRButtonComponent.bButtonState` _s_switchboard_onoff)
    (`self.SwitchboardTurnedOn`)
    (set `VRButtonComponent.bIsEnabled` false _s_switchboard_onoff)))

(event `BeginOverlap_Port`
  (params (OverlappedComponent :type "PrimitiveComponent Object Reference") (OtherActor :type "Actor Object Reference") (OtherComp :type "PrimitiveComponent Object Reference") (OtherBodyIndex :type Integer) (bFromSweep :type Boolean) (SweepResult :type "HitResult Structure (by ref)"))
  (bind _returnvalue (`SceneComponent.K2_GetComponentLocation` OverlappedComponent))
  (bind _aux2_lastport (`self.Aux2_LastPort`))
  (bind _aux1_lastport (`self.Aux1_LastPort`))
  (bind _s_switchboard_aux2_grippable (`self.S_Switchboard_Aux2_Grippable`))
  (bind _s_switchboard_aux1_grippable (`self.S_Switchboard_Aux1_Grippable`))
  ;[1 1 1] Move Aux Jack to Port
  (`|ExecutionSequence`
    (:`then_0`
      (if (== OtherComp _s_switchboard_aux2_grippable)
        (set `self.OverlappedPortTrigger` OverlappedComponent)
        (if (!= OverlappedComponent (`self.AuxPort1`))
          (if (`KismetSystemLibrary.IsValid` _aux2_lastport)
            (if (!= OverlappedComponent _aux2_lastport)
              (`SceneComponent.K2_SetWorldLocation` _s_switchboard_aux2_grippable _returnvalue false false :!label _label_3) ; Snaps aux jack 2 to the port it overlapped with but doesn't drop or socket
              (set `self.Aux2_LastPort` OverlappedComponent) ; The port that aux jack 2 most recently entered, used to prevent infinite snapping in a port
            )
            (else
              (goto _label_3))))))
    (:`then_1`
      (if (== OtherComp _s_switchboard_aux1_grippable)
        (set `self.OverlappedPortTrigger` OverlappedComponent)
        (if (!= OverlappedComponent (`self.AuxPort2`))
          (if (`KismetSystemLibrary.IsValid` _aux1_lastport)
            (if (!= OverlappedComponent _aux1_lastport)
              (`SceneComponent.K2_SetWorldLocation` _s_switchboard_aux1_grippable _returnvalue false false :!label _label_4)
              (set `self.Aux1_LastPort` OverlappedComponent))
            (else
              (goto _label_4))))))))

(event `SwitchboardTurnedOn`
  ;[1 1 1] Task Event Timeline - ERICK/SHAWN/GEORGE add sounds, delays, audio cues, etc. You guys also set up when task start is sent.
  (set `VRDialComponent.bDenyGripping` false (`self.S_Switchboard_BigKnob`))
  (`|ExecutionSequence`
    (:`then_0`
      (`KismetSystemLibrary.PrintString` "Switchboard Turned On - Now Tune Dial"))
    (:`then_1`
      (bind (_direction _emissive_strength _indicatorglass_color) (`Timeline|EmissionOn` :!via `PlayFromStart`)
        (:`Update`
          (`MaterialInstanceDynamic.SetScalarParameterValue` (`self.Switchboard_Emission_DynamicMat`) "Switchboard_EmissiveMul" _emissive_strength)
          (`MaterialInstanceDynamic.SetScalarParameterValue` (`self.Switchboard_IndicatorGlass_DynamicMat`) "Switchboard_GlassLight" _indicatorglass_color))))))

(event `self.S_Switchboard_Flipswitch_2.OnButtonStateChanged`
  (params (ButtonState :type Boolean) (InteractingActor :type "Actor Object Reference") (InteractingComponent :type "PrimitiveComponent Object Reference"))
  (bind _s_switchboard_flipswitch_2 (`self.S_Switchboard_Flipswitch_2`))
  ;[1 1 1] Set rotation for Flipswitches + On/Off when pressed (They are VRButton Components but don't translate up or down when pressed, this makes them rotate correctly)
  (if (`VRButtonComponent.bButtonState` _s_switchboard_flipswitch_2)
    (`SceneComponent.K2_SetRelativeTransform` _s_switchboard_flipswitch_2 (`KismetMathLibrary.MakeTransform` (0.0 0.0 0.0) (struct :`Roll` 50.0)) false false)
    (else
      (`SceneComponent.K2_SetRelativeTransform` _s_switchboard_flipswitch_2 (`KismetMathLibrary.MakeTransform` (0.0 0.0 0.0)) false false))))

(event `self.S_Switchboard_Flipswitch_5.OnButtonStateChanged`
  (params (ButtonState :type Boolean) (InteractingActor :type "Actor Object Reference") (InteractingComponent :type "PrimitiveComponent Object Reference"))
  (bind _s_switchboard_flipswitch_5 (`self.S_Switchboard_Flipswitch_5`))
  ;[1 1 1] Set rotation for Flipswitches + On/Off when pressed (They are VRButton Components but don't translate up or down when pressed, this makes them rotate correctly)
  (if (`VRButtonComponent.bButtonState` _s_switchboard_flipswitch_5)
    (`SceneComponent.K2_SetRelativeTransform` _s_switchboard_flipswitch_5 (`KismetMathLibrary.MakeTransform` (0.0 0.0 0.0) (struct :`Roll` 50.0)) false false)
    (else
      (`SceneComponent.K2_SetRelativeTransform` _s_switchboard_flipswitch_5 (`KismetMathLibrary.MakeTransform` (0.0 0.0 0.0)) false false))))

(event `self.S_Switchboard_BigKnob.OnDropped`
  (params (GrippingController :type "GripMotionControllerComponent Object Reference") (GripInformation :type "BPActorGripInformation Structure (by ref)") (bWasSocketed :type Boolean))
  (bind _s_switchboard_bigknob (`self.S_Switchboard_BigKnob`))
  ;[1 1 1] Task Event Timeline - ERICK/SHAWN/GEORGE add sounds, delays, audio cues, etc. You guys also set up when task start is sent.
  (if (== (`VRDialComponent.CurrentDialAngle` _s_switchboard_bigknob) 40.0)
    (`self.SwitchboardDialTuned`)
    (set `VRDialComponent.bDenyGripping` true _s_switchboard_bigknob)))

(event `self.S_Switchboard_Aux1_Grippable.OnDropped`
  (params (GrippingController :type "GripMotionControllerComponent Object Reference") (GripInformation :type "BPActorGripInformation Structure (by ref)") (bWasSocketed :type Boolean))
  (bind _overlappedporttrigger (`self.OverlappedPortTrigger`))
  (bind _s_switchboard_aux1_grippable (`self.S_Switchboard_Aux1_Grippable`))
  ;[1 1 1] Stop simulating cable when dropped, if dropped into port then snap to it
  (if (`KismetSystemLibrary.IsValid` _overlappedporttrigger)
    (`PrimitiveComponent.SetSimulatePhysics` _s_switchboard_aux1_grippable false)
    (`SceneComponent.K2_AttachToComponent` _s_switchboard_aux1_grippable _overlappedporttrigger "None" "SnapToTarget" "SnapToTarget" "KeepWorld" false)
    (`|ExecutionSequence`
      (:`then_0`
        (bind _output_get (set `self.AuxPort1` _overlappedporttrigger))
        ;[1 1 1] Disable Gripping if correct slot, trigger next if both correct
        (if (== (`self.PortE4`) (`self.AuxPort1`))
          (`GrippableStaticMeshComponent.SetDenyGripping` (`self.S_Switchboard_Aux1_Grippable`) true)
          (if (and (`KismetSystemLibrary.IsValid` (stale `self.S_Switchboard_Aux2_Grippable.OnDropped` _output_get)) (`KismetSystemLibrary.IsValid` _output_get))
            (goto _label))))
      (:`then_1`
        (`KismetSystemLibrary.RetriggerableDelay` 0.5 :!label _label_5)
        (`ActorComponent.SetComponentTickEnabled` (`self.Aux1_Cable`) false)))
    (else
      (goto _label_5))))

(event `SwitchboardDialTuned`
  ;[1 1 1] Task Event Timeline - ERICK/SHAWN/GEORGE add sounds, delays, audio cues, etc. You guys also set up when task start is sent.
  (set `self.Switchboard_LiveAuxJacks` true)
  (`GrippableStaticMeshComponent.SetDenyGripping` (`self.S_Switchboard_Aux1_Grippable`) false)
  (`GrippableStaticMeshComponent.SetDenyGripping` (`self.S_Switchboard_Aux2_Grippable`) false)
  (`KismetSystemLibrary.PrintString` "Dial Tuned - Now plug In Aux Jack (Front one) to Port B2 and Out Aux Jack (Back one) to Port E4"))

(event `SwitchboardCorrectAuxes`
  ;[1 1 1] Task Event Timeline - ERICK/SHAWN/GEORGE add sounds, delays, audio cues, etc. You guys also set up when task start is sent.
  (set `VRButtonComponent.bIsEnabled` true (`self.S_Switchboard_Flipswitch_1`))
  (set `VRButtonComponent.bIsEnabled` true (`self.S_Switchboard_Flipswitch_2`))
  (set `VRButtonComponent.bIsEnabled` true (`self.S_Switchboard_Flipswitch_3`))
  (set `VRButtonComponent.bIsEnabled` true (`self.S_Switchboard_Flipswitch_4`))
  (set `VRButtonComponent.bIsEnabled` true (`self.S_Switchboard_Flipswitch_5`))
  (set `VRButtonComponent.bIsEnabled` true (`self.S_Switchboard_Flipswitch_6`))
  (set `VRButtonComponent.bIsEnabled` true (`self.S_Switchboard_Flipswitch_7`))
  (`KismetSystemLibrary.PrintString` "Auxes correctly connected, now flip switches T W X & Z"))

(event `self.S_Switchboard_Flipswitch_1.OnButtonStateChanged`
  (params (ButtonState :type Boolean) (InteractingActor :type "Actor Object Reference") (InteractingComponent :type "PrimitiveComponent Object Reference"))
  (bind _s_switchboard_flipswitch_1 (`self.S_Switchboard_Flipswitch_1`))
  ;[1 1 1] Set rotation for Flipswitches + On/Off when pressed (They are VRButton Components but don't translate up or down when pressed, this makes them rotate correctly)
  (if (`VRButtonComponent.bButtonState` _s_switchboard_flipswitch_1)
    (`SceneComponent.K2_SetRelativeTransform` _s_switchboard_flipswitch_1 (`KismetMathLibrary.MakeTransform` (0.0 0.0 0.0) (struct :`Roll` 50.0)) false false)
    (else
      (`SceneComponent.K2_SetRelativeTransform` _s_switchboard_flipswitch_1 (`KismetMathLibrary.MakeTransform` (0.0 0.0 0.0)) false false))))

(event `self.S_Switchboard_Flipswitch_6.OnButtonStateChanged`
  (params (ButtonState :type Boolean) (InteractingActor :type "Actor Object Reference") (InteractingComponent :type "PrimitiveComponent Object Reference"))
  (bind _s_switchboard_flipswitch_6 (`self.S_Switchboard_Flipswitch_6`))
  ;[1 1 1] Set rotation for Flipswitches + On/Off when pressed (They are VRButton Components but don't translate up or down when pressed, this makes them rotate correctly)
  (if (`VRButtonComponent.bButtonState` _s_switchboard_flipswitch_6)
    (`SceneComponent.K2_SetRelativeTransform` _s_switchboard_flipswitch_6 (`KismetMathLibrary.MakeTransform` (0.0 0.0 0.0) (struct :`Roll` 50.0)) false false)
    (else
      (`SceneComponent.K2_SetRelativeTransform` _s_switchboard_flipswitch_6 (`KismetMathLibrary.MakeTransform` (0.0 0.0 0.0)) false false))))

(event `self.S_Switchboard_Flipswitch_1.OnButtonEndInteraction`
  (params (InteractingActor :type "Actor Object Reference") (InteractingComponent :type "PrimitiveComponent Object Reference"))
  ;[1 1 1] Task Event Timeline - ERICK/SHAWN/GEORGE add sounds, delays, audio cues, etc. You guys also set up when task start is sent.
  (if (and (== (`VRButtonComponent.bButtonState` (`self.S_Switchboard_Flipswitch_1`)) true) (== (`VRButtonComponent.bButtonState` (`self.S_Switchboard_Flipswitch_2`)) false) (== (`VRButtonComponent.bButtonState` (`self.S_Switchboard_Flipswitch_3`)) false) (== (`VRButtonComponent.bButtonState` (`self.S_Switchboard_Flipswitch_4`)) true) (== (`VRButtonComponent.bButtonState` (`self.S_Switchboard_Flipswitch_5`)) true) (== (`VRButtonComponent.bButtonState` (`self.S_Switchboard_Flipswitch_6`)) false) (== (`VRButtonComponent.bButtonState` (`self.S_Switchboard_Flipswitch_7`)) true)) :!label _label_6
    (if (not (`self.flipswitchesCorrect`))
      (set `self.flipswitchesCorrect` true)
      (set `VRButtonComponent.bIsEnabled` false (`self.S_Switchboard_Flipswitch_1`))
      (set `VRButtonComponent.bIsEnabled` false (`self.S_Switchboard_Flipswitch_2`))
      (set `VRButtonComponent.bIsEnabled` false (`self.S_Switchboard_Flipswitch_3`))
      (set `VRButtonComponent.bIsEnabled` false (`self.S_Switchboard_Flipswitch_4`))
      (set `VRButtonComponent.bIsEnabled` false (`self.S_Switchboard_Flipswitch_5`))
      (set `VRButtonComponent.bIsEnabled` false (`self.S_Switchboard_Flipswitch_6`))
      (set `VRButtonComponent.bIsEnabled` false (`self.S_Switchboard_Flipswitch_7`))
      (`self.SwitchboardShort`))))

(event `self.S_Switchboard_Flipswitch_2.OnButtonEndInteraction`
  (params (InteractingActor :type "Actor Object Reference") (InteractingComponent :type "PrimitiveComponent Object Reference"))
  ;[1 1 1] Task Event Timeline - ERICK/SHAWN/GEORGE add sounds, delays, audio cues, etc. You guys also set up when task start is sent.
  (goto _label_6))

(event `EndOverlap_Port`
  (params (OverlappedComponent :type "PrimitiveComponent Object Reference") (OtherActor :type "Actor Object Reference") (OtherComp :type "PrimitiveComponent Object Reference") (OtherBodyIndex :type Integer))
  (bind _jack2triggersoverlapped (`self.Jack2TriggersOverlapped`))
  (bind _allporttriggers (`self.AllPortTriggers`))
  (bind _jack1triggersoverlapped (`self.Jack1TriggersOverlapped`))
  (bind _jack1triggersoverlapped_2 (`self.Jack1TriggersOverlapped`))
  (bind _jack2triggersoverlapped_2 (`self.Jack2TriggersOverlapped`))
  (bind _s_switchboard_aux1_grippable (`self.S_Switchboard_Aux1_Grippable`))
  (bind _s_switchboard_aux2_grippable (`self.S_Switchboard_Aux2_Grippable`))
  (bind _returnvalue (== _jack2triggersoverlapped 0))
  (bind _returnvalue_2 (== _jack1triggersoverlapped_2 0))
  ;[1 1 1] Set Nulls
  (`|ExecutionSequence`
    (:`then_0`
      (if (== OtherComp _s_switchboard_aux1_grippable)
        (bind (_holdingcontrollers _bisheld) (message `VRGripInterface.IsHeld` _s_switchboard_aux1_grippable))
        (if _bisheld
          (for _array_element (`self.AllPortTriggers`)
            (if (`PrimitiveComponent.IsOverlappingComponent` _s_switchboard_aux1_grippable _array_element)
              (set `self.Jack1TriggersOverlapped` (+ _jack1triggersoverlapped_2 1))))
          (`|ExecutionSequence`
            (:`then_0`
              (if _returnvalue_2
                (set `self.Aux1_LastPort` null) ; Set to null so if brought back to this port before touching another it will allow snapping
                (for _array_element_2 _allporttriggers
                  (if (`PrimitiveComponent.IsOverlappingComponent` (`self.S_Switchboard_Aux2_Grippable`) _array_element_2)
                    (set `self.Jack2TriggersOverlapped` (+ _jack2triggersoverlapped_2 1))))
                (if (== _jack2triggersoverlapped_2 0)
                  (set `self.OverlappedPortTrigger` null :!label _label_7) ; If ((Aux Jack 1 isn't in any aux port triggers) AND (Aux Jack 2 isn't in any aux port triggers OR if it is but it is plugged in)) Then set null the aux port trigger sphere that was being overlapped
                  (else
                    (set `self.Jack2TriggersOverlapped` 0) ; Reset count of overlapped triggers
                    (if (`KismetSystemLibrary.IsValid` (`self.AuxPort2`))
                      (goto _label_7))))
                (else
                  (set `self.Jack1TriggersOverlapped` 0) ; Reset count of overlapped triggers
                )))
            (:`then_1`
              (if _returnvalue_2
                (set `self.AuxPort1` null) ; The aux port trigger sphere that Aux Jack 1 was attached to (if it was attached to one) is set to null
              ))))))
    (:`then_1`
      (if (== OtherComp _s_switchboard_aux2_grippable)
        (bind (_holdingcontrollers_2 _bisheld_2) (message `VRGripInterface.IsHeld` _s_switchboard_aux2_grippable))
        (if _bisheld_2
          (for _array_element_3 (`self.AllPortTriggers`)
            (if (`PrimitiveComponent.IsOverlappingComponent` _s_switchboard_aux2_grippable _array_element_3)
              (set `self.Jack2TriggersOverlapped` (+ _jack2triggersoverlapped 1))))
          (`|ExecutionSequence`
            (:`then_0`
              (if _returnvalue
                (set `self.Aux2_LastPort` null)
                (for _array_element_4 _allporttriggers
                  (if (`PrimitiveComponent.IsOverlappingComponent` (`self.S_Switchboard_Aux1_Grippable`) _array_element_4)
                    (set `self.Jack1TriggersOverlapped` (+ _jack1triggersoverlapped 1))))
                (if (== _jack1triggersoverlapped 0)
                  (set `self.OverlappedPortTrigger` null :!label _label_8)
                  (else
                    (set `self.Jack2TriggersOverlapped` 0)
                    (if (`KismetSystemLibrary.IsValid` (`self.AuxPort1`))
                      (goto _label_8))))
                (else
                  (set `self.Jack2TriggersOverlapped` 0))))
            (:`then_1`
              (if _returnvalue
                (set `self.AuxPort2` null)))))))))

(event `self.S_Switchboard_Flipswitch_3.OnButtonEndInteraction`
  (params (InteractingActor :type "Actor Object Reference") (InteractingComponent :type "PrimitiveComponent Object Reference"))
  ;[1 1 1] Task Event Timeline - ERICK/SHAWN/GEORGE add sounds, delays, audio cues, etc. You guys also set up when task start is sent.
  (goto _label_6))

(event `self.S_Switchboard_Flipswitch_7.OnButtonStateChanged`
  (params (ButtonState :type Boolean) (InteractingActor :type "Actor Object Reference") (InteractingComponent :type "PrimitiveComponent Object Reference"))
  (bind _s_switchboard_flipswitch_7 (`self.S_Switchboard_Flipswitch_7`))
  ;[1 1 1] Set rotation for Flipswitches + On/Off when pressed (They are VRButton Components but don't translate up or down when pressed, this makes them rotate correctly)
  (if (`VRButtonComponent.bButtonState` _s_switchboard_flipswitch_7)
    (`SceneComponent.K2_SetRelativeTransform` _s_switchboard_flipswitch_7 (`KismetMathLibrary.MakeTransform` (0.0 0.0 0.0) (struct :`Roll` 50.0)) false false)
    (else
      (`SceneComponent.K2_SetRelativeTransform` _s_switchboard_flipswitch_7 (`KismetMathLibrary.MakeTransform` (0.0 0.0 0.0)) false false))))

(event `self.S_Switchboard_Flipswitch_4.OnButtonEndInteraction`
  (params (InteractingActor :type "Actor Object Reference") (InteractingComponent :type "PrimitiveComponent Object Reference"))
  ;[1 1 1] Task Event Timeline - ERICK/SHAWN/GEORGE add sounds, delays, audio cues, etc. You guys also set up when task start is sent.
  (goto _label_6))

(event `self.S_Switchboard_OnOff.OnButtonBeginInteraction`
  (params (InteractingActor :type "Actor Object Reference") (InteractingComponent :type "PrimitiveComponent Object Reference"))
  ;[1 1 1] Set rotation for Flipswitches + On/Off when pressed (They are VRButton Components but don't translate up or down when pressed, this makes them rotate correctly)
  (`SceneComponent.K2_SetRelativeTransform` (`self.S_Switchboard_OnOff`) (`KismetMathLibrary.MakeTransform` (0.0 0.0 0.0)) false false))

(event `self.S_Switchboard_Flipswitch_5.OnButtonEndInteraction`
  (params (InteractingActor :type "Actor Object Reference") (InteractingComponent :type "PrimitiveComponent Object Reference"))
  ;[1 1 1] Task Event Timeline - ERICK/SHAWN/GEORGE add sounds, delays, audio cues, etc. You guys also set up when task start is sent.
  (goto _label_6))

(event `self.S_Switchboard_Flipswitch_6.OnButtonEndInteraction`
  (params (InteractingActor :type "Actor Object Reference") (InteractingComponent :type "PrimitiveComponent Object Reference"))
  ;[1 1 1] Task Event Timeline - ERICK/SHAWN/GEORGE add sounds, delays, audio cues, etc. You guys also set up when task start is sent.
  (goto _label_6))

(event `self.S_Switchboard_Flipswitch_7.OnButtonEndInteraction`
  (params (InteractingActor :type "Actor Object Reference") (InteractingComponent :type "PrimitiveComponent Object Reference"))
  ;[1 1 1] Task Event Timeline - ERICK/SHAWN/GEORGE add sounds, delays, audio cues, etc. You guys also set up when task start is sent.
  (goto _label_6))

(event `self.Switchboard_Trigger.OnComponentBeginOverlap`
  (params (OverlappedComponent :type "PrimitiveComponent Object Reference") (OtherActor :type "Actor Object Reference") (OtherComp :type "PrimitiveComponent Object Reference") (OtherBodyIndex :type Integer) (bFromSweep :type Boolean) (SweepResult :type "HitResult Structure (by ref)"))
  ;[1 1 1] Start/Stop Aux Simulation when entering/leaving area & when gripped
  (if (== OtherActor (`GameplayStatics.GetPlayerPawn` 0))
    (if (not (`self.playerInTrigger`))
      (set `self.playerInTrigger` true) ; Prevents different components of player pawn from running this code more than once without leaving the trigger first
      (if (not (`self.Switchboard_LiveAuxJacks`))
        (`|ExecutionSequence`
          (:`then_0`
            (`PrimitiveComponent.SetSimulatePhysics` (`self.S_Switchboard_Aux2_Grippable`) false :!label _label_9) ; Turn off cable sim and aux jack physics for aux jack 2
            (`ActorComponent.SetComponentTickEnabled` (`self.Aux2_Cable`) false))
          (:`then_1`
            (`PrimitiveComponent.SetSimulatePhysics` (`self.S_Switchboard_Aux1_Grippable`) false :!label _label_10)
            (`ActorComponent.SetComponentTickEnabled` (`self.Aux1_Cable`) false)))))))

(event `SwitchboardShort`
  ;[1 1 1] Task Event Timeline - ERICK/SHAWN/GEORGE add sounds, delays, audio cues, etc. You guys also set up when task start is sent.
  (`self.SwitchboardTaskEnd`)
  (`|ExecutionSequence`
    (:`then_0`
      (bind (_direction _emissive_strength _indicatorglass_color) (`Timeline|EmissionOff` :!via `PlayFromStart`)
        (:`Update`
          (`MaterialInstanceDynamic.SetScalarParameterValue` (`self.Switchboard_Emission_DynamicMat`) "Switchboard_EmissiveMul" _emissive_strength)
          (`MaterialInstanceDynamic.SetScalarParameterValue` (`self.Switchboard_IndicatorGlass_DynamicMat`) "Switchboard_GlassLight" _indicatorglass_color))))
    (:`then_1`
      (`KismetSystemLibrary.PrintString` "The switchboard shorted out!")
      (`ActorComponent.Activate` (`self.NS_ElectricArcs`) false)
      (`KismetSystemLibrary.Delay` 5.0)
      (`/Game/VRExpansion/Vive/Vive_PawnCharacter.Teleport to Map` (cast `/Game/VRExpansion/Vive/Vive_PawnCharacter` (`GameplayStatics.GetPlayerPawn` 0) :!pure true)))))

(event `self.Switchboard_Trigger.OnComponentEndOverlap`
  (params (OverlappedComponent :type "PrimitiveComponent Object Reference") (OtherActor :type "Actor Object Reference") (OtherComp :type "PrimitiveComponent Object Reference") (OtherBodyIndex :type Integer))
  ;[1 1 1] Start/Stop Aux Simulation when entering/leaving area & when gripped
  (if (== OtherActor (`GameplayStatics.GetPlayerPawn` 0))
    (set `self.playerInTrigger` false)
    (`|ExecutionSequence`
      (:`then_0`
        (bind _controller (`self.Get Both Motion Controllers`))
        (`GripMotionControllerComponent.DropComponent` _controller (`self.S_Switchboard_Aux2_Grippable`) true (0.0 0.0 0.0) (0.0 0.0 0.0)) ; Drop aux jack 2 (if it is held)
        (`KismetSystemLibrary.RetriggerableDelay` 1.0)
        (goto _label_9))
      (:`then_1`
        (bind _controller_2 (`self.Get Both Motion Controllers`))
        (`GripMotionControllerComponent.DropComponent` _controller_2 (`self.S_Switchboard_Aux1_Grippable`) true (0.0 0.0 0.0) (0.0 0.0 0.0))
        (`KismetSystemLibrary.RetriggerableDelay` 1.0)
        (goto _label_10)))))

(event `self.S_Switchboard_Aux1_Grippable.OnGripped`
  (params (GrippingController :type "GripMotionControllerComponent Object Reference") (GripInformation :type "BPActorGripInformation Structure (by ref)"))
  ;[1 1 1] Start/Stop Aux Simulation when entering/leaving area & when gripped
  (`PrimitiveComponent.SetSimulatePhysics` (`self.S_Switchboard_Aux1_Grippable`) true) ; Turn on physics and cable sim for aux jack 1
  (`ActorComponent.SetComponentTickEnabled` (`self.Aux1_Cable`) true))

(event `self.S_Switchboard_Aux2_Grippable.OnGripped`
  (params (GrippingController :type "GripMotionControllerComponent Object Reference") (GripInformation :type "BPActorGripInformation Structure (by ref)"))
  ;[1 1 1] Start/Stop Aux Simulation when entering/leaving area & when gripped
  (`PrimitiveComponent.SetSimulatePhysics` (`self.S_Switchboard_Aux2_Grippable`) true)
  (`ActorComponent.SetComponentTickEnabled` (`self.Aux2_Cable`) true))

(fn `UserConstructionScript`
  ;[1 1 1] Dynamic Material for Changing Emission
  (bind _returnvalue (`KismetMaterialLibrary.CreateDynamicMaterialInstance` (`PrimitiveComponent.GetMaterial` (`self.S_Switchboard`) 1)))
  (bind _output_get (set `self.Switchboard_Emission_DynamicMat` _returnvalue))
  (`PrimitiveComponent.SetMaterial` (`self.S_Switchboard`) 1 _output_get)
  (bind _returnvalue_2 (`KismetMaterialLibrary.CreateDynamicMaterialInstance` (`PrimitiveComponent.GetMaterial` (`self.Switchboard_IndicatorGlass_lp`) 0)))
  (bind _output_get_2 (set `self.Switchboard_IndicatorGlass_DynamicMat` _returnvalue_2))
  (`PrimitiveComponent.SetMaterial` (`self.Switchboard_IndicatorGlass_lp`) 0 _output_get_2))