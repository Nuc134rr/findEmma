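; BP_FakeCan is a test can prop that completes the notebook's first task when its inner can is rolled to a target angle.
; Gripping the Lid starts a looping timer on Shawn, which compares InnerCan's world roll to a reference roll within a wide tolerance.
; On a match, Akudfusidov hides InnerCan, stops the timer and updates the notebook text, with debug prints throughout.
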(event `akudfusidov`
  (bind _notebookref (`self.notebookRef`))
  (`SceneComponent.SetVisibility` (`self.InnerCan`) false false)
  (`KismetSystemLibrary.PrintString` "All Good")
  (`KismetSystemLibrary.K2_ClearAndInvalidateTimerHandle` (stale `self.Lid .OnGripped` _returnvalue))
  (`/Game/findEmma/Blueprints/Props/BP_notebook.changeTextColorToComplete` _notebookref (`/Game/findEmma/Blueprints/Props/BP_notebook.Task1` _notebookref) 0))

(event `self.Lid .OnGripped`
  (params (GrippingController :type "GripMotionControllerComponent Object Reference") (GripInformation :type "BPActorGripInformation Structure (by ref)"))
  (`KismetSystemLibrary.PrintString` "B e a n s")
  (bind _returnvalue (`KismetSystemLibrary.K2_SetTimer` null "Shawn" 0.1 true)))

(fn `Shawn`
  (bind _roll (.roll (`self.118y`)))
  (bind _roll_2 (.roll (`SceneComponent.K2_GetComponentRotation` (`self.InnerCan`))))
  (`KismetSystemLibrary.PrintString` (`KismetStringLibrary.Conv_DoubleToString` _roll_2))
  (`KismetSystemLibrary.PrintString` (`KismetStringLibrary.Conv_DoubleToString` _roll) true true (struct :`G` 0.136427 :`B` 1.0 :`A` 1.0))
  (if (`KismetMathLibrary.NearlyEqual_FloatFloat` _roll_2 _roll 30.0)
    (`self.akudfusidov`)))

(fn `UserConstructionScript`)