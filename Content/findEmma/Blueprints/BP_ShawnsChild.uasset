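; VR valve puzzle actor that the player turns to a random goal angle, set at BeginPlay, to complete a notebook task.
; Gripping starts looping timers that play rust sounds, mostly scaled in volume and pitch by dial angle, and check the goal; dropping stops them.
; Reaching the goal plays a ding, stops the timers, disables valve collision, forces a drop and marks Task2 complete in the notebook.
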(event `self.Valve.OnDropped`
  (params (GrippingController :type "GripMotionControllerComponent Object Reference") (GripInformation :type "BPActorGripInformation Structure (by ref)") (bWasSocketed :type Boolean))
  (`KismetSystemLibrary.K2_ClearAndInvalidateTimerHandle` (stale `self.Valve.OnGripped` _returnvalue))
  (`KismetSystemLibrary.K2_ClearAndInvalidateTimerHandle` (stale `self.Valve.OnGripped` _returnvalue_2)))

(event `self.Valve.OnGripped`
  (params (GrippingController :type "GripMotionControllerComponent Object Reference") (GripInformation :type "BPActorGripInformation Structure (by ref)"))
  (`self.On Gripped`)
  (bind _returnvalue (`KismetSystemLibrary.K2_SetTimer` null "On Gripped" 3.0 true))
  (bind _returnvalue_2 (`KismetSystemLibrary.K2_SetTimer` null "Checking" 0.5 true)))

(event `Angle Correct`
  (bind _notebookref (`self.notebookRef`))
  (bind _valve (`self.Valve`))
  (if (>= (`VRDialComponent.CurrentDialAngle` (`self.Valve`)) (stale `self.ReceiveBeginPlay` _output_get))
    (`GameplayStatics.PlaySoundAtLocation` "/Game/findEmma/Sound/ding.ding" (0.0 0.0 0.0) (struct) 1.0 1.0 0.0 null null null)
    (`KismetSystemLibrary.K2_ClearAndInvalidateTimerHandle` (stale `self.Valve.OnGripped` _returnvalue))
    (`KismetSystemLibrary.K2_ClearAndInvalidateTimerHandle` (stale `self.Valve.OnGripped` _returnvalue_2))
    (`PrimitiveComponent.SetCollisionEnabled` _valve "NoCollision")
    (`GripMotionControllerComponent.DropObject` (stale `self.Valve.OnGripped` GrippingController) _valve 0 false (0.0 0.0 0.0) (0.0 0.0 0.0))
    (`/Engine/EditorBlueprintResources/StandardMacros.IsValid` _notebookref
      (:`Is Valid`
        (`/Game/findEmma/Blueprints/BP_notebook.changeTextColorToComplete` _notebookref (`/Game/findEmma/Blueprints/BP_notebook.Task2` _notebookref))))))

(event `self.ReceiveBeginPlay`
  (bind _output_get (set `self.Goal Float` (`KismetMathLibrary.RandomFloatInRange` 200.0 500.0)))
  (`KismetSystemLibrary.PrintString` (`KismetStringLibrary.Conv_DoubleToString` _output_get)))

(fn `Checking`
  (`self.Angle Correct`))

(fn `On Gripped`
  (bind _currentdialangle (`VRDialComponent.CurrentDialAngle` (`self.Valve`)))
  (bind _returnvalue (/ (`KismetMathLibrary.Conv_IntToDouble` (`KismetMathLibrary.Round` (/ (`VRDialComponent.CurrentDialAngle` (`self.Valve`)) 100.0))) 3.0))
  (`KismetSystemLibrary.PrintString` (`KismetStringLibrary.Conv_DoubleToString` (`VRDialComponent.CurrentDialAngle` (`self.Valve`))))
  (if (<= _currentdialangle 0.0)
    (`GameplayStatics.PlaySoundAtLocation` "/Game/findEmma/Sound/rust.rust" (0.0 0.0 0.0) (struct) 2.0 2.0 0.0 null null null)
    (elif (not (>= _currentdialangle 460.0))
      (`GameplayStatics.PlaySoundAtLocation` "/Game/findEmma/Sound/rust.rust" (0.0 0.0 0.0) (struct) _returnvalue _returnvalue 0.0 null null null))))

(fn `UserConstructionScript`)