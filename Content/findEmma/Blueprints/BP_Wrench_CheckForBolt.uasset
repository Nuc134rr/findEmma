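; Wrench actor that detects a referenced bolt and attaches it to the wrench mesh.
; A sphere overlap runs CheckForBolt, which calls Grip2 when the overlapping actor is BoltRef and its IsAttachedToBolt2 flag is already set.
; Grip2 snaps the bolt to socket "1" keeping world scale, sets that flag again and calls Transform2 on the bolt.
; Grip events track DoesHaveWrench, which is not read here.
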(event `VRGripInterface.OnGrip`
  (params (GrippingController :type "GripMotionControllerComponent Object Reference") (GripInformation :type "BPActorGripInformation Structure (by ref)"))
  (set `self.Does Have Wrench` true))

(event `VRGripInterface.OnGripRelease`
  (params (ReleasingController :type "GripMotionControllerComponent Object Reference") (GripInformation :type "BPActorGripInformation Structure (by ref)") (bWasSocketed :type Boolean))
  (set `self.Does Have Wrench` false))

(event `self.Sphere.OnComponentBeginOverlap`
  (params (OverlappedComponent :type "PrimitiveComponent Object Reference") (OtherActor :type "Actor Object Reference") (OtherComp :type "PrimitiveComponent Object Reference") (OtherBodyIndex :type Integer) (bFromSweep :type Boolean) (SweepResult :type "HitResult Structure (by ref)"))
  (set `self.Other Actor` OtherActor)
  (`self.Check for Bolt`))

(event `Grip2`
  (bind _bolt_ref (`self.Bolt Ref`))
  (`SceneComponent.K2_AttachToComponent` (`Actor.RootComponent` (`self.Bolt Ref`)) (`self.StaticMeshComponent`) "1" "SnapToTarget" "SnapToTarget" "KeepWorld" true)
  (set `/Game/findEmma/Blueprints/BP_Bolt.Is attached to bolt2` true _bolt_ref)
  (`/Game/findEmma/Blueprints/BP_Bolt.Transform2` _bolt_ref))

(fn `Check for Bolt`
  (returns (BoltFound :type Boolean))
  (bind _bolt_ref (`self.Bolt Ref`))
  (bind _other_actor (`self.Other Actor`))
  (`/Engine/EditorBlueprintResources/StandardMacros.IsValid` _other_actor
    (:`Is Valid`
      (if (and (`/Game/findEmma/Blueprints/BP_Bolt.Is attached to bolt2` _bolt_ref) (== _other_actor _bolt_ref))
        (`self.Grip2`)
        (return true)))))

(fn `UserConstructionScript`)