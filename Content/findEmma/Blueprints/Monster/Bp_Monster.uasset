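; Monster actor Blueprint that turns to follow the player character's facing and reacts to overlaps on its box.
; A looping timer started at BeginPlay copies the player's rotation with a yaw offset and prints a debug message when the player's height is near a threshold.
; The OnGrip event stops that timer.
; Box overlaps only print whether the other actor's display name matches the axe.
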(event `VRGripInterface.OnGrip`
  (params (GrippingController :type "GripMotionControllerComponent Object Reference") (GripInformation :type "BPActorGripInformation Structure (by ref)"))
  (`KismetSystemLibrary.K2_ClearAndInvalidateTimerHandle` (stale `Check Height Event` _returnvalue)))

(event `self.ReceiveBeginPlay`
  (`self.Check Height Event`))

(event `Check Height Event`
  (bind _returnvalue (`KismetSystemLibrary.K2_SetTimer` null "CheckHeight" 0.2 true)))

(event `self.Box.OnComponentBeginOverlap`
  (params (OverlappedComponent :type "PrimitiveComponent Object Reference") (OtherActor :type "Actor Object Reference") (OtherComp :type "PrimitiveComponent Object Reference") (OtherBodyIndex :type Integer) (bFromSweep :type Boolean) (SweepResult :type "HitResult Structure (by ref)"))
  (if (`KismetStringLibrary.EqualEqual_StrStr` (`KismetSystemLibrary.GetDisplayName` OtherActor) "BP_axe")
    (`KismetSystemLibrary.PrintString` "yes")
    (else
      (`KismetSystemLibrary.PrintString` "no"))))

(fn `CheckHeight`
  (bind (_returnvalue_x _returnvalue_y _returnvalue_z) (`KismetMathLibrary.BreakVector` (`SceneComponent.K2_GetComponentLocation` (`Actor.RootComponent` (`GameplayStatics.GetPlayerCharacter` 0)))))
  (bind (_returnvalue_roll _returnvalue_pitch _returnvalue_yaw) (`KismetMathLibrary.BreakRotator` (`SceneComponent.K2_GetComponentRotation` (`Actor.RootComponent` (`GameplayStatics.GetPlayerCharacter` 0)))))
  (`|ExecutionSequence`
    (:`then_0`
      (`self.K2_SetActorRotation` (`KismetMathLibrary.MakeRotator` _returnvalue_roll _returnvalue_pitch (- _returnvalue_yaw 270.0)) true))
    (:`then_1`
      (if (`KismetMathLibrary.NearlyEqual_FloatFloat` _returnvalue_z 100.0 50.0)
        (`KismetSystemLibrary.PrintString` "high")))))

(fn `UserConstructionScript`)