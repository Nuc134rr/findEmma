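; BP_Wrench1 is a grippable wrench for a VR game, linked to a Bolt actor.
; Gripping sets DoesHaveWrench, and releasing clears it and calls OnDraw on the Bolt.
; An unconnected chain would match the Bolt's roll and pitch and derive yaw from the right motion controller's offset along the initial right vector, but it never runs.
; The Transform event and construction script are empty.
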(event `Transform`)

(event `VRGripInterface.OnGrip`
  (params (GrippingController :type "GripMotionControllerComponent Object Reference") (GripInformation :type "BPActorGripInformation Structure (by ref)"))
  (set `self.Does Have Wrench` true))

(event `VRGripInterface.OnGripRelease`
  (params (ReleasingController :type "GripMotionControllerComponent Object Reference") (GripInformation :type "BPActorGripInformation Structure (by ref)") (bWasSocketed :type Boolean))
  (set `self.Does Have Wrench` false)
  (`/Game/findEmma/Blueprints/BP_TEGOODBOLT.On Draw` (`self.Bolt`)))

(fn `UserConstructionScript`)