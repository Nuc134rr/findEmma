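; BP_VentButton is a one-use button that completes the second notebook task when its state changes.
; The ButtonComp state-change event toggles the point light's visibility through TurnOffLight, disables the button's collision and tells the notebook to color Task2's text as complete.
; A timeline that would drive the light's intensity is present but never runs.
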(event `self.ButtonComp.OnButtonStateChanged`
  (params (ButtonState :type Boolean) (InteractingActor :type "Actor Object Reference") (InteractingComponent :type "PrimitiveComponent Object Reference"))
  (bind _notebookref (`self.notebookRef`))
  (`self.TurnOffLight`)
  (`PrimitiveComponent.SetCollisionEnabled` (`self.ButtonComp`) "NoCollision")
  (`/Game/findEmma/Blueprints/BP_notebook.changeTextColorToComplete` _notebookref (`/Game/findEmma/Blueprints/BP_notebook.Task2` _notebookref) 1))

(event `TurnOffLight`
  (`SceneComponent.ToggleVisibility` (`self.PointLight`) true))

(fn `UserConstructionScript`)