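; BP_valve is a grippable valve dial that marks itself done when turned to a target angle.
; Gripping the valve plays a sound whose pitch multiplier is the current dial angle.
; Tick tests for an exact angle match, then plays a fire cue, disables the valve's collision and sets IsValveDone.
; The check has no one-shot guard, so it repeats every frame while the angle stays on target.
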(event `self.Valve.OnGripped`
  (params (GrippingController :type "GripMotionControllerComponent Object Reference") (GripInformation :type "BPActorGripInformation Structure (by ref)"))
  (`GameplayStatics.PlaySoundAtLocation` "/Game/VRTemplateContent/VRTemplate/Audio/Fire01.Fire01" (0.0 0.0 0.0) (struct) 1.0 (`VRDialComponent.CurrentDialAngle` (`self.Valve`)) 0.0 null null null))

(event `self.ReceiveTick`
  (params (DeltaSeconds :type "Float (single-precision)"))
  (if (== (`VRDialComponent.CurrentDialAngle` (`self.Valve`)) 20.0)
    (`GameplayStatics.PlaySoundAtLocation` "/Game/VRTemplateContent/VRTemplate/Audio/Fire_Cue.Fire_Cue" (0.0 0.0 0.0) (struct) 1.0 1.0 0.0 null null null)
    (`PrimitiveComponent.SetCollisionEnabled` (`self.Valve`) "NoCollision")
    (set `self.bIsValveDone` true)))

(fn `UserConstructionScript`)