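; BP_FakeCan is a grippable VR can with a hidden-object task that only works on day two.
; Shortly after BeginPlay it denies gripping unless the current level is second in the pawn's LevelNames.
; Gripping the Lid starts a looping timer that polls InnerCan's world roll against WinConditionAngle within a tolerance.
; A match hides InnerCan, stops the timer and marks Task1 complete in the notebook.
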(event `self.ReceiveBeginPlay`
  (`KismetSystemLibrary.Delay` 1.0)
  (bind _returnvalue (`GameplayStatics.GetCurrentLevelName` true))
  (if (!= (`KismetArrayLibrary.Array_Find` (`/Game/VRExpansion/Vive/Vive_PawnCharacter.Level_Names` (cast `/Game/VRExpansion/Vive/Vive_PawnCharacter` (`GameplayStatics.GetPlayerPawn` 0) :!pure true)) _returnvalue) 1)
    (`KismetSystemLibrary.PrintString` "not day two")
    (`self.SetDenyGripping` true)))

(event `self.Lid .OnGripped`
  (params (GrippingController :type "GripMotionControllerComponent Object Reference") (GripInformation :type "BPActorGripInformation Structure (by ref)"))
  (bind _returnvalue (`KismetSystemLibrary.K2_SetTimer` null "CheckForAngle" 0.1 true)))

(event `WinCondition`
  (bind _notebookref (`self.notebookRef`))
  (`SceneComponent.SetVisibility` (`self.InnerCan`) false false)
  (`KismetSystemLibrary.K2_ClearAndInvalidateTimerHandle` (stale `self.Lid .OnGripped` _returnvalue))
  (`/Game/findEmma/Blueprints/BP_notebook.changeTextColorToComplete` _notebookref (`/Game/findEmma/Blueprints/BP_notebook.Task1` _notebookref) 0))

(fn `CheckForAngle`
  (if (`KismetMathLibrary.NearlyEqual_FloatFloat` (.roll (`SceneComponent.K2_GetComponentRotation` (`self.InnerCan`))) (`self.WinConditionAngle`) 10.0)
    (`self.WinCondition`)))

(fn `UserConstructionScript`)