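; Generator Blueprint for a VR wrench-and-bolt interaction driven by the Vive pawn.
; When the wrench's root component overlaps the sphere and DoesHaveWrench is set, the wrench snaps to the bolt's WrenchAttach socket, is flagged attached, and the pawn's Rotation is called.
; A separate BoltRotation event copies the pawn's BoltRot onto the bolt's relative rotation.
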(event `self.Sphere.OnComponentBeginOverlap`
  (params (OverlappedComponent :type "PrimitiveComponent Object Reference") (OtherActor :type "Actor Object Reference") (OtherComp :type "PrimitiveComponent Object Reference") (OtherBodyIndex :type Integer) (bFromSweep :type Boolean) (SweepResult :type "HitResult Structure (by ref)"))
  (set `self.Other Comp` OtherComp)
  (bind _bolted (`self.CheckForWrench`))
  (if _bolted
    (`SceneComponent.K2_AttachToComponent` (`Actor.RootComponent` (`self.WrenchRef`)) (`self.Bolt`) "WrenchAttach" "SnapToTarget" "SnapToTarget" "KeepWorld" true)
    (set `/Game/findEmma/Blueprints/Wrench.IsAttachedTo Bolt` true (`self.WrenchRef`))
    (bind _asvive_pawn_character (cast `/Game/VRExpansion/Vive/Vive_PawnCharacter` (`GameplayStatics.GetPlayerPawn` 0)))
    (`/Game/VRExpansion/Vive/Vive_PawnCharacter.Rotation` _asvive_pawn_character)))

(event `Bolt Rotation`
  (bind (_bolt_rot_roll _bolt_rot_pitch _bolt_rot_yaw) (`KismetMathLibrary.BreakRotator` (`/Game/VRExpansion/Vive/Vive_PawnCharacter.Bolt Rot` (`self.Vive Pawn`))))
  (`SceneComponent.K2_SetRelativeRotation` (`self.Bolt`) (`KismetMathLibrary.MakeRotator` _bolt_rot_roll _bolt_rot_pitch _bolt_rot_yaw) false false))

(fn `CheckForWrench`
  (returns (Bolted :type Boolean))
  (bind _wrenchref (`self.WrenchRef`))
  (bind _other_comp (`self.Other Comp`))
  (`/Engine/EditorBlueprintResources/StandardMacros.IsValid` _other_comp
    (:`Is Valid`
      (if (and (`/Game/findEmma/Blueprints/Wrench.DoesHaveWrench` _wrenchref) (== _other_comp (`Actor.RootComponent` _wrenchref)))
        (return true)))))

(fn `UserConstructionScript`)