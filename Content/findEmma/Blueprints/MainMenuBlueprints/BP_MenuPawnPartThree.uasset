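; VR main menu pawn that disables movement and uses motion controllers as laser pointers for Start and Quit buttons.
; A visibility trace along the active controller's negated up vector runs each tick with debug drawing; either trigger switches the active hand.
; Only right-hand presses act, matching hit actors by display name.
; Start plays a fade sequence before opening Level_Day1; Quit spawns Yes/No confirmation actors.
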(event `self.ReceiveBeginPlay`
  (`CharacterMovementComponent.DisableMovement` (`self.CharacterMovement`))
  (set `self.TracingController` (`self.RightMotionController`)))

(event `self.ReceiveTick`
  (params (DeltaSeconds :type "Float (single-precision)"))
  (`self.TraceForUI`))

(event `InputAction|UseHeldObjectLeft`
  (params (Key :type "Key Structure"))
  (:`Pressed`
    (set `self.TracingController` (`self.LeftMotionController`))
    (bind _hitresult (`self.TraceForUI`))
    (if _hitresult
      _)))

(event `InputAction|UseHeldObjectRight`
  (params (Key :type "Key Structure"))
  (:`Pressed`
    (set `self.TracingController` (`self.RightMotionController`))
    (bind (_hitresult _outhitactor) (`self.TraceForUI`))
    (if _hitresult
      (bind _returnvalue (`KismetSystemLibrary.GetDisplayName` _outhitactor))
      (if (`KismetStringLibrary.EqualEqual_StrStr` _returnvalue "BP_StartButton")
        ;[1 1 1] Starts the game
        (bind (_outactor _returnvalue_2) (`LevelSequencePlayer.CreateLevelSequencePlayer` "/Game/findEmma/Blueprints/FadeOut.FadeOut"))
        (`MovieSceneSequencePlayer.Play` _returnvalue_2)
        (`KismetSystemLibrary.Delay` 5.0)
        (`GameplayStatics.OpenLevel` "Level_Day1")
        (elif (`KismetStringLibrary.EqualEqual_StrStr` _returnvalue "BP_QuitButton")
          ;[1 1 1] "Are You Sure?" assets
          (bind _returnvalue_3 (`|SpawnActorFromClass` "/Game/findEmma/Blueprints/MainMenuBlueprints/BP_QuitButtonYes.BP_QuitButtonYes_C" (`self.YesTransform`) "Undefined" "OverrideRootScale" null null))
          (bind _returnvalue_4 (`|SpawnActorFromClass` "/Game/findEmma/Blueprints/MainMenuBlueprints/BP_QuitButtonNo.BP_QuitButtonNo_C" (`self.NoTransform`) "Undefined" "OverrideRootScale" null null))
          (bind _returnvalue_5 (`|SpawnActorFromClass` "/Game/findEmma/Blueprints/MainMenuBlueprints/BP_QuitButton2.BP_QuitButton2_C" (`self.AYSTransform`) "Undefined" "OverrideRootScale" null null))
          (elif (`KismetStringLibrary.EqualEqual_StrStr` _returnvalue "BP_QuitButtonNo")
            (`self.K2_DestroyActor` _returnvalue_5)
            (`self.K2_DestroyActor` _returnvalue_3)
            (`self.K2_DestroyActor` _returnvalue_4)
            (elif (`KismetStringLibrary.EqualEqual_StrStr` _returnvalue "BP_QuitButtonYes")
              (`KismetSystemLibrary.QuitGame` null "Quit"))))))))

(fn `TraceForUI`
  (returns (HitResult :type Boolean) (OutHitActor :type "Actor Object Reference"))
  (bind _tracingcontroller (`self.TracingController`))
  (bind _returnvalue (`SceneComponent.K2_GetComponentLocation` _tracingcontroller))
  (bind (_outhit _returnvalue_2) (`KismetSystemLibrary.LineTraceSingle` :`Start` _returnvalue :`End` (+ _returnvalue (* (`KismetMathLibrary.GetUpVector` (`SceneComponent.K2_GetComponentRotation` _tracingcontroller)) -5000.0)) :`TraceChannel` "TraceTypeQuery1" :`bTraceComplex` true :`DrawDebugType` "ForOneFrame"))
  (return _returnvalue_2 (`.HitActor` (`GameplayStatics.BreakHitResult` _outhit))))

(fn `UserConstructionScript`
  (`parent.UserConstructionScript`))