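; VR character for the main menu, with character movement disabled on BeginPlay so it cannot walk.
; Every tick it runs a debug-drawn Visibility line trace from the right motion controller along the VR camera's forward vector, rather than the controller's.
; The hit actor is cast to BP_BaseMenuProp, but nothing follows a successful cast, so detecting a menu prop has no effect here.
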(event `self.ReceiveBeginPlay`
  (`CharacterMovementComponent.DisableMovement` (`self.CharacterMovement`)))

(event `self.ReceiveTick`
  (params (DeltaSeconds :type "Float (single-precision)"))
  (bind _returnvalue (`SceneComponent.K2_GetComponentLocation` (`self.RightMotionController`)))
  (bind _outhit (`KismetSystemLibrary.LineTraceSingle` :`Start` _returnvalue :`End` (+ _returnvalue (* (`KismetMathLibrary.GetForwardVector` (`SceneComponent.K2_GetComponentRotation` (`self.VRReplicatedCamera`))) 5000.0)) :`TraceChannel` "TraceTypeQuery1" :`bTraceComplex` true :`DrawDebugType` "ForOneFrame"))
  (if (`.bSuccess` (cast `/Game/findEmma/Blueprints/MainMenuBlueprints/BP_BaseMenuProp` (`.HitActor` (`GameplayStatics.BreakHitResult` _outhit)) :!pure true))
    _))

(fn `UserConstructionScript`
  (`parent.UserConstructionScript`))