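; Bolt actor that the wrench can snap onto when something enters its sphere trigger.
; On overlap it calls CheckForWrench, which tests whether the wrench is held and is the overlapping component, but sets no state in this graph.
; If the separate Bolted flag is true, the wrench root snaps to the bolt mesh's WrenchAttach socket, keeping world scale, and the wrench is marked attached.
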(event `self.Sphere.OnComponentBeginOverlap`
  (params (OverlappedComponent :type "PrimitiveComponent Object Reference") (OtherActor :type "Actor Object Reference") (OtherComp :type "PrimitiveComponent Object Reference") (OtherBodyIndex :type Integer) (bFromSweep :type Boolean) (SweepResult :type "HitResult Structure (by ref)"))
  (set `self.Other Comp` OtherComp)
  (`self.Check For Wrench`)
  (if (`self.Bolted`)
    (`SceneComponent.K2_AttachToComponent` (`Actor.RootComponent` (`self.WrenchRef`)) (`self.StaticMeshComponent`) "WrenchAttach" "SnapToTarget" "SnapToTarget" "KeepWorld" true)
    (set `/Game/findEmma/Blueprints/Wrench.IsAttachedTo Bolt` true (`self.WrenchRef`))))

(fn `Check For Wrench`
  (bind _wrenchref (`self.WrenchRef`))
  (bind _other_comp (`self.Other Comp`))
  (`/Engine/EditorBlueprintResources/StandardMacros.IsValid` _other_comp
    (:`Is Valid`
      (if (and (`/Game/findEmma/Blueprints/Wrench.DoesHaveWrench` _wrenchref) (== _other_comp (`Actor.RootComponent` _wrenchref)))
        (return)))))

(fn `UserConstructionScript`)