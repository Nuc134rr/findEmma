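; VR wrench that snaps onto bolts and turns them with motion controller roll.
; While held, Tick scans all Bolt actors for a bolted-in one of matching TypeID near the controller's pointer, then attaches to it.
; Within range, roll changes in one direction feed the bolt's AddRotationValue; a true result reattaches the wrench to the controller.
; An interpolated transform lerp eases the wrench between poses.
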(event `self.ReceiveTick`
  (params (DeltaSeconds :type "Float (single-precision)"))
  (if (`self.In Hand`)
    (`|ExecutionSequence`
      (:`then_0`
        (if (`self.Bolt Found`)
          (if (not (>= (`KismetMathLibrary.VSize` (- (`self.K2_GetActorLocation` (`self.Active Screw`)) (`self.Bolt Pointer Location`))) (`self.Dissconnet Distance`)))
            (`|ExecutionSequence`
              (:`then_0`
                (set `self.NewRotation` (`self.Motion Controller Roll `))
                (set `self.Delta Rotation` (- (`self.Start Rotation`) (`self.NewRotation`)))
                (if (> (`self.Delta Rotation`) 0.0)
                  (bind _bolt_out (`/Game/findEmma/Bolt.Add Rotation Value` (`self.Active Screw`) (`self.Delta Rotation`)))
                  (if _bolt_out
                    (`SceneComponent.K2_AttachToComponent` (`self.RootComponent`) (`self.Active Motion Controller`) "None" "KeepRelative" "KeepRelative" "KeepRelative" true)
                    (set `self.Bolt Found` false)
                    (set `self.From Transfrom` (`SceneComponent.GetRelativeTransform` (`self.RootComponent`)))
                    (set `self.To Transfrom` (`self.Initial In Hand Transfrom`))
                    (set `self.Transform Blending Coeff` 0.0))))
              (:`then_1`
                (set `self.Start Rotation` (`self.NewRotation`)))))
          (else
            (bind _outactors (`GameplayStatics.GetAllActorsOfClass` "/Game/findEmma/Bolt.Bolt_C"))
            (for _array_element _outactors
              (if (and (`/Game/findEmma/Bolt.Is Bolted in` _array_element) (== (`/Game/findEmma/Bolt.Type ID` _array_element) (`self.Type ID`)))
                (if (<= (`KismetMathLibrary.VSize` (- (`self.K2_GetActorLocation` _array_element) (`self.Bolt Pointer Location`))) (`self.connection Distance`))
                  (set `self.Active Screw` _array_element)
                  (`self.K2_AttachToActor` (`self.Active Screw`) "None" "KeepRelative" "KeepRelative" "KeepRelative")
                  (set `self.From Transfrom` (`SceneComponent.GetRelativeTransform` (`self.StaticMeshComponent`)))
                  (set `self.To Transfrom` (`KismetMathLibrary.MakeTransform` (0.0 0.0 0.0) (struct :`Pitch` 180.0)))
                  (set `self.Transfrom Blending Cofficent` 0)
                  (set `self.Bolt Found` true)
                  (set `self.Start Rotation` (`self.Motion Controller Roll `))))))))
      (:`then_1`
        (if (< (`self.Transform Blending Coeff`) 1.0)
          (set `self.Transform Blending Coeff` (`KismetMathLibrary.FInterpTo` (`self.Transform Blending Coeff`) 1.0 DeltaSeconds 10.0))
          (`SceneComponent.K2_SetRelativeTransform` (`self.K2_GetRootComponent`) (`KismetMathLibrary.TLerp` (`self.From Transfrom`) (`self.To Transfrom`) (`self.Transform Blending Coeff`)) false false))))))

(fn `UserConstructionScript`)