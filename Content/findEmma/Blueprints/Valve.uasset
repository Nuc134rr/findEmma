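; Valve is a grippable dial puzzle that counts as won when it is turned to exactly 360 degrees.
; Grip and drop events set a Gripped flag, and Tick polls the dial angle, replaying a weapon-fire sound every frame while gripped, with pitch derived from the angle.
; At the target angle it plays the sound at default pitch and disables the dial's collision, with debug prints throughout.
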(event `self.Valve.OnDropped`
  (params (GrippingController :type "GripMotionControllerComponent Object Reference") (GripInformation :type "BPActorGripInformation Structure (by ref)") (bWasSocketed :type Boolean))
  ;[1 1 1] UnGripped
  (`KismetSystemLibrary.PrintString` "UnGripped")
  (set `self.Gripped` false))

(event `self.Valve.OnGripped`
  (params (GrippingController :type "GripMotionControllerComponent Object Reference") (GripInformation :type "BPActorGripInformation Structure (by ref)"))
  ;[1 1 1] Gripped
  (`KismetSystemLibrary.PrintString` "Gripped")
  (set `self.Gripped` true))

(event `self.ReceiveTick`
  (params (DeltaSeconds :type "Float (single-precision)"))
  (bind _valve (`self.Valve`))
  ;[1 1 1] Checking
  (`KismetSystemLibrary.PrintString` (`KismetStringLibrary.Conv_DoubleToString` (`VRDialComponent.CurrentDialAngle` _valve)))
  (if (== (`VRDialComponent.CurrentDialAngle` _valve) 360.0)
    (`KismetSystemLibrary.PrintString` "Won")
    ;[1 1 1] Win
    (`GameplayStatics.PlaySoundAtLocation` "/Game/VRExpansion/FirstPersonBP/FirstPerson/Audio/FirstPersonTemplateWeaponFire02.FirstPersonTemplateWeaponFire02" (0.0 0.0 0.0) (struct) 1.0 1.0 0.0 null null null)
    (`PrimitiveComponent.SetCollisionEnabled` (`self.Valve`) "NoCollision")
    (elif (`self.Gripped`)
      (`GameplayStatics.PlaySoundAtLocation` "/Game/VRExpansion/FirstPersonBP/FirstPerson/Audio/FirstPersonTemplateWeaponFire02.FirstPersonTemplateWeaponFire02" (0.0 0.0 0.0) (struct) 1.0 (- (`VRDialComponent.CurrentDialAngle` _valve) 100.0) 0.0 null null null))))

(fn `UserConstructionScript`)