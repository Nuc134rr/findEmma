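; VR bolt that the player tightens by turning a wrench with the right Vive motion controller.
; When the held wrench overlaps the sphere, it snaps to the bolt's socket, sets a roll goal and starts a looping timer on Tick.
; Tick derives wrench roll from the atan2 angle between bolt and controller, also offsetting the bolt mesh by that angle.
; Near the goal, the wrench detaches and the bolt is marked bolted.
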(event `self.Sphere.OnComponentBeginOverlap`
  (params (OverlappedComponent :type "PrimitiveComponent Object Reference") (OtherActor :type "Actor Object Reference") (OtherComp :type "PrimitiveComponent Object Reference") (OtherBodyIndex :type Integer) (bFromSweep :type Boolean) (SweepResult :type "HitResult Structure (by ref)"))
  (set `self.Other Actor` OtherActor)
  (`self.Check For Wrench`))

(event `grip`
  (bind _wrench_ref (`self.Wrench Ref`))
  (bind _returnvalue_roll (`KismetMathLibrary.BreakRotator` (`SceneComponent.K2_GetComponentRotation` (`Actor.RootComponent` _wrench_ref))))
  (if (not (`self.Bolted`))
    (set `self.WorldLocation` (`SceneComponent.K2_GetComponentLocation` (`self.StaticMeshComponent`)))
    (`SceneComponent.K2_AttachToComponent` (`Actor.RootComponent` (`self.Wrench Ref`)) (`self.StaticMeshComponent`) "1" "SnapToTarget" "SnapToTarget" "KeepWorld" true)
    (set `/Game/findEmma/Blueprints/BP_Wrench1.Is attached to Bolt` true _wrench_ref)
    (set `self.Goal` (+ _returnvalue_roll 60.0))
    (bind _returnvalue (`KismetSystemLibrary.K2_SetTimer` null "Tick" 0.1 true))))

(event `On Draw`
  (`KismetSystemLibrary.K2_ClearAndInvalidateTimerHandle` (stale `grip` _returnvalue)))

(event `Transform2`)

(event `self.ReceiveTick`
  (params (DeltaSeconds :type "Float (single-precision)")))

(fn `Check For Wrench`
  (returns (Bolted :type Boolean))
  (bind _wrench_ref (`self.Wrench Ref`))
  (bind _other_actor (`self.Other Actor`))
  (`/Engine/EditorBlueprintResources/StandardMacros.IsValid` _other_actor
    (:`Is Valid`
      (if (and (`/Game/findEmma/Blueprints/BP_Wrench1.Does Have Wrench` _wrench_ref) (== _other_actor _wrench_ref))
        (`self.grip`)
        (return true)))))

(fn `Tick`
  (bind (_returnvalue_roll _returnvalue_pitch _returnvalue_yaw) (`KismetMathLibrary.BreakRotator` (`SceneComponent.K2_GetComponentRotation` (`self.StaticMeshComponent`))))
  (bind (_returnvalue_x _returnvalue_y) (`KismetMathLibrary.BreakVector` (- (`SceneComponent.K2_GetComponentLocation` (`self.StaticMeshComponent`)) (`SceneComponent.K2_GetComponentLocation` (`VRBaseCharacter.RightMotionController` (cast `/Game/VRExpansion/Vive/Vive_PawnCharacter` (`Controller.K2_GetPawn` (`GameplayStatics.GetPlayerController` 0)) :!pure true))))))
  (bind _returnvalue (`KismetMathLibrary.DegAtan2` _returnvalue_y _returnvalue_x))
  (if (not (`self.Bolted`))
    (if (<= _returnvalue 0.0)
      (bind _output_get (set `self.Whatever` (* (`KismetMathLibrary.Abs` _returnvalue) 2.0)))
      (`KismetSystemLibrary.PrintString` (`KismetStringLibrary.Conv_DoubleToString` _output_get))
      (else
        (set `self.Whatever` _returnvalue)))
    (`self.K2_SetActorRotation` (`self.Wrench Ref`) (`KismetMathLibrary.MakeRotator` _output_get) false)
    (`SceneComponent.K2_SetRelativeLocationAndRotation` (`self.StaticMeshComponent`) (+ (`self.WorldLocation`) (`KismetMathLibrary.MakeVector` (`KismetMathLibrary.Abs` _returnvalue))) (`KismetMathLibrary.MakeRotator` _returnvalue_roll _returnvalue_pitch _returnvalue_yaw) false false)
    (if (`KismetMathLibrary.NearlyEqual_FloatFloat` (`self.Goal`) _output_get 10.0)
      (`KismetSystemLibrary.PrintString` "gaming")
      (`SceneComponent.K2_DetachFromComponent` (`Actor.RootComponent` (`self.Wrench Ref`)) "KeepRelative" "KeepRelative" "KeepWorld" true)
      (set `self.Bolted` true))))

(fn `UserConstructionScript`)