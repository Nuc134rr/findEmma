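; BP_Bed is a bed prop that lets the player sleep once the day is complete, teleporting them to the map.
; Two box triggers run identical overlap logic, skipped in Level_StartMenu, and call CheckForSleep.
; That function confirms the player pawn and the notebook's DayComplete flag, printing debug feedback and holding a placeholder comment for a fade.
; On success, the Vive pawn's TeleportToMap is called.
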(event `self.Box.OnComponentBeginOverlap`
  (params (OverlappedComponent :type "PrimitiveComponent Object Reference") (OtherActor :type "Actor Object Reference") (OtherComp :type "PrimitiveComponent Object Reference") (OtherBodyIndex :type Integer) (bFromSweep :type Boolean) (SweepResult :type "HitResult Structure (by ref)"))
  (bind _returnvalue (`GameplayStatics.GetCurrentLevelName` true))
  (if (not (`KismetStringLibrary.EqualEqual_StrStr` _returnvalue "Level_StartMenu"))
    (bind _shouldteleport (`self.CheckForSleep` OtherActor))
    (if _shouldteleport
      (`/Game/VRExpansion/Vive/Vive_PawnCharacter.Teleport to Map` (cast `/Game/VRExpansion/Vive/Vive_PawnCharacter` (`GameplayStatics.GetPlayerPawn` 0) :!pure true)))))

(event `self.Box1.OnComponentBeginOverlap`
  (params (OverlappedComponent :type "PrimitiveComponent Object Reference") (OtherActor :type "Actor Object Reference") (OtherComp :type "PrimitiveComponent Object Reference") (OtherBodyIndex :type Integer) (bFromSweep :type Boolean) (SweepResult :type "HitResult Structure (by ref)"))
  (bind _returnvalue (`GameplayStatics.GetCurrentLevelName` true))
  (if (not (`KismetStringLibrary.EqualEqual_StrStr` _returnvalue "Level_StartMenu"))
    (bind _shouldteleport (`self.CheckForSleep` OtherActor))
    (if _shouldteleport
      (`/Game/VRExpansion/Vive/Vive_PawnCharacter.Teleport to Map` (cast `/Game/VRExpansion/Vive/Vive_PawnCharacter` (`GameplayStatics.GetPlayerPawn` 0) :!pure true)))))

(fn `CheckForSleep`
  (params (OverlappedActor :type "Actor Object Reference"))
  (returns (ShouldTeleport :type Boolean))
  (if (== OverlappedActor (`GameplayStatics.GetPlayerPawn` 0))
    (if (`/Game/findEmma/Blueprints/Props/BP_notebook.DayComplete` (`self.notebookRef`))
      ;[1 1 1] SHAWN PUT YO CALL FADE EVENT HERE
      (`KismetSystemLibrary.PrintString` "thumbs up")
      (return true)
      (else
        (`KismetSystemLibrary.PrintString` "thumbs down")
        (return false)))))

(fn `UserConstructionScript`)