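; BP_Generator is a grippable generator prop that completes the second notebook task in two stages: pull the cord, then hit it with the wrench.
; Tick sizes the cable to the handle's distance, force-dropping it past a limit and playing a one-time ding that marks it pulled.
; Releasing the handle triggers a MoveComponentTo toward its cached start position.
; Once pulled, overlaps from one wrench, matched by object name, deplete Health to complete the task.
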(event `self.ReceiveTick`
  (params (DeltaSeconds :type "Float (single-precision)"))
  (bind _returnvalue (`SceneComponent.K2_GetComponentLocation` (`self.Gene`)))
  (bind _returnvalue_2 (- (`KismetMathLibrary.Vector_Distance` _returnvalue (`SceneComponent.K2_GetComponentLocation` (`self.Cube`))) 100.0))
  (if (< _returnvalue_2 100.0)
    (set `CableComponent.CableLength` _returnvalue_2 (`self.Cable`))
    (else
      (`GripMotionControllerComponent.DropObject` (stale `self.Cube.OnGripped` _output_get) (`self.Cube`) 0 false (0.0 0.0 0.0) (0.0 0.0 0.0))
      (if (`self.Condition`)
        (set `self.Condition` false)
        (`GameplayStatics.PlaySoundAtLocation` "/Game/findEmma/Sound/ding.ding" _returnvalue (struct) 1.0 1.0 0.0 null null null)
        (set `self.Pulled` true)))))

(event `self.Box.OnComponentBeginOverlap`
  (params (OverlappedComponent :type "PrimitiveComponent Object Reference") (OtherActor :type "Actor Object Reference") (OtherComp :type "PrimitiveComponent Object Reference") (OtherBodyIndex :type Integer) (bFromSweep :type Boolean) (SweepResult :type "HitResult Structure (by ref)"))
  (bind _notebookref (`self.notebookRef`))
  ;[1 1 1] Wrench Overlap
  (if (`self.Check`)
    (if (`self.Pulled`)
      (if (`KismetStringLibrary.EqualEqual_StrStr` (`KismetSystemLibrary.GetObjectName` OtherActor) "BP_THEGOODWRENCH_2")
        (set `self.Health` (- (`self.Health`) 1))
        (if (<= (`self.Health`) 0)
          (`/Game/findEmma/Blueprints/Props/BP_notebook.changeTextColorToComplete` _notebookref (`/Game/findEmma/Blueprints/Props/BP_notebook.Task2` _notebookref) 1)
          (set `self.Check` false))))))

(event `self.Cube.OnGripped`
  (params (GrippingController :type "GripMotionControllerComponent Object Reference") (GripInformation :type "BPActorGripInformation Structure (by ref)"))
  (bind _output_get (set `self.Gripping Controller` GrippingController))
  (goto _label :!via `Stop`))

(event `self.Cube.OnDropped`
  (params (GrippingController :type "GripMotionControllerComponent Object Reference") (GripInformation :type "BPActorGripInformation Structure (by ref)") (bWasSocketed :type Boolean))
  (`KismetSystemLibrary.MoveComponentTo` (`self.Cube`) (stale `self.ReceiveBeginPlay` _output_get) (`SceneComponent.K2_GetComponentRotation` (`self.Cube`)) false false 0.5 :!label _label))

(event `self.ReceiveBeginPlay`
  (bind _output_get (set `self.cube location` (`KismetMathLibrary.MakeVector` (.x (`SceneComponent.K2_GetComponentLocation` (`self.Cube`))) (.y (`SceneComponent.K2_GetComponentLocation` (`self.Cube`))) (+ (.z (`SceneComponent.K2_GetComponentLocation` (`self.Cube`))) 2.0)))))

(fn `UserConstructionScript`)