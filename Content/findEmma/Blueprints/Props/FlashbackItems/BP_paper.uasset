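; BP_paper is a grippable paper prop that triggers a flashback when the VR player grips it.
; On the first allowed grip it calls FlashbackType with index 0, flags the Vive pawn as holding a flashback item, and disables further gripping.
; It then marks the second task as complete in the referenced notebook.
; FlashbackType is an empty stub in this Blueprint.
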(event `VRGripInterface.OnGrip`
  (params (GrippingController :type "GripMotionControllerComponent Object Reference") (GripInformation :type "BPActorGripInformation Structure (by ref)"))
  (bind _notebookref (`self.notebookRef`))
  ;[1 1 1] trigger flashback
  (bind _returnvalue (`VRGripInterface.DenyGripping` null))
  (if (not _returnvalue)
    (`/Game/findEmma/Blueprints/I_Flashbacks.FlashbackType` 0)
    (set `/Game/VRExpansion/Vive/Vive_PawnCharacter.bIsFlashbackGripped` true (cast `/Game/VRExpansion/Vive/Vive_PawnCharacter` (`GameplayStatics.GetPlayerPawn` 0) :!pure true))
    (`self.SetDenyGripping` true)
    (`/Game/findEmma/Blueprints/Props/BP_notebook.changeTextColorToComplete` _notebookref (`/Game/findEmma/Blueprints/Props/BP_notebook.Task2` _notebookref) 1)))

(fn `FlashbackType`
  (params (FlashbackInt :type Integer))
  (return))

(fn `UserConstructionScript`)