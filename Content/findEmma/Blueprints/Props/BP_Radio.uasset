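; BP_Radio is a VR radio-tuning puzzle where the player turns two grip dials to match a target wave line.
; BeginPlay picks random snap angles for both dials and scales a Checker to show the target.
; Each dial snap rescales the Line, left on X and right on Z, then compares both angles.
; A match plays a ding, locks and drops the dials, completes a notebook task and can start the switchboard task.
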(event `self.Dial_L.OnDialHitSnapAngle`
  (params (DialMilestoneAngle :type "Float (single-precision)"))
  ;[1 1 1] Scale
  (`self.Scale`))

(event `self.Dial_R.OnDialHitSnapAngle`
  (params (DialMilestoneAngle :type "Float (single-precision)"))
  ;[1 1 1] Scale
  (`self.Scale`))

(event `Scale`
  ;[1 1 1] Scale
  (bind _output_get (set `self.Dial R` (* (`KismetMathLibrary.Conv_DoubleToVector` (`VRDialComponent.CurrentDialAngle` (`self.Dial_R`))) (0.0 0.0 0.0006))))
  (bind _output_get_2 (set `self.Dial L ` (* (`KismetMathLibrary.Conv_DoubleToVector` (`VRDialComponent.CurrentDialAngle` (`self.Dial_L`))) (0.0014 0.0 0.0))))
  (`SceneComponent.SetWorldScale3D` (`self.Line`) (+ (+ _output_get _output_get_2) (0.25 0.05 0.25)))
  (`self.Check`))

(event `Reset`
  ;[1 1 1] Scale
  (`VRDialComponent.SetDialAngle` (`self.Dial_L`) 0.0 false)
  (`VRDialComponent.SetDialAngle` (`self.Dial_R`) 0.0 false)
  (`VRDialComponent.ResetInitialDialLocation` (`self.Dial_L`))
  (`VRDialComponent.ResetInitialDialLocation` (`self.Dial_R`))
  (`SceneComponent.SetWorldScale3D` (`self.Line`) (`self.Reset Vector`))
  (`self.Scale`))

(event `Check`
  (bind _notebookref (`self.notebookRef`))
  ;[1 1 1] Check
  (if (and (== (`VRDialComponent.CurrentDialAngle` (`self.Dial_R`)) (`self.Dial R Check`)) (== (`VRDialComponent.CurrentDialAngle` (`self.Dial_L`)) (`self.Dial L Check`)))
    (`KismetSystemLibrary.PrintString` "Good Job You Won!!!!!")
    (`GameplayStatics.PlaySound2D` "/Game/findEmma/Sound/ding.ding" 5.0 1.0 0.0 null null)
    (`self.DenyGripAll`)
    (`/Game/findEmma/Blueprints/Props/BP_notebook.changeTextColorToComplete` _notebookref (`/Game/findEmma/Blueprints/Props/BP_notebook.Task3` _notebookref) 2)
    (bind _returnvalue (`GameplayStatics.GetCurrentLevelName` true))
    (if (and (== (`KismetArrayLibrary.Array_Find` (`/Game/VRExpansion/Vive/Vive_PawnCharacter.Level_Names` (cast `/Game/VRExpansion/Vive/Vive_PawnCharacter` (`GameplayStatics.GetPlayerPawn` 0) :!pure true)) _returnvalue) 2) (`/Game/findEmma/Blueprints/Props/BP_Vent.CanTurnOnSwitchboard` (`self.VentRef`)) true)
      (`/Game/findEmma/Meshes/Switchboard/BP_Switchboard.SwitchboardTaskStart` (`self.SwitchboardRef`)))))

(event `self.ReceiveBeginPlay`
  ;[1 1 1] Set Win Condition
  (`self.Win`))

(event `DenyGripAll`
  (set `VRDialComponent.bDenyGripping` true (`self.Dial_R`))
  (set `VRDialComponent.bDenyGripping` true (`self.Dial_L`))
  (for _array_element (`|MakeArray` (`self.Dial_R`) (`self.Dial_L`))
    (`KismetSystemLibrary.Delay` 0.1)
    (`GripMotionControllerComponent.DropComponent` (`self.Gripping Controller`) _array_element false (0.0 0.0 0.0) (0.0 0.0 0.0))))

(event `Win`
  (bind _outitem (`KismetArrayLibrary.Array_Random` (`|MakeArray` 20.0 40.0 60.0 80.0 100.0 120.0 140.0 160.0 180.0 :!type "Float (single-precision)")))
  ;[1 1 1] Set Win Condition
  (set `self.Dial R Check` _outitem)
  (set `self.Dial L Check` _outitem)
  (`SceneComponent.SetWorldScale3D` (`self.Checker`) (+ (+ (* (`KismetMathLibrary.Conv_DoubleToVector` (`self.Dial R Check`)) (0.0 0.0 0.0006)) (* (`KismetMathLibrary.Conv_DoubleToVector` (`self.Dial L Check`)) (0.0014 0.0 0.0))) (0.25 0.05 0.25))))

(event `self.Dial_L.OnGripped`
  (params (GrippingController :type "GripMotionControllerComponent Object Reference") (GripInformation :type "BPActorGripInformation Structure (by ref)"))
  (if (not (and (== (`VRDialComponent.CurrentDialAngle` (`self.Dial_R`)) (`self.Dial R Check`)) (== (`VRDialComponent.CurrentDialAngle` (`self.Dial_L`)) (`self.Dial L Check`))))
    (set `self.Gripping Controller` GrippingController)))

(event `self.Dial_R.OnGripped`
  (params (GrippingController :type "GripMotionControllerComponent Object Reference") (GripInformation :type "BPActorGripInformation Structure (by ref)"))
  (if (not (and (== (`VRDialComponent.CurrentDialAngle` (`self.Dial_R`)) (`self.Dial R Check`)) (== (`VRDialComponent.CurrentDialAngle` (`self.Dial_L`)) (`self.Dial L Check`))))
    (set `self.Gripping Controller` GrippingController)))

(fn `UserConstructionScript`)