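; BP_notebook is a notebook prop that tracks completion of three tasks for the day.
; Its ChangeTextColorToComplete function recolors the given text render, plays a ding and sets the completion flag matching the task index.
; Once all three flags are true it sets DayComplete; otherwise it prints a reminder that tasks remain.
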(fn `changeTextColorToComplete`
  (params (Text :type "TextRenderComponent Object Reference") (CompletedTask :type Integer))
  (`TextRenderComponent.SetTextRenderColor` Text (`self.TaskComplete`))
  (`GameplayStatics.PlaySound2D` "/Game/findEmma/Sound/ding.ding" 1.0 1.0 0.0 null null)
  (switch `int` CompletedTask
    (:`0`
      (bind _output_get (set `self.TaskOneCompleted` true)))
    (:`1`
      (bind _output_get_2 (set `self.TaskTwoCompleted` true)))
    (:`2`
      (bind _output_get_3 (set `self.TaskThreeCompleted` true))))
  (if (and _output_get _output_get_2 _output_get_3)
    (set `self.DayComplete` true)
    (else
      (`KismetSystemLibrary.PrintString` "you still have tasks to do"))))

(fn `UserConstructionScript`)