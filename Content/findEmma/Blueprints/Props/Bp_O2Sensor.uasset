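; O2 sensor prop: a VR valve puzzle that locks itself unless the current level is first in the pawn's LevelNames.
; Gripping any valve starts a timer running Checker, which rotates red, blue and yellow dials plus averaged purple and green mix dials.
; Purple latches when red and blue1 valves reach 80 degrees, green when yellow and blue2 do.
; Both together stop the timer, lock all valves and mark the notebook's first task complete.
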(event `self.ReceiveBeginPlay`
  (`KismetSystemLibrary.Delay` 1.0)
  (bind _returnvalue (`GameplayStatics.GetCurrentLevelName` true))
  (if (!= (`KismetArrayLibrary.Array_Find` (`/Game/VRExpansion/Vive/Vive_PawnCharacter.Level_Names` (cast `/Game/VRExpansion/Vive/Vive_PawnCharacter` (`GameplayStatics.GetPlayerPawn` 0) :!pure true)) _returnvalue) 0)
    (`KismetSystemLibrary.PrintString` "not day one")
    (`self.DenyGrippingAll`)))

(event `self.Valve_Blue2.OnGripped`
  (params (GrippingController :type "GripMotionControllerComponent Object Reference") (GripInformation :type "BPActorGripInformation Structure (by ref)"))
  (if (stale _output_get) :!label _label
    (bind _output_get (set `self.Grip Check` false))
    (bind _returnvalue (`KismetSystemLibrary.K2_SetTimer` null "Checker" (`self.Time`) true))))

(event `self.Valve_Blue1.OnGripped`
  (params (GrippingController :type "GripMotionControllerComponent Object Reference") (GripInformation :type "BPActorGripInformation Structure (by ref)"))
  (goto _label))

(event `Check Purple`
  (bind _notebookref (`self.notebookRef`))
  (if (and (>= (`VRDialComponent.CurrentDialAngle` (`self.Valve_Red`)) 80.0) (>= (`VRDialComponent.CurrentDialAngle` (`self.Valve_Blue1`)) 80.0))
    (bind _output_get (set `self.Purple` true))
    (if (and _output_get (stale `Check Green` _output_get)) :!label _label_2
      (set `self.Green` false)
      (`KismetSystemLibrary.K2_ClearAndInvalidateTimerHandle` (stale `self.Valve_Blue2.OnGripped` _returnvalue))
      (`KismetSystemLibrary.PrintString` "win")
      (`self.DenyGrippingAll`)
      (`/Game/findEmma/Blueprints/Props/BP_notebook.changeTextColorToComplete` _notebookref (`/Game/findEmma/Blueprints/Props/BP_notebook.Task1` _notebookref) 0))))

(event `self.Valve_Red.OnGripped`
  (params (GrippingController :type "GripMotionControllerComponent Object Reference") (GripInformation :type "BPActorGripInformation Structure (by ref)"))
  (goto _label))

(event `Check Green`
  (if (and (>= (`VRDialComponent.CurrentDialAngle` (`self.Valve_Yellow`)) 80.0) (>= (`VRDialComponent.CurrentDialAngle` (`self.Valve_Blue2`)) 80.0))
    (bind _output_get (set `self.Green` true))
    (goto _label_2)))

(event `self.Valve_Yellow.OnGripped`
  (params (GrippingController :type "GripMotionControllerComponent Object Reference") (GripInformation :type "BPActorGripInformation Structure (by ref)"))
  (goto _label))

(event `DenyGrippingAll`
  (set `VRDialComponent.bDenyGripping` true (`self.Valve_Red`))
  (set `VRDialComponent.bDenyGripping` true (`self.Valve_Yellow`))
  (set `VRDialComponent.bDenyGripping` true (`self.Valve_Blue2`))
  (set `VRDialComponent.bDenyGripping` true (`self.Valve_Blue1`)))

(fn `Checker`
  (`|ExecutionSequence`
    (:`then_0`
      (`self.Check Purple`)
      (`SceneComponent.K2_SetRelativeRotation` (`self.PurpleDial`) (`KismetMathLibrary.ComposeRotators` (struct :`Roll` 90.0) (`KismetMathLibrary.MakeRotator` 0.0 (+ (/ (+ (`VRDialComponent.CurrentDialAngle` (`self.Valve_Red`)) (`VRDialComponent.CurrentDialAngle` (`self.Valve_Blue1`))) -2.0) 45.0))) false false))
    (:`then_1`
      (`self.Check Green`)
      (`SceneComponent.K2_SetRelativeRotation` (`self.GreenDial`) (`KismetMathLibrary.ComposeRotators` (struct :`Roll` 90.0) (`KismetMathLibrary.MakeRotator` 0.0 (+ (/ (+ (`VRDialComponent.CurrentDialAngle` (`self.Valve_Yellow`)) (`VRDialComponent.CurrentDialAngle` (`self.Valve_Blue2`))) -2.0) 45.0))) false false))
    (:`then_2`
      (`SceneComponent.K2_SetRelativeRotation` (`self.Red_Dial`) (`KismetMathLibrary.ComposeRotators` (struct :`Roll` 90.0) (`KismetMathLibrary.MakeRotator` 0.0 (+ (* (`VRDialComponent.CurrentDialAngle` (`self.Valve_Red`)) -1.0) 45.0))) false false))
    (:`then_3`
      (`SceneComponent.K2_SetRelativeRotation` (`self.Blue_Dial`) (`KismetMathLibrary.ComposeRotators` (struct :`Roll` 90.0) (`KismetMathLibrary.MakeRotator` 0.0 (+ (/ (+ (`VRDialComponent.CurrentDialAngle` (`self.Valve_Blue2`)) (`VRDialComponent.CurrentDialAngle` (`self.Valve_Blue1`))) -2.0) 45.0))) false false))
    (:`then_4`
      (`SceneComponent.K2_SetRelativeRotation` (`self.Yellow_Dial`) (`KismetMathLibrary.ComposeRotators` (struct :`Roll` 90.0) (`KismetMathLibrary.MakeRotator` 0.0 (+ (* (`VRDialComponent.CurrentDialAngle` (`self.Valve_Yellow`)) -1.0) 45.0))) false false))))

(fn `UserConstructionScript`)