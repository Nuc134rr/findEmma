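; Fake can prop that hides its inner can once that component is turned to a target orientation.
; Gripping the lid starts a looping timer that polls the inner can's world rotation, ignoring pitch, against a fixed rotator with a loose tolerance.
; A match hides the inner can and clears the timer.
; Debug strings print at each stage.
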(event `akudfusidov`
  (`SceneComponent.SetVisibility` (`self.InnerCan`) false false)
  (`KismetSystemLibrary.PrintString` "All Good")
  (`KismetSystemLibrary.K2_ClearAndInvalidateTimerHandle` (stale `self.Lid .OnGripped` _returnvalue)))

(event `self.Lid .OnGripped`
  (params (GrippingController :type "GripMotionControllerComponent Object Reference") (GripInformation :type "BPActorGripInformation Structure (by ref)"))
  (`KismetSystemLibrary.PrintString` "B e a n s")
  (bind _returnvalue (`KismetSystemLibrary.K2_SetTimer` null "Shawn" 0.5 true)))

(fn `Shawn`
  (bind _returnvalue (`KismetMathLibrary.MakeRotator` (.roll (`SceneComponent.K2_GetComponentRotation` (`self.InnerCan`))) 0.0 (.yaw (`SceneComponent.K2_GetComponentRotation` (`self.InnerCan`)))))
  (`KismetSystemLibrary.PrintString` (`KismetStringLibrary.Conv_RotatorToString` _returnvalue))
  (if (== _returnvalue (`self.118y`) :`ErrorTolerance` 30.0)
    (`self.akudfusidov`)))

(fn `UserConstructionScript`)