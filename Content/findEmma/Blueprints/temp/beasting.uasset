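; Blueprint for a two-dial VR puzzle, with left and right dials checked against target angles.
; Gripping either dial stores the gripping controller unless both angles already match their targets.
; DenyGripAll blocks further gripping and loops over both dials with a short Delay to drop them from that stored controller.
; An unconnected fragment would start a switchboard task based on level and vent state, but never runs.
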(event `self.Dial_L.OnGripped`
  (params (GrippingController :type "GripMotionControllerComponent Object Reference") (GripInformation :type "BPActorGripInformation Structure (by ref)"))
  ;[1 1 1] code 2
  (if (not (and (== (`VRDialComponent.CurrentDialAngle` (`self.Dial_R`)) (`self.Dial R Check`)) (== (`VRDialComponent.CurrentDialAngle` (`self.Dial_L`)) (`self.Dial L Check`))))
    (set `self.Gripping Controller` GrippingController)))

(event `self.Dial_R.OnGripped`
  (params (GrippingController :type "GripMotionControllerComponent Object Reference") (GripInformation :type "BPActorGripInformation Structure (by ref)"))
  ;[1 1 1] code 2
  (if (not (and (== (`VRDialComponent.CurrentDialAngle` (`self.Dial_R`)) (`self.Dial R Check`)) (== (`VRDialComponent.CurrentDialAngle` (`self.Dial_L`)) (`self.Dial L Check`))))
    (set `self.Gripping Controller` GrippingController)))

(event `DenyGripAll`
  ;[1 1 1] quid game
  (set `VRDialComponent.bDenyGripping` true (`self.Dial_R`))
  (set `VRDialComponent.bDenyGripping` true (`self.Dial_L`))
  (for _array_element (`|MakeArray` (`self.Dial_R`) (`self.Dial_L`))
    (`KismetSystemLibrary.Delay` 0.1)
    (`GripMotionControllerComponent.DropComponent` (`self.Gripping Controller`) _array_element false (0.0 0.0 0.0) (0.0 0.0 0.0))))

(fn `UserConstructionScript`)