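; BP_Emma is the Emma character, which runs one-time VR flashbacks for the paper, mug and floppy items.
; BeginPlay caches the player and sets Day1 from the level name's index, blocking flashbacks while true.
; Each event teleports the player to a room, spawns the item near a mesh after a delay, then starts a fade sequence and returns them.
; GetGoalLocation supplies her controller and an offset player-body position.
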(event `self.ReceiveBeginPlay`
  (bind _returnvalue (`GameplayStatics.GetPlayerPawn` 0))
  ;[1 1 1] Day Check
  (`KismetSystemLibrary.Delay` 1.0)
  (cast `/Game/findEmma/Blueprints/Character/BP_PlayerCharacter` _returnvalue
    (:`then`
      _)
    (:`CastFailed`
      (bind _asvive_pawn_character (cast `/Game/VRExpansion/Vive/Vive_PawnCharacter` _returnvalue))))
  (set `self.Player` _asvive_pawn_character)
  (`KismetSystemLibrary.PrintString` "Hello")
  (`KismetSystemLibrary.Delay` 1.0)
  (bind _returnvalue_2 (`GameplayStatics.GetCurrentLevelName` true))
  (if (!= (`KismetArrayLibrary.Array_Find` (`/Game/VRExpansion/Vive/Vive_PawnCharacter.Level_Names` (`self.Player`)) _returnvalue_2) 1)
    (set `self.day 1` true)
    (else
      (set `self.day 1` false))))

(event `PaperFlashback`
  (bind (_returnvalue_location _returnvalue_rotation _returnvalue_scale) (`KismetMathLibrary.BreakTransform` (`SceneComponent.K2_GetComponentToWorld` (`self.StaticMesh`))))
  (bind _rootcomponent (`Actor.RootComponent` (`self.Player`)))
  ;[1 1 1] Paper Flashback
  (if (`self.paper`)
    _
    (elif (not (`self.day 1`))
      (set `self.Baseloc` (`SceneComponent.K2_GetComponentLocation` _rootcomponent))
      (set `self.Baserot` (`SceneComponent.K2_GetComponentRotation` _rootcomponent))
      (`VRBaseCharacter.SetActorLocationAndRotationVR` (`self.Player`) (`self.Roomloc`) (struct :`Yaw` 180.0) false true false)
      (`KismetSystemLibrary.Delay` 5.0)
      (bind _returnvalue (`|SpawnActorFromClass` "/Game/findEmma/Blueprints/Props/FlashbackItems/BP_flashbackPaper.BP_flashbackPaper_C" (`KismetMathLibrary.MakeTransform` (+ _returnvalue_location (0.0 100.0 0.0)) _returnvalue_rotation _returnvalue_scale) "Undefined" "OverrideRootScale" null null))
      (`KismetSystemLibrary.Delay` 3.0)
      (bind _outactor (`LevelSequencePlayer.CreateLevelSequencePlayer` "/Game/findEmma/Blueprints/FadeOut_Flashback.FadeOut_Flashback"))
      (`MovieSceneSequencePlayer.Play` (`LevelSequenceActor.SequencePlayer` _outactor))
      (`self.K2_DestroyActor` _returnvalue)
      (`VRBaseCharacter.SetActorLocationAndRotationVR` (`self.Player`) (`self.Baseloc`) (`self.Baserot`) true true true)
      (set `self.paper` true))))

(event `MugFlashback`
  (bind (_returnvalue_location _returnvalue_rotation _returnvalue_scale) (`KismetMathLibrary.BreakTransform` (`SceneComponent.K2_GetComponentToWorld` (`self.StaticMesh`))))
  (bind _rootcomponent (`Actor.RootComponent` (`self.Player`)))
  ;[1 1 1] Mug Flashback
  (if (`self.mug`)
    _
    (elif (not (`self.day 1`))
      (set `self.Baseloc` (`SceneComponent.K2_GetComponentLocation` _rootcomponent))
      (set `self.Baserot` (`SceneComponent.K2_GetComponentRotation` _rootcomponent))
      (`VRBaseCharacter.SetActorLocationAndRotationVR` (`self.Player`) (`self.Roomloc`) (struct :`Yaw` 180.0) false true false)
      (`KismetSystemLibrary.Delay` 5.0)
      (bind _returnvalue (`|SpawnActorFromClass` "/Game/findEmma/Blueprints/Props/FlashbackItems/BP_flashbackMug.BP_flashbackMug_C" (`KismetMathLibrary.MakeTransform` (+ _returnvalue_location (0.0 100.0 0.0)) _returnvalue_rotation _returnvalue_scale) "Undefined" "OverrideRootScale" null null))
      (`KismetSystemLibrary.Delay` 3.0)
      (bind _outactor (`LevelSequencePlayer.CreateLevelSequencePlayer` "/Game/findEmma/Blueprints/FadeOut_Flashback.FadeOut_Flashback"))
      (`MovieSceneSequencePlayer.Play` (`LevelSequenceActor.SequencePlayer` _outactor))
      (`self.K2_DestroyActor` _returnvalue)
      (`VRBaseCharacter.SetActorLocationAndRotationVR` (`self.Player`) (`self.Baseloc`) (`self.Baserot`) true true true)
      (set `self.mug` true))))

(event `FloppyFlashback`
  (bind (_returnvalue_location _returnvalue_rotation _returnvalue_scale) (`KismetMathLibrary.BreakTransform` (`SceneComponent.K2_GetComponentToWorld` (`self.StaticMesh`))))
  (bind _rootcomponent (`Actor.RootComponent` (`self.Player`)))
  ;[1 1 1] Floppy Flashback
  (if (`self.floppy`)
    _
    (elif (not (`self.day 1`))
      (set `self.Baseloc` (`SceneComponent.K2_GetComponentLocation` _rootcomponent))
      (set `self.Baserot` (`SceneComponent.K2_GetComponentRotation` _rootcomponent))
      (`VRBaseCharacter.SetActorLocationAndRotationVR` (`self.Player`) (`self.Roomloc`) (struct :`Yaw` 180.0) false true false)
      (`KismetSystemLibrary.Delay` 5.0)
      (bind _returnvalue (`|SpawnActorFromClass` "/Game/findEmma/Blueprints/Props/FlashbackItems/BP_floppy.BP_floppy_C" (`KismetMathLibrary.MakeTransform` (+ _returnvalue_location (0.0 100.0 0.0)) _returnvalue_rotation _returnvalue_scale) "Undefined" "OverrideRootScale" null null))
      (`KismetSystemLibrary.Delay` 3.0)
      (bind _outactor (`LevelSequencePlayer.CreateLevelSequencePlayer` "/Game/findEmma/Blueprints/FadeOut_Flashback.FadeOut_Flashback"))
      (`MovieSceneSequencePlayer.Play` (`LevelSequenceActor.SequencePlayer` _outactor))
      (`self.K2_DestroyActor` _returnvalue)
      (`VRBaseCharacter.SetActorLocationAndRotationVR` (`self.Player`) (`self.Baseloc`) (`self.Baserot`) true true true)
      (set `self.floppy` true))))

(fn `GetGoalLocation`
  (returns (Controller :type "Controller Object Reference") (Goal :type "Vector Structure"))
  (bind _output_get (set `self.Goal` (+ (`SceneComponent.K2_GetComponentLocation` (`/Game/VRExpansion/Vive/Vive_PawnCharacter.Body` (cast `/Game/VRExpansion/Vive/Vive_PawnCharacter` (`GameplayStatics.GetPlayerPawn` 0) :!pure true))) (`self.Offset`))))
  (return (`self.GetController`) _output_get))

(fn `UserConstructionScript`)