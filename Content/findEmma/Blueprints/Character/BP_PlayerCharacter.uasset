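; VR player character with motion-controller locomotion and object gripping, built on VR plugin components.
; Left thumbstick drives either camera-relative smooth movement or a spawned teleport controller, switched by a toggle input, while the right thumbstick snap-turns.
; Per-hand grab spheres track overlapping actors, which grip inputs pick up and drop through VRGripInterface.
; Closest-object search only runs with at most one overlap; a helper starts climbing when allowed.
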(event `self.GrabSphereRight.OnComponentBeginOverlap`
  (params (OverlappedComponent :type "PrimitiveComponent Object Reference") (OtherActor :type "Actor Object Reference") (OtherComp :type "PrimitiveComponent Object Reference") (OtherBodyIndex :type Integer) (bFromSweep :type Boolean) (SweepResult :type "HitResult Structure (by ref)"))
  ;[1 1 0] Handle Gripping
  (`KismetArrayLibrary.Array_Add` (`self.OverlappingObjectsRight`) OtherActor))

(event `InputAction|PrimaryGripLeft`
  (params (Key :type "Key Structure"))
  ;[1 1 0] Handle Gripping
  (:`Pressed`
    (`KismetSystemLibrary.PrintString` "Left Grip Called" true true (struct :`R` 1.0 :`G` 1.0 :`A` 1.0))
    (bind _heldobject (`self.TryGrip` (`self.OverlappingObjectsLeft`) (`self.LeftMotionController`)))
    (set `self.HeldObjectLeft` _heldobject))
  (:`Released`
    (bind _dropsucceed (`self.TryDrop` (`self.LeftMotionController`) (`self.HeldObjectLeft`)))
    (if _dropsucceed
      (set `self.HeldObjectLeft` null)
      (set `self.NearestObject` null))))

(event `InputAxis|MotionControllerThumbLeft_Y`
  (params (AxisValue :type "Float (single-precision)"))
  ;[0.09543 1 0.1731] HAND MOVEMENT
  ;;[1 1 1] Decide the movement mode (read teleport variable)
  (bind _output_get (set `self.yAxisValue` AxisValue))
  (if (`self.bTeleport`)
    ;;[1 1 1] Handle Teleportation Inputs
    (if (> (`self.yAxisValue`) (`self.Deadzone`))
      (`self.SetTeleporterActive` true)
      (set `self.bIsTeleporting` true)
      (elif (`self.bIsTeleporting`)
        (`self.SetTeleporterActive` false)
        (`self.Teleport`)))
    (else
      ;;[1 1 1] Move forward and backward (smooth locomotion)
      (if (> (`KismetMathLibrary.Abs` _output_get) (`self.Deadzone`))
        (`self.AddMovementInput` (`SceneComponent.GetForwardVector` (`self.VRReplicatedCamera`)) (`self.yAxisValue`))))))

(event `self.GrabSphereRight.OnComponentEndOverlap`
  (params (OverlappedComponent :type "PrimitiveComponent Object Reference") (OtherActor :type "Actor Object Reference") (OtherComp :type "PrimitiveComponent Object Reference") (OtherBodyIndex :type Integer))
  ;[1 1 0] Handle Gripping
  (`KismetArrayLibrary.Array_RemoveItem` (`self.OverlappingObjectsRight`) OtherActor))

(event `InputAction|ToggleMovementMode`
  (params (Key :type "Key Structure"))
  ;[0.09543 1 0.1731] HAND MOVEMENT
  ;;[1 1 1] Toggle Movement Mode
  (:`Pressed`
    (`/Engine/EditorBlueprintResources/StandardMacros.FlipFlop`
      (:`A`
        (set `self.bTeleport` true))
      (:`B`
        (set `self.bTeleport` false)))))

(event `InputAction|PrimaryGripRight`
  (params (Key :type "Key Structure"))
  ;[1 1 0] Handle Gripping
  (:`Pressed`
    (`KismetSystemLibrary.PrintString` "Right Grip Called" true true (struct :`R` 1.0 :`G` 1.0 :`A` 1.0))
    (bind _heldobject (`self.TryGrip` (`self.OverlappingObjectsRight`) (`self.RightMotionController`)))
    (set `self.HeldObjectRight` _heldobject))
  (:`Released`
    (bind _dropsucceed (`self.TryDrop` (`self.RightMotionController`) (`self.HeldObjectRight`)))
    (if _dropsucceed
      (set `self.HeldObjectRight` null)
      (set `self.NearestObject` null))))

(event `self.GrabSphereLeft.OnComponentBeginOverlap`
  (params (OverlappedComponent :type "PrimitiveComponent Object Reference") (OtherActor :type "Actor Object Reference") (OtherComp :type "PrimitiveComponent Object Reference") (OtherBodyIndex :type Integer) (bFromSweep :type Boolean) (SweepResult :type "HitResult Structure (by ref)"))
  ;[1 1 0] Handle Gripping
  (`KismetSystemLibrary.PrintString` (`KismetSystemLibrary.GetDisplayName` OtherActor) true true (struct :`G` 1.0 :`A` 1.0) 10.0)
  (`KismetArrayLibrary.Array_Add` (`self.OverlappingObjectsLeft`) OtherActor))

(event `self.GrabSphereLeft.OnComponentEndOverlap`
  (params (OverlappedComponent :type "PrimitiveComponent Object Reference") (OtherActor :type "Actor Object Reference") (OtherComp :type "PrimitiveComponent Object Reference") (OtherBodyIndex :type Integer))
  ;[1 1 0] Handle Gripping
  (`KismetSystemLibrary.PrintString` (`KismetSystemLibrary.GetDisplayName` OtherActor) true true (struct :`R` 1.0 :`A` 1.0) 10.0)
  (`KismetArrayLibrary.Array_RemoveItem` (`self.OverlappingObjectsLeft`) OtherActor))

(event `InputAxis|MotionControllerThumbLeft_X`
  (params (AxisValue :type "Float (single-precision)"))
  ;[0.09543 1 0.1731] HAND MOVEMENT
  ;;[1 1 1] Move Left and Right (Smooth Locomotion)
  (bind _output_get (set `self.xAxisValue` AxisValue))
  (if (`self.bTeleport`)
    _
    (elif (> (`KismetMathLibrary.Abs` _output_get) (`self.Deadzone`))
      (`self.AddMovementInput` (`SceneComponent.GetRightVector` (`self.VRReplicatedCamera`)) (`self.xAxisValue`)))))

(event `self.ReceiveBeginPlay`
  ;[1 1 1] Spawns Teleport Controller (from plugin)
  (bind _returnvalue (`|SpawnActorFromClass` "/Game/VRExpansion/Vive/BP_Teleport_Controller.BP_Teleport_Controller_C" (`KismetMathLibrary.MakeTransform` (0.0 0.0 0.0)) "AlwaysSpawn" "OverrideRootScale" self (`self.LeftMotionController`) (`self.IsLocallyControlled`) null))
  (bind _output_get (set `self.TeleportControllerLeft` _returnvalue))
  (`self.K2_AttachToComponent` _output_get null "None" "SnapToTarget" "SnapToTarget" "SnapToTarget" false))

(event `Teleport`
  ;[0.09543 1 0.1731] HAND MOVEMENT
  ;;[1 1 1] Handle Teleport
  (`MovementComponent.StopMovementImmediately` (`self.VRMovementReference`))
  (set `self.bIsTeleporting` true)
  (`self.SetTeleporterActive` false)
  (`self.K2_TeleportTo` (`self.GetTeleportLocation` (`/Game/VRExpansion/Vive/BP_Teleport_Controller.GetTeleportDestination` (`self.TeleportControllerLeft`) false)) (`self.K2_GetActorRotation`))
  (set `self.bIsTeleporting` false))

(event `InputAxis|MotionControllerThumbRight_X`
  (params (AxisValue :type "Float (single-precision)"))
  ;[0.09543 1 0.1731] HAND MOVEMENT
  ;;[1 1 1] Handle Snap Turning
  (bind _output_get (set `self.snapTurnDir` AxisValue))
  (if (`self.bTurning`)
    (bind _returnvalue (> (`KismetMathLibrary.Abs` _output_get) (`self.Deadzone`)))
    (if (not _returnvalue)
      (set `self.bTurning` false))
    (elif _returnvalue
      (set `self.bTurning` true)
      (`VRBaseCharacterMovementComponent.PerformMoveAction_SnapTurn` (`self.VRMovementReference`) (* (`self.snapTurnAngle`) (`KismetMathLibrary.SignOfFloat` (`self.snapTurnDir`))) "VRMOVEACTION_Velocity_None" false false))))

(fn `CompareObjectClass`
  (params (Object :type "Object Object Reference"))
  (returns (ReturnValue :type Boolean))
  (bind _returnvalue (`GameplayStatics.GetObjectClass` Object))
  (return (or (== (`self.GrippableClass`) _returnvalue) (`KismetMathLibrary.ClassIsChildOf` _returnvalue (`self.GrippableClass`)))))

(fn `GetClosestOverlappingObject`
  (params (OverlappingObjectsArray :type "Array of Actor Object Reference") (MotionController :type "GripMotionControllerComponent Object Reference"))
  (returns (NearestObject :type "Actor Object Reference"))
  (if (> (`KismetArrayLibrary.Array_Length` OverlappingObjectsArray) 1)
    (return null)
    (else
      (`KismetSystemLibrary.PrintString` "FOR EACH CALLED")
      (for _array_element (`local.OverlappingObjectsArray`)
        (if (`KismetSystemLibrary.DoesImplementInterface` _array_element "/Script/VRExpansionPlugin.VRGripInterface")
          (bind _returnvalue (`KismetMathLibrary.VSize` (- (`self.K2_GetActorLocation` _array_element) (`SceneComponent.K2_GetComponentLocation` (`local.MotionController`)))))
          (if (<= _returnvalue (`self.NearestObjectDistance`))
            (set `self.NearestObjectDistance` _returnvalue)
            (bind _output_get (set `self.NearestObject` _array_element)))
          (else
            (`KismetSystemLibrary.PrintString` "Does Not Implement Interface!"))))
      (`KismetSystemLibrary.PrintText` (`|FormatText` "Nearest Object: {1}" _output_get))
      (return _output_get))))

(fn `SetTeleporterActive`
  (params (Active :type Boolean))
  (bind _teleportcontrollerleft (`self.TeleportControllerLeft`))
  (`/Engine/EditorBlueprintResources/StandardMacros.IsValid` _teleportcontrollerleft
    (:`Is Valid`
      (if Active
        (`/Game/VRExpansion/Vive/BP_Teleport_Controller.ActivateTeleporter` _teleportcontrollerleft)
        (else
          (`/Game/VRExpansion/Vive/BP_Teleport_Controller.DisableTeleporter` _teleportcontrollerleft))))
    (:`Is Not Valid`
      (`KismetSystemLibrary.PrintString` "Controller Not Valid!"))))

(fn `TryDrop`
  (params (MotionController :type "GripMotionControllerComponent Object Reference") (HeldObject :type "Actor Object Reference"))
  (returns (DropSucceed :type Boolean))
  (bind _returnvalue (`GripMotionControllerComponent.DropObjectByInterface` MotionController HeldObject 0 (0.0 0.0 0.0) (0.0 0.0 0.0)))
  (return _returnvalue))

(fn `TryGrip`
  (params (OverlappingObjectsArray :type "Array of Actor Object Reference") (MotionController :type "GripMotionControllerComponent Object Reference"))
  (returns (HeldObject :type "Actor Object Reference"))
  (bind _nearestobject (`self.GetClosestOverlappingObject` OverlappingObjectsArray MotionController))
  (`/Engine/EditorBlueprintResources/StandardMacros.IsValid` _nearestobject
    (:`Is Valid`
      (bind _returnvalue (`GripMotionControllerComponent.GripObjectByInterface` (`local.MotionController`) _nearestobject (`self.GetTransform` _nearestobject) false "None" "None" false))
      (if _returnvalue
        (`KismetSystemLibrary.PrintString` "Grip Succeed!" true true (struct :`G` 1.0 :`A` 1.0))
        (return (`self.NearestObject`))
        (else
          (`KismetSystemLibrary.PrintString` "Grip Failed!" true true (struct :`R` 1.0 :`A` 1.0)))))))

(fn `UpdateLaserBeam`
  (params (Deltatime :type "Float (double-precision)")))

(fn `UserConstructionScript`)