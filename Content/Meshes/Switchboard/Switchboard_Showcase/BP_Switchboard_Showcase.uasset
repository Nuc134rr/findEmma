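; Showcase Blueprint for a switchboard mesh that cycles through three material variants when U is pressed.
; On BeginPlay it enables input and replaces every material on its static mesh components with dynamic instances, cached in an array.
; Each press advances a wrapping counter and writes it to the MaterialID scalar parameter on all cached instances.
; Emission material setup in the construction script is disconnected, so it never runs.
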(event `Key|U`
  (params (Key :type "Key Structure"))
  (bind _materialid (`self.MaterialID`))
  (bind _showcase_dynamicmats (`self.Showcase_DynamicMats`))
  (:`Pressed`
    (set `self.MaterialID` (+ _materialid 1))
    (if (> _materialid 2)
      (set `self.MaterialID` 0))
    (switch `int` _materialid
      (:`0`
        (for _array_element _showcase_dynamicmats
          (`MaterialInstanceDynamic.SetScalarParameterValue` _array_element "MaterialID" 0.0)))
      (:`1`
        (for _array_element_2 _showcase_dynamicmats
          (`MaterialInstanceDynamic.SetScalarParameterValue` _array_element_2 "MaterialID" 1.0)))
      (:`2`
        (for _array_element_3 _showcase_dynamicmats
          (`MaterialInstanceDynamic.SetScalarParameterValue` _array_element_3 "MaterialID" 2.0))))))

(event `self.ReceiveBeginPlay`
  ;[1 1 1] Preview
  (`self.EnableInput` (`GameplayStatics.GetPlayerController` 0))
  (for _array_element (`self.K2_GetComponentsByClass` "/Script/Engine.StaticMeshComponent")
    (for (_array_element_2 _array_index) (`MeshComponent.GetMaterials` _array_element)
      (bind _returnvalue (`KismetMaterialLibrary.CreateDynamicMaterialInstance` _array_element_2))
      (`PrimitiveComponent.SetMaterial` _array_element _array_index _returnvalue)
      (`KismetArrayLibrary.Array_Add` (`self.Showcase_DynamicMats`) _returnvalue))))

(fn `UserConstructionScript`
  ;[1 1 1] Dynamic Material for Changing Emission
)